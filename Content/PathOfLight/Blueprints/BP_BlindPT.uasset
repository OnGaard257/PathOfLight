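; Blind enemy character that roams at random and hunts the player by hearing.
; Roaming loops through AIMoveTo to random reachable points with random pauses.
; Hearing updates while the player isn't crouched raise a detection counter, starting a self-repeating, delayed LocaterMode at a threshold.
; That mode decays the counter back toward roaming or, at maximum, starts a chase that never resets; older investigate logic is disconnected.
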(event `self.ReceiveBeginPlay`
  (`self.Random Blind Roam`))

(event `self.ReceiveTick`
  (params (DeltaSeconds :type "Float (single-precision)")))

(event `Random Blind Roam`
  ;[1 1 1] Random Movement for Blind Enemy AI
  (set `CharacterMovementComponent.MaxWalkSpeed` 500.0 (`self.CharacterMovement`))
  (`|AIMoveTo` self (`NavigationSystemV1.K2_GetRandomReachablePointInRadius` (`self.K2_GetActorLocation`) 1500.0 null null) null
    (:`OnSuccess`
      (`KismetSystemLibrary.Delay` (`KismetMathLibrary.RandomFloatInRange` 1.0 5.0))
      (if (not (`self.Investigating`))
        (`self.Random Blind Roam` :!label _label)))
    (:`OnFail`
      (goto _label))))

(event `self.AIPerception (Blind Enemy Hearing).OnTargetPerceptionUpdated`
  (params (Actor :type "Actor Object Reference") (Stimulus :type "AIStimulus Structure"))
  (bind _hearingdetection (`self.HearingDetection`))
  (if (not (`self.ChasingMode`))
    (bind _asbp_character (cast `/Game/PathOfLight/bp_Imports/bp_Character` (`GameplayStatics.GetPlayerCharacter` 0)))
    (if (not (`/Game/PathOfLight/bp_Imports/bp_Character.Crouched` _asbp_character))
      (`KismetSystemLibrary.Delay` 0.5)
      (bind _result (`/Engine/EditorBlueprintResources/StandardMacros.IncrementInt` _hearingdetection)
        (:`  `
          (`KismetSystemLibrary.PrintString` (`KismetStringLibrary.Conv_IntToString` _result))
          (if (>= _hearingdetection 5)
            (`self.LocaterMode`)
            (`KismetSystemLibrary.PrintString` "Locating")))))))

(event `ChasePlayer`
  (set `self.ChasingMode` true)
  (set `CharacterMovementComponent.MaxWalkSpeed` 500.0 (`self.CharacterMovement`))
  (bind _asbp_character (cast `/Game/PathOfLight/bp_Imports/bp_Character` (`GameplayStatics.GetPlayerCharacter` 0)))
  (`|AIMoveTo` self (0.0 0.0 0.0) _asbp_character))

(event `LocaterMode`
  (`KismetSystemLibrary.Delay` 2.0)
  (if (< (`self.HearingDetection`) 10)
    (bind _result (`/Engine/EditorBlueprintResources/StandardMacros.DecrementInt` (`self.HearingDetection`))
      (:`  `
        (bind _output_get (set `self.HearingDetection` (`KismetMathLibrary.Clamp` _result 0 10)))
        (`KismetSystemLibrary.PrintString` (`KismetStringLibrary.Conv_IntToString` _output_get))
        (if (== (`self.HearingDetection`) 0)
          (`self.Random Blind Roam`)
          (set `self.HearingDetection` 0)
          (set `self.Locating` false)
          (else
            (`self.LocaterMode`)))))
    (else
      (`self.ChasePlayer`)
      (`KismetSystemLibrary.PrintString` "Chasing")
      (set `self.HearingDetection` 10))))

(fn `UserConstructionScript`)