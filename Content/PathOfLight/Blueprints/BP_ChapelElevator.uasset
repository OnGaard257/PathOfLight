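; Chapel elevator that the player rides up and down by pressing Interact at its switch.
; Collider overlap with bp_Character enables input and outlines the switch.
; After a short delay, two FlipFlops alternately play and reverse the gear-rotation and cage-movement timelines.
; The cage timeline's Update also triggers the front and back door timelines, staggered by a Delay, with order and direction set by GoingUp.
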(event `EnhancedInput|/Game/PathOfLight/bp_Imports/ia_Interact`
  (params (ActionValue :type Boolean) (ElapsedSeconds :type "Float (double-precision)") (TriggeredSeconds :type "Float (double-precision)") (InputAction :type "InputAction Object Reference" :default "/Game/PathOfLight/bp_Imports/ia_Interact.ia_Interact"))
  (:`Triggered`
    (`/Game/PathOfLight/bp_Imports/bp_Character.Interact` (stale `self.Collider.OnComponentBeginOverlap` _asbp_character))
    (`KismetSystemLibrary.Delay` 0.5)
    (`|ExecutionSequence`
      (:`then_0`
        (`/Engine/EditorBlueprintResources/StandardMacros.FlipFlop`
          (:`A`
            ;[1 1 1] Rotate Gears
            (bind (_direction _rotategearsclockwise) (`Timeline|Rotating Gears` :!label _label)
              (:`Update`
                (`SceneComponent.K2_SetRelativeRotation` (`self.MovingGear1`) (`KismetMathLibrary.RLerp` (`self.GearsStartingRotation`) (`self.GearsEndingRotation`) _rotategearsclockwise) false false)
                (`SceneComponent.K2_SetRelativeRotation` (`self.MovingGear2`) (`KismetMathLibrary.RLerp` (`self.GearsStartingRotation`) (`self.GearsEndingRotation`) _rotategearsclockwise) false false)
                (`SceneComponent.K2_SetRelativeRotation` (`self.MovingGear3`) (`KismetMathLibrary.RLerp` (`self.GearsStartingRotation`) (`self.GearsEndingRotation`) _rotategearsclockwise) false false)
                (`SceneComponent.K2_SetRelativeRotation` (`self.RotatingGear1`) (`KismetMathLibrary.RLerp` (`self.GearsStartingRotation`) (`self.GearsEndingRotation`) _rotategearsclockwise) false false)
                (`SceneComponent.K2_SetRelativeRotation` (`self.RotatingGear2`) (`KismetMathLibrary.RLerp` (`self.GearsStartingRotation`) (`self.GearsEndingRotation`) _rotategearsclockwise) false false)
                (`SceneComponent.K2_SetRelativeRotation` (`self.RotatingGear3`) (`KismetMathLibrary.RLerp` (`self.GearsStartingRotation`) (`self.GearsEndingRotation`) _rotategearsclockwise) false false)
                (`SceneComponent.K2_SetRelativeRotation` (`self.RotatingGear4`) (`KismetMathLibrary.RLerp` (`self.GearsStartingRotation`) (`self.GearsEndingRotation`) _rotategearsclockwise) false false)
                (`SceneComponent.K2_SetRelativeRotation` (`self.RotatingGear5`) (`KismetMathLibrary.RLerp` (`self.GearsStartingRotation`) (`self.GearsEndingRotation`) _rotategearsclockwise) false false)
                (`SceneComponent.K2_SetRelativeRotation` (`self.RotatingGear6`) (`KismetMathLibrary.RLerp` (`self.GearsStartingRotation`) (`self.GearsEndingRotation`) _rotategearsclockwise) false false))))
          (:`B`
            (goto _label :!via `Reverse`))))
      (:`then_1`
        (`/Engine/EditorBlueprintResources/StandardMacros.FlipFlop`
          (:`A`
            (set `self.GoingUp` true)
            ;[1 1 1] Elevator Moves Up and Down
            (bind (_direction_2 _elevatorcagemove _newtrack_6 _elevator) (`Timeline|Elevator Move Up` :!label _label_2)
              (:`Update`
                (`|ExecutionSequence`
                  (:`then_0`
                    (`SceneComponent.K2_SetRelativeLocation` (`self.ElevatorCage`) _elevatorcagemove false false))
                  (:`then_1`
                    (if (`self.GoingUp`)
                      ;[1 1 1] Front Door Close when Going Up
                      (bind (_direction_3 _dooropentime) (`Timeline|FrontDoors` :!label _label_3)
                        (:`Update`
                          (`SceneComponent.K2_SetRelativeLocation` (`self.ElevatorDoorFrontLeft`) (`KismetMathLibrary.VLerp` (`self.LeftDoorStartPos`) (`self.LeftDoorEndPos`) _dooropentime) false false)
                          (`SceneComponent.K2_SetRelativeLocation` (`self.ElevatorDoorFrontRight`) (`KismetMathLibrary.VLerp` (`self.RightDoorStartPos`) (`self.RightDoorEndPos`) _dooropentime) false false)
                          (`KismetSystemLibrary.Delay` 5.0)
                          (bind (_direction_4 _dooropentime_2) (`Timeline|BackDoors` :!label _label_4)
                            (:`Update`
                              (`SceneComponent.K2_SetRelativeLocation` (`self.ElevatorDoorBackLeft`) (`KismetMathLibrary.VLerp` (`self.B_LeftDoorStartPos`) (`self.B_LeftDoorEndPos`) _dooropentime_2) false false)
                              (`SceneComponent.K2_SetRelativeLocation` (`self.ElevatorDoorBackRight`) (`KismetMathLibrary.VLerp` (`self.B_RightDoorStartPos`) (`self.B_RightDoorEndPos`) _dooropentime_2) false false)))))
                      (else
                        (`|ExecutionSequence`
                          (:`then_0`
                            (goto _label_4 :!via `Reverse`))
                          (:`then_1`
                            (`KismetSystemLibrary.Delay` 5.0)
                            (goto _label_3 :!via `Reverse`))))))))))
          (:`B`
            (set `self.GoingUp` false)
            (goto _label_2 :!via `Reverse`)))))))

(event `self.Collider.OnComponentBeginOverlap`
  (params (OverlappedComponent :type "PrimitiveComponent Object Reference") (OtherActor :type "Actor Object Reference") (OtherComp :type "PrimitiveComponent Object Reference") (OtherBodyIndex :type Integer) (bFromSweep :type Boolean) (SweepResult :type "HitResult Structure (by ref)"))
  (bind _asbp_character (cast `/Game/PathOfLight/bp_Imports/bp_Character` OtherActor))
  (`self.EnableInput` (`GameplayStatics.GetPlayerController` 0))
  (`MeshComponent.SetOverlayMaterial` (`self.ElevatorSwitch`) "/Game/PathOfLight/Materials/m_Outline_Inst.m_Outline_Inst"))

(event `self.Collider.OnComponentEndOverlap`
  (params (OverlappedComponent :type "PrimitiveComponent Object Reference") (OtherActor :type "Actor Object Reference") (OtherComp :type "PrimitiveComponent Object Reference") (OtherBodyIndex :type Integer))
  (cast `/Game/PathOfLight/bp_Imports/bp_Character` OtherActor)
  (`self.DisableInput` (`GameplayStatics.GetPlayerController` 0))
  (`MeshComponent.SetOverlayMaterial` (`self.ElevatorSwitch`) null))

(fn `UserConstructionScript`)