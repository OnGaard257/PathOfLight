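; Chapel elevator that the player character raises and lowers from a switch, with animated gears.
; Overlapping the collider caches the character, enables input and outlines the switch; leaving disables input and clears the overlay.
; Interact calls the character's Interact, then after a short delay two FlipFlops alternately play and reverse timelines that rotate the gears and move the cage.
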(event `EnhancedInput|/Game/PathOfLight/bp_Imports/ia_Interact`
  (params (ActionValue :type Boolean) (ElapsedSeconds :type "Float (double-precision)") (TriggeredSeconds :type "Float (double-precision)") (InputAction :type "InputAction Object Reference" :default "/Game/PathOfLight/bp_Imports/ia_Interact.ia_Interact"))
  (:`Triggered`
    (`/Game/PathOfLight/bp_Imports/bp_Character.Interact` (stale `self.Collider.OnComponentBeginOverlap` _asbp_character))
    (`KismetSystemLibrary.Delay` 0.5)
    (`|ExecutionSequence`
      (:`then_0`
        (`/Engine/EditorBlueprintResources/StandardMacros.FlipFlop`
          (:`A`
            ;[1 1 1] RotateGears
            (bind (_direction _rotategearsclockwise) (`Timeline|Rotating Gears` :!label _label)
              (:`Update`
                (`SceneComponent.K2_SetRelativeRotation` (`self.MovingGear1`) (`KismetMathLibrary.RLerp` (`self.GearsStartingRotation`) (`self.GearsEndingRotation`) _rotategearsclockwise) false false)
                (`SceneComponent.K2_SetRelativeRotation` (`self.MovingGear2`) (`KismetMathLibrary.RLerp` (`self.GearsStartingRotation`) (`self.GearsEndingRotation`) _rotategearsclockwise) false false)
                (`SceneComponent.K2_SetRelativeRotation` (`self.MovingGear3`) (`KismetMathLibrary.RLerp` (`self.GearsStartingRotation`) (`self.GearsEndingRotation`) _rotategearsclockwise) false false)
                (`SceneComponent.K2_SetRelativeRotation` (`self.RotatingGear1`) (`KismetMathLibrary.RLerp` (`self.GearsStartingRotation`) (`self.GearsEndingRotation`) _rotategearsclockwise) false false)
                (`SceneComponent.K2_SetRelativeRotation` (`self.RotatingGear2`) (`KismetMathLibrary.RLerp` (`self.GearsStartingRotation`) (`self.GearsEndingRotation`) _rotategearsclockwise) false false)
                (`SceneComponent.K2_SetRelativeRotation` (`self.RotatingGear3`) (`KismetMathLibrary.RLerp` (`self.GearsStartingRotation`) (`self.GearsEndingRotation`) _rotategearsclockwise) false false)
                (`SceneComponent.K2_SetRelativeRotation` (`self.RotatingGear4`) (`KismetMathLibrary.RLerp` (`self.GearsStartingRotation`) (`self.GearsEndingRotation`) _rotategearsclockwise) false false)
                (`SceneComponent.K2_SetRelativeRotation` (`self.RotatingGear5`) (`KismetMathLibrary.RLerp` (`self.GearsStartingRotation`) (`self.GearsEndingRotation`) _rotategearsclockwise) false false)
                (`SceneComponent.K2_SetRelativeRotation` (`self.RotatingGear6`) (`KismetMathLibrary.RLerp` (`self.GearsStartingRotation`) (`self.GearsEndingRotation`) _rotategearsclockwise) false false))))
          (:`B`
            (goto _label :!via `Reverse`))))
      (:`then_1`
        (`/Engine/EditorBlueprintResources/StandardMacros.FlipFlop`
          (:`A`
            ;[1 1 1] Elevator Moves Up and Down
            (bind (_direction_2 _elevatorcagemove _newtrack_6 _elevator) (`Timeline|Elevator Move Up` :!label _label_2)
              (:`Update`
                (`|ExecutionSequence`
                  (:`then_0`
                    (`SceneComponent.K2_SetRelativeLocation` (`self.ElevatorCage`) _elevatorcagemove false false))))))
          (:`B`
            (goto _label_2 :!via `Reverse`)))))))

(event `self.Collider.OnComponentBeginOverlap`
  (params (OverlappedComponent :type "PrimitiveComponent Object Reference") (OtherActor :type "Actor Object Reference") (OtherComp :type "PrimitiveComponent Object Reference") (OtherBodyIndex :type Integer) (bFromSweep :type Boolean) (SweepResult :type "HitResult Structure (by ref)"))
  (bind _asbp_character (cast `/Game/PathOfLight/bp_Imports/bp_Character` OtherActor))
  (`self.EnableInput` (`GameplayStatics.GetPlayerController` 0))
  (`MeshComponent.SetOverlayMaterial` (`self.ElevatorSwitch`) "/Game/PathOfLight/Materials/m_Outline_Inst.m_Outline_Inst"))

(event `self.Collider.OnComponentEndOverlap`
  (params (OverlappedComponent :type "PrimitiveComponent Object Reference") (OtherActor :type "Actor Object Reference") (OtherComp :type "PrimitiveComponent Object Reference") (OtherBodyIndex :type Integer))
  (cast `/Game/PathOfLight/bp_Imports/bp_Character` OtherActor)
  (`self.DisableInput` (`GameplayStatics.GetPlayerController` 0))
  (`MeshComponent.SetOverlayMaterial` (`self.ElevatorSwitch`) null))

(fn `UserConstructionScript`)