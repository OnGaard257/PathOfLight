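; BP_JournalTest is a test interactable for a journal page UI, usable while the character is inside its box.
; Box overlap events for bp_Character set a CanInteract flag that gates the ia_Interact input.
; Interacting collapses BookUI if visible; otherwise it creates and displays a Wbp_journalpage widget only when BookUI is invalid.
; The graph never assigns the new widget to BookUI or makes a collapsed BookUI visible again.
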(event `self.Box.OnComponentBeginOverlap`
  (params (OverlappedComponent :type "PrimitiveComponent Object Reference") (OtherActor :type "Actor Object Reference") (OtherComp :type "PrimitiveComponent Object Reference") (OtherBodyIndex :type Integer) (bFromSweep :type Boolean) (SweepResult :type "HitResult Structure (by ref)"))
  (cast `/Game/PathOfLight/bp_Imports/bp_Character` OtherActor)
  (set `self.bCanInteract?` true))

(event `self.Box.OnComponentEndOverlap`
  (params (OverlappedComponent :type "PrimitiveComponent Object Reference") (OtherActor :type "Actor Object Reference") (OtherComp :type "PrimitiveComponent Object Reference") (OtherBodyIndex :type Integer))
  (cast `/Game/PathOfLight/bp_Imports/bp_Character` OtherActor)
  (set `self.bCanInteract?` false))

(event `EnhancedInput|/Game/PathOfLight/bp_Imports/ia_Interact`
  (params (ActionValue :type Boolean) (ElapsedSeconds :type "Float (double-precision)") (TriggeredSeconds :type "Float (double-precision)") (InputAction :type "InputAction Object Reference" :default "/Game/PathOfLight/bp_Imports/ia_Interact.ia_Interact"))
  (:`Triggered`
    (if (`self.bCanInteract?`)
      (if (`|EnumEquality` (`Widget.GetVisibility` (`self.BookUI`)) "Visible")
        (`Widget.SetVisibility` (`self.BookUI`) "Collapsed")
        (else
          (`/Engine/EditorBlueprintResources/StandardMacros.IsValid` (`self.BookUI`)
            (:`Is Not Valid`
              (bind _returnvalue (`|CreateWidget` "/Game/PathOfLight/UI/wbp_journalpage.wbp_journalpage_C"))
              (`UserWidget.AddToViewport` _returnvalue 0))))))))

(fn `UserConstructionScript`)