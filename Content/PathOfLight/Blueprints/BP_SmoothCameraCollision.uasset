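; BP_SmoothCameraCollision is an unfinished camera collision Blueprint for a spring arm and follow camera.
; Its tick runs a sphere trace from the spring arm toward the camera and stores the impact point on a blocking hit.
; The trace end adds the spring arm's world scale, not location, to the scaled direction.
; The smoothing interpolation is unconnected and the helper functions are empty, so arm length never changes.
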(event `self.ReceiveTick`
  (params (DeltaSeconds :type "Float (single-precision)"))
  (`self.CameraCollision` 0.0))

(event `CameraCollision`
  (params (DeltaSeconds :type "Float (single-precision)"))
  (bind _outhit (`KismetSystemLibrary.SphereTraceSingle` (`SceneComponent.K2_GetComponentLocation` (`self.SpringArm`)) (+ (`SceneComponent.K2_GetComponentScale` (`self.SpringArm`)) (* (`KismetMathLibrary.Normal` (- (`SceneComponent.K2_GetComponentLocation` (`self.FollowCamera`)) (`SceneComponent.K2_GetComponentLocation` (`self.SpringArm`)))) (`self.DefaultSpringArmLength`))) (`self.ProbeRadius`) "TraceTypeQuery1" true (`|MakeArray` self :!type "Actor Object Reference")))
  (bind (_bblockinghit _binitialoverlap _time _distance _location _impactpoint) (`GameplayStatics.BreakHitResult` _outhit))
  (if _bblockinghit
    (bind _output_get (set `self.ImpactPoint` _impactpoint))))

(fn `CameraDistAdjust`)

(fn `GetInterpSpeed`)

(fn `UserConstructionScript`)