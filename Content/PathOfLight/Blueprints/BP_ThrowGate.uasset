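; BP_ThrowGate is a gate that opens when an actor tagged "Throw Key" overlaps its box trigger.
; The overlap unpauses the skeletal mesh, plays the gate animation once, destroys the key actor and increments the Gates counter on the player's bp_Character.
; DoorSequence is an empty event, and leftover ActorSequence, rotation and component-destruction nodes are disconnected and never run.
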(event `self.ReceiveBeginPlay`)

(event `DoorSequence`)

(event `self.Box.OnComponentBeginOverlap`
  (params (OverlappedComponent :type "PrimitiveComponent Object Reference") (OtherActor :type "Actor Object Reference") (OtherComp :type "PrimitiveComponent Object Reference") (OtherBodyIndex :type Integer) (bFromSweep :type Boolean) (SweepResult :type "HitResult Structure (by ref)"))
  (bind _skeletalmesh (`self.SkeletalMesh`))
  (if (`self.ActorHasTag` OtherActor "Throw Key")
    (set `SkeletalMeshComponent.bPauseAnims` false _skeletalmesh)
    (`SkeletalMeshComponent.PlayAnimation` _skeletalmesh "/Game/PathOfLight/Animations/ThrowGate/ThrowGateAnim.ThrowGateAnim" false)
    (`self.K2_DestroyActor` OtherActor)
    (bind _asbp_character (cast `/Game/PathOfLight/bp_Imports/bp_Character` (`GameplayStatics.GetPlayerPawn` 0)))
    (`/Engine/EditorBlueprintResources/StandardMacros.IncrementInt` (`/Game/PathOfLight/bp_Imports/bp_Character.Gates` _asbp_character))))

(fn `UserConstructionScript`)