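; BP_ThrowGateBroken is a two-door gate that is removed when an actor tagged "Throw Key" overlaps its Box.
; That overlap destroys both door components and the key actor.
; BeginPlay resets the doors' relative rotation and stops the ActorSequence.
; A separate DoorBreak event plays that sequence, but nothing in this graph calls it.
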(event `self.ReceiveBeginPlay`
  (`SceneComponent.K2_SetRelativeRotation` :`self` (`self.GateDoor2`))
  (`SceneComponent.K2_SetRelativeRotation` :`self` (`self.GateDoor1`))
  (`ActorSequenceComponent.StopSequence` (`self.ActorSequence`)))

(event `self.Box.OnComponentBeginOverlap`
  (params (OverlappedComponent :type "PrimitiveComponent Object Reference") (OtherActor :type "Actor Object Reference") (OtherComp :type "PrimitiveComponent Object Reference") (OtherBodyIndex :type Integer) (bFromSweep :type Boolean) (SweepResult :type "HitResult Structure (by ref)"))
  (if (`self.ActorHasTag` OtherActor "Throw Key")
    (`ActorComponent.K2_DestroyComponent` (`self.GateDoor1`))
    (`ActorComponent.K2_DestroyComponent` (`self.GateDoor2`))
    (`self.K2_DestroyActor` OtherActor)))

(event `DoorBreak`
  (`ActorSequenceComponent.PlaySequence` (`self.ActorSequence`)))

(fn `UserConstructionScript`)