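; BP_ThrowTutorialTrigger is a one-shot trigger that plays the ThrowScene cutscene when the character overlaps it, introducing the throw tutorial.
; During playback it disables input and swaps the HUD for a skip-cutscene widget; Tab or the gamepad right face button skips to the end.
; Finishing or skipping restores input, HUD and camera, spawns BP_tutorialthrow at a hardcoded transform, and shows a fade-in widget.
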(event `Key|Tab`
  (params (Key :type "Key Structure"))
  (:`Pressed`
    (if (`MovieSceneSequencePlayer.IsPlaying` (stale `self.Collision.OnComponentBeginOverlap` _returnvalue)) :!label _label
      (add `MovieSceneSequencePlayer.OnStop` (stale `self.Collision.OnComponentBeginOverlap` _returnvalue) (`|CreateDelegate` :!event `OnStop`))
      (`MovieSceneSequencePlayer.GoToEndAndStop` (stale `self.Collision.OnComponentBeginOverlap` _returnvalue)))))

(event `Key|Gamepad_FaceButton_Right`
  (params (Key :type "Key Structure"))
  (:`Pressed`
    (goto _label)))

(event `self.Collision.OnComponentBeginOverlap`
  (params (OverlappedComponent :type "PrimitiveComponent Object Reference") (OtherActor :type "Actor Object Reference") (OtherComp :type "PrimitiveComponent Object Reference") (OtherBodyIndex :type Integer) (bFromSweep :type Boolean) (SweepResult :type "HitResult Structure (by ref)"))
  (cast `/Game/PathOfLight/bp_Imports/bp_Character` OtherActor)
  (`/Engine/EditorBlueprintResources/StandardMacros.DoOnce` false
    (:`Completed`
      (bind (_outactor _returnvalue) (`LevelSequencePlayer.CreateLevelSequencePlayer` (`self.ThrowScene`)))
      (add `MovieSceneSequencePlayer.OnFinished` _returnvalue (`|CreateDelegate` :!event `OnFinished`))
      (`MovieSceneSequencePlayer.Play` _returnvalue)
      (`self.DisableInput` (`GameplayStatics.GetPlayerCharacter` 0) null)
      (bind _foundwidgets (`WidgetBlueprintLibrary.GetAllWidgetsOfClass` "/Game/PathOfLight/bp_Imports/HUD_UI.HUD_UI_C"))
      (bind _foundwidgets_2 (`WidgetBlueprintLibrary.GetAllWidgetsOfClass` "/Game/PathOfLight/UI/wbp_SkipCutscene.wbp_SkipCutscene_C"))
      (`Widget.SetVisibility` _foundwidgets_2 "Visible")
      (`Widget.SetVisibility` _foundwidgets "Hidden"))))

(event `OnFinished`
  (`self.EnableInput` (`GameplayStatics.GetPlayerCharacter` 0) null :!label _label_2)
  (`Widget.SetVisibility` (stale `self.Collision.OnComponentBeginOverlap` _foundwidgets) "Visible")
  (`Widget.SetVisibility` (stale `self.Collision.OnComponentBeginOverlap` _foundwidgets_2) "Hidden")
  (`|SpawnActorFromClass` "/Game/PathOfLight/Blueprints/Tutorial_PopUps/BP_tutorialthrow.BP_tutorialthrow_C" (`KismetMathLibrary.MakeTransform` (-9329.0 11851.0 -790.0) (struct) (17.684095 13.520599 1.202262)) "Undefined" "MultiplyWithRoot" null null)
  (bind _asbp_character (cast `/Game/PathOfLight/bp_Imports/bp_Character` (`GameplayStatics.GetPlayerCharacter` 0)))
  (`PlayerController.SetViewTargetWithBlend` (`GameplayStatics.GetPlayerController` 0) _asbp_character 0.0 "VTBlend_Linear" 0.0 false)
  (`CameraComponent.SetFieldOfView` (`/Game/PathOfLight/bp_Imports/bp_Character.CineCamera` _asbp_character) 75.0)
  (bind _returnvalue (`|CreateWidget` "/Game/PathOfLight/UI/FadeIn.FadeIn_C"))
  (bind _output_get (set `self.Fade` _returnvalue))
  (`UserWidget.AddToViewport` _output_get 0))

(event `OnStop`
  (goto _label_2))

(fn `UserConstructionScript`)