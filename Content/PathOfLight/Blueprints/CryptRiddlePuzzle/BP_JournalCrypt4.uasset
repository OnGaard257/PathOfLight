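; BP_JournalCrypt4 is the fourth journal pickup in the crypt riddle puzzle, letting the player toggle its journal view.
; A box overlap by bp_Character sets its Journal4Overlap flag, enables input on the actor and applies an outline overlay material to the mesh.
; Leaving the box clears the flag, disables input and removes the outline.
; The Journal4Interact event calls ToggleJournal4 on the player character, which handles the display.
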(event `Journal4Interact`
  (bind _asbp_character (cast `/Game/PathOfLight/bp_Imports/bp_Character` (`GameplayStatics.GetPlayerCharacter` 0)))
  (`/Game/PathOfLight/bp_Imports/bp_Character.ToggleJournal4` _asbp_character))

(event `self.Box.OnComponentBeginOverlap`
  (params (OverlappedComponent :type "PrimitiveComponent Object Reference") (OtherActor :type "Actor Object Reference") (OtherComp :type "PrimitiveComponent Object Reference") (OtherBodyIndex :type Integer) (bFromSweep :type Boolean) (SweepResult :type "HitResult Structure (by ref)"))
  (bind _asbp_character (cast `/Game/PathOfLight/bp_Imports/bp_Character` OtherActor))
  (set `/Game/PathOfLight/bp_Imports/bp_Character.Journal4Overlap?` true _asbp_character)
  (`self.EnableInput` (`GameplayStatics.GetPlayerController` 0))
  (`MeshComponent.SetOverlayMaterial` (`self.StaticMesh`) "/Game/PathOfLight/Materials/m_Outline_Inst.m_Outline_Inst"))

(event `self.Box.OnComponentEndOverlap`
  (params (OverlappedComponent :type "PrimitiveComponent Object Reference") (OtherActor :type "Actor Object Reference") (OtherComp :type "PrimitiveComponent Object Reference") (OtherBodyIndex :type Integer))
  (bind _asbp_character (cast `/Game/PathOfLight/bp_Imports/bp_Character` OtherActor))
  (set `/Game/PathOfLight/bp_Imports/bp_Character.Journal4Overlap?` false _asbp_character)
  (`self.DisableInput` (`GameplayStatics.GetPlayerController` 0))
  (`MeshComponent.SetOverlayMaterial` (`self.StaticMesh`) null))

(fn `UserConstructionScript`)