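; PuzzleValve1 is the first valve in the crypt riddle puzzle, which releases steam when the player turns it.
; Its collider flags the overlap on bp_Character, outlines the valve and enables input.
; Valve1Interact calls the character's Interact, then after a short delay sets RiddleCheck1 and runs the steam function.
; That function drives delayed steam visibility and a DoOnce-guarded positional sound from RiddleCheck1, switching both off when it is false.
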(event `self.ReceiveTick`
  (params (DeltaSeconds :type "Float (single-precision)")))

(event `SteamValve1Funtionality`
  (bind _steam (`self.Steam`))
  (`|ExecutionSequence`
    (:`then_0`
      (`KismetSystemLibrary.Delay` 0.2)
      (if (`self.Valve1Steam?`)
        (`SceneComponent.SetVisibility` _steam true false)
        (else
          (`SceneComponent.SetVisibility` _steam false false))))
    (:`then_1`
      (if (`self.RiddleCheck1`)
        (set `self.Valve1Steam?` true)
        (`/Engine/EditorBlueprintResources/StandardMacros.DoOnce` false :!label _label
          (:`Completed`
            (bind _returnvalue (`GameplayStatics.SpawnSoundAtLocation` "/Game/StarterContent/Audio/Steam01_Cue.Steam01_Cue" (`SceneComponent.K2_GetComponentLocation` (`self.sm_Door_pTorus5`)) (struct) 1.0 1.0 0.0 "/Game/PathOfLight/VFX/Fire_and_smoke/VFX-k/Steam.Steam" null))))
        (else
          (set `self.Valve1Steam?` false)
          (`ActorComponent.Deactivate` _returnvalue)
          (goto _label :!via `Reset`))))))

(event `Valve1Interact`
  (bind _asbp_character (cast `/Game/PathOfLight/bp_Imports/bp_Character` (`GameplayStatics.GetPlayerCharacter` 0)))
  (`/Game/PathOfLight/bp_Imports/bp_Character.Interact` _asbp_character)
  (`KismetSystemLibrary.Delay` 0.4)
  (set `self.RiddleCheck1` true)
  (`self.SteamValve1Funtionality`))

(event `self.PuzzleCollider1.OnComponentBeginOverlap`
  (params (OverlappedComponent :type "PrimitiveComponent Object Reference") (OtherActor :type "Actor Object Reference") (OtherComp :type "PrimitiveComponent Object Reference") (OtherBodyIndex :type Integer) (bFromSweep :type Boolean) (SweepResult :type "HitResult Structure (by ref)"))
  (bind _asbp_character (cast `/Game/PathOfLight/bp_Imports/bp_Character` OtherActor))
  (set `/Game/PathOfLight/bp_Imports/bp_Character.Valve1Overlap?` true _asbp_character)
  (`MeshComponent.SetOverlayMaterial` (`self.sm_Door_pTorus5`) "/Game/PathOfLight/Materials/m_Outline_Inst.m_Outline_Inst")
  (`self.EnableInput` (`GameplayStatics.GetPlayerController` 0)))

(event `self.PuzzleCollider1.OnComponentEndOverlap`
  (params (OverlappedComponent :type "PrimitiveComponent Object Reference") (OtherActor :type "Actor Object Reference") (OtherComp :type "PrimitiveComponent Object Reference") (OtherBodyIndex :type Integer))
  (bind _asbp_character (cast `/Game/PathOfLight/bp_Imports/bp_Character` OtherActor))
  (set `/Game/PathOfLight/bp_Imports/bp_Character.Valve1Overlap?` false _asbp_character)
  (`MeshComponent.SetOverlayMaterial` (`self.sm_Door_pTorus5`) null)
  (`self.DisableInput` (`GameplayStatics.GetPlayerController` 0)))

(fn `UserConstructionScript`)