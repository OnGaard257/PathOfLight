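; Second valve in the crypt riddle puzzle, which only turns on after the first valve's check has passed.
; Overlapping its box lets the character interact, setting RiddleCheck2 if PuzzleValve1, found by class lookup, has RiddleCheck1 set.
; Tick copies RiddleCheck2 into Valve2Steam and uses that to show or hide Steam2.
; Nodes that would clear RiddleCheck1 are unconnected, so they never run.
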(event `self.ReceiveTick`
  (params (DeltaSeconds :type "Float (single-precision)"))
  (bind _steam2 (`self.Steam2`))
  (`|ExecutionSequence`
    (:`then_0`
      (if (`self.Valve2Steam?`)
        (`SceneComponent.SetVisibility` _steam2 true false)
        (else
          (`SceneComponent.SetVisibility` _steam2 false false))))
    (:`then_1`
      (if (`self.RiddleCheck2`)
        (set `self.Valve2Steam?` true)
        (else
          (set `self.Valve2Steam?` false))))))

(event `EnhancedInput|/Game/PathOfLight/bp_Imports/ia_Interact`
  (params (ActionValue :type Boolean) (ElapsedSeconds :type "Float (double-precision)") (TriggeredSeconds :type "Float (double-precision)") (InputAction :type "InputAction Object Reference" :default "/Game/PathOfLight/bp_Imports/ia_Interact.ia_Interact"))
  (:`Triggered`
    (bind _returnvalue (`GameplayStatics.GetActorOfClass` "/Game/PathOfLight/Blueprints/CryptRiddlePuzzle/PuzzleValve1.PuzzleValve1_C"))
    (if (`/Game/PathOfLight/Blueprints/CryptRiddlePuzzle/PuzzleValve1.RiddleCheck1` _returnvalue)
      (set `self.RiddleCheck2` true))))

(event `self.Box.OnComponentBeginOverlap`
  (params (OverlappedComponent :type "PrimitiveComponent Object Reference") (OtherActor :type "Actor Object Reference") (OtherComp :type "PrimitiveComponent Object Reference") (OtherBodyIndex :type Integer) (bFromSweep :type Boolean) (SweepResult :type "HitResult Structure (by ref)"))
  (cast `/Game/PathOfLight/bp_Imports/bp_Character` OtherActor)
  (`self.EnableInput` (`GameplayStatics.GetPlayerController` 0)))

(event `self.Box.OnComponentEndOverlap`
  (params (OverlappedComponent :type "PrimitiveComponent Object Reference") (OtherActor :type "Actor Object Reference") (OtherComp :type "PrimitiveComponent Object Reference") (OtherBodyIndex :type Integer))
  (cast `/Game/PathOfLight/bp_Imports/bp_Character` OtherActor)
  (`self.DisableInput` (`GameplayStatics.GetPlayerController` 0)))

(fn `UserConstructionScript`)