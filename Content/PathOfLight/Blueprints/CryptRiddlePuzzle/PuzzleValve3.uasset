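; PuzzleValve3 is the third valve in the crypt riddle puzzle, accepting interaction only while the player character overlaps its box.
; On interact, it reads the check flags on PuzzleValve1 and PuzzleValve2, found by class lookup.
; If both are set, it sets RiddleCheck3 and spawns two attached Niagara steam effects.
; Otherwise it clears earlier valve flags, printing "Incorrect" only when the first valve's flag is unset.
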(event `EnhancedInput|/Game/PathOfLight/bp_Imports/ia_Interact`
  (params (ActionValue :type Boolean) (ElapsedSeconds :type "Float (double-precision)") (TriggeredSeconds :type "Float (double-precision)") (InputAction :type "InputAction Object Reference" :default "/Game/PathOfLight/bp_Imports/ia_Interact.ia_Interact"))
  (bind _sm_door_ptorus5 (`self.sm_Door_pTorus5`))
  (:`Triggered`
    (bind _returnvalue (`GameplayStatics.GetActorOfClass` "/Game/PathOfLight/Blueprints/CryptRiddlePuzzle/PuzzleValve1.PuzzleValve1_C"))
    (if (`/Game/PathOfLight/Blueprints/CryptRiddlePuzzle/PuzzleValve1.RiddleCheck1` _returnvalue)
      (bind _returnvalue_2 (`GameplayStatics.GetActorOfClass` "/Game/PathOfLight/Blueprints/CryptRiddlePuzzle/PuzzleValve2.PuzzleValve2_C"))
      (if (`/Game/PathOfLight/Blueprints/CryptRiddlePuzzle/PuzzleValve2.RiddleCheck2` _returnvalue_2)
        (set `self.RiddleCheck3` true)
        (`|ExecutionSequence`
          (:`then_0`
            (`NiagaraFunctionLibrary.SpawnSystemAttached` "/Game/PathOfLight/VFX/Fire_and_smoke/fx_StylizedSteam.fx_StylizedSteam" _sm_door_ptorus5 "None" (-135.0 -30.0 0.0) (struct :`Roll` -120.0) "KeepRelativeOffset"))
          (:`then_1`
            (`NiagaraFunctionLibrary.SpawnSystemAttached` "/Game/PathOfLight/VFX/Fire_and_smoke/fx_StylizedSteam.fx_StylizedSteam" _sm_door_ptorus5 "None" (45.0 -30.0 0.0) (struct :`Roll` -55.0) "KeepRelativeOffset")))
        (else
          (`|ExecutionSequence`
            (:`then_0`
              (set `/Game/PathOfLight/Blueprints/CryptRiddlePuzzle/PuzzleValve2.RiddleCheck2` false _returnvalue_2))
            (:`then_1`
              (set `/Game/PathOfLight/Blueprints/CryptRiddlePuzzle/PuzzleValve1.RiddleCheck1` false _returnvalue)))))
      (else
        (set `/Game/PathOfLight/Blueprints/CryptRiddlePuzzle/PuzzleValve1.RiddleCheck1` false _returnvalue)
        (`KismetSystemLibrary.PrintString` "Incorrect")))))

(event `self.Box.OnComponentBeginOverlap`
  (params (OverlappedComponent :type "PrimitiveComponent Object Reference") (OtherActor :type "Actor Object Reference") (OtherComp :type "PrimitiveComponent Object Reference") (OtherBodyIndex :type Integer) (bFromSweep :type Boolean) (SweepResult :type "HitResult Structure (by ref)"))
  (cast `/Game/PathOfLight/bp_Imports/bp_Character` OtherActor)
  (`self.EnableInput` (`GameplayStatics.GetPlayerController` 0)))

(event `self.Box.OnComponentEndOverlap`
  (params (OverlappedComponent :type "PrimitiveComponent Object Reference") (OtherActor :type "Actor Object Reference") (OtherComp :type "PrimitiveComponent Object Reference") (OtherBodyIndex :type Integer))
  (cast `/Game/PathOfLight/bp_Imports/bp_Character` OtherActor)
  (`self.DisableInput` (`GameplayStatics.GetPlayerController` 0)))

(fn `UserConstructionScript`)