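; Fourth and final valve in the crypt riddle's ordered steam valve puzzle, highlighted and usable while the player overlaps its box.
; On interaction it checks valves 1 to 3 in order, found by class lookup.
; If all are set, it turns on its own steam and calls DeleteSteam on the SteamBlocker.
; Otherwise it clears the checks up to the first unset valve and refreshes their steam.
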(event `SteamValve4Funtionality`
  (bind _steam4 (`self.Steam4`))
  (`|ExecutionSequence`
    (:`then_0`
      (`KismetSystemLibrary.Delay` 0.2)
      (if (`self.Valve4Steam?`)
        (`SceneComponent.SetVisibility` _steam4 true false)
        (else
          (`SceneComponent.SetVisibility` _steam4 false false))))
    (:`then_1`
      (if (`self.RiddleCheck4`)
        (set `self.Valve4Steam?` true)
        (`/Engine/EditorBlueprintResources/StandardMacros.DoOnce` false
          (:`Completed`
            (`GameplayStatics.SpawnSoundAtLocation` "/Game/StarterContent/Audio/Steam01_Cue.Steam01_Cue" (`SceneComponent.K2_GetComponentLocation` (`self.sm_Door_pTorus5`)) (struct) 0.3 1.0 0.0 "/Game/PathOfLight/VFX/Fire_and_smoke/VFX-k/Steam.Steam" null)))
        (else
          (set `self.Valve4Steam?` false))))))

(event `self.ReceiveTick`
  (params (DeltaSeconds :type "Float (single-precision)")))

(event `Valve4Interact`
  (bind _asbp_character (cast `/Game/PathOfLight/bp_Imports/bp_Character` (`GameplayStatics.GetPlayerCharacter` 0)))
  (`/Game/PathOfLight/bp_Imports/bp_Character.Interact` _asbp_character)
  (`KismetSystemLibrary.Delay` 0.4)
  (`GameplayStatics.PlaySound2D` "/Game/PathOfLight/Sounds/NickSFX/4-13/SFX_ValvePlace.SFX_ValvePlace" 0.6 1.0 0.0 null null)
  (bind _returnvalue (`GameplayStatics.GetActorOfClass` "/Game/PathOfLight/Blueprints/CryptRiddlePuzzle/PuzzleValve1.PuzzleValve1_C"))
  (if (`/Game/PathOfLight/Blueprints/CryptRiddlePuzzle/PuzzleValve1.RiddleCheck1` _returnvalue)
    (bind _returnvalue_2 (`GameplayStatics.GetActorOfClass` "/Game/PathOfLight/Blueprints/CryptRiddlePuzzle/PuzzleValve2.PuzzleValve2_C"))
    (if (`/Game/PathOfLight/Blueprints/CryptRiddlePuzzle/PuzzleValve2.RiddleCheck2` _returnvalue_2)
      (bind _returnvalue_3 (`GameplayStatics.GetActorOfClass` "/Game/PathOfLight/Blueprints/CryptRiddlePuzzle/PuzzleValve3.PuzzleValve3_C"))
      (if (`/Game/PathOfLight/Blueprints/CryptRiddlePuzzle/PuzzleValve3.RiddleCheck3` _returnvalue_3)
        (set `self.RiddleCheck4` true)
        (`self.SteamValve4Funtionality`)
        (bind _returnvalue_4 (`GameplayStatics.GetActorOfClass` "/Game/PathOfLight/Blueprints/CryptRiddlePuzzle/SteamBlocker.SteamBlocker_C"))
        (`/Game/PathOfLight/Blueprints/CryptRiddlePuzzle/SteamBlocker.DeleteSteam` _returnvalue_4)
        (else
          (`|ExecutionSequence`
            (:`then_0`
              (set `/Game/PathOfLight/Blueprints/CryptRiddlePuzzle/PuzzleValve2.RiddleCheck2` false _returnvalue_2)
              (`/Game/PathOfLight/Blueprints/CryptRiddlePuzzle/PuzzleValve2.SteamValve2Funtionality` _returnvalue_2))
            (:`then_1`
              (set `/Game/PathOfLight/Blueprints/CryptRiddlePuzzle/PuzzleValve1.RiddleCheck1` false _returnvalue)
              (`/Game/PathOfLight/Blueprints/CryptRiddlePuzzle/PuzzleValve1.SteamValve1Funtionality` _returnvalue))
            (:`then_2`
              (set `/Game/PathOfLight/Blueprints/CryptRiddlePuzzle/PuzzleValve3.RiddleCheck3` false _returnvalue_3)
              (`/Game/PathOfLight/Blueprints/CryptRiddlePuzzle/PuzzleValve3.Valve3Funtionality` _returnvalue_3)))))
      (else
        (`|ExecutionSequence`
          (:`then_0`
            (set `/Game/PathOfLight/Blueprints/CryptRiddlePuzzle/PuzzleValve2.RiddleCheck2` false _returnvalue_2)
            (`/Game/PathOfLight/Blueprints/CryptRiddlePuzzle/PuzzleValve2.SteamValve2Funtionality` _returnvalue_2))
          (:`then_1`
            (set `/Game/PathOfLight/Blueprints/CryptRiddlePuzzle/PuzzleValve1.RiddleCheck1` false _returnvalue)
            (`/Game/PathOfLight/Blueprints/CryptRiddlePuzzle/PuzzleValve1.SteamValve1Funtionality` _returnvalue)))))
    (else
      (set `/Game/PathOfLight/Blueprints/CryptRiddlePuzzle/PuzzleValve1.RiddleCheck1` false _returnvalue)
      (`/Game/PathOfLight/Blueprints/CryptRiddlePuzzle/PuzzleValve1.SteamValve1Funtionality` _returnvalue))))

(event `self.Box_0.OnComponentBeginOverlap`
  (params (OverlappedComponent :type "PrimitiveComponent Object Reference") (OtherActor :type "Actor Object Reference") (OtherComp :type "PrimitiveComponent Object Reference") (OtherBodyIndex :type Integer) (bFromSweep :type Boolean) (SweepResult :type "HitResult Structure (by ref)"))
  (bind _asbp_character (cast `/Game/PathOfLight/bp_Imports/bp_Character` OtherActor))
  (set `/Game/PathOfLight/bp_Imports/bp_Character.Valve4Overlap?` true _asbp_character)
  (`self.EnableInput` (`GameplayStatics.GetPlayerController` 0))
  (`MeshComponent.SetOverlayMaterial` (`self.sm_Door_pTorus5`) "/Game/PathOfLight/Materials/m_Outline_Inst.m_Outline_Inst"))

(event `self.Box_0.OnComponentEndOverlap`
  (params (OverlappedComponent :type "PrimitiveComponent Object Reference") (OtherActor :type "Actor Object Reference") (OtherComp :type "PrimitiveComponent Object Reference") (OtherBodyIndex :type Integer))
  (bind _asbp_character (cast `/Game/PathOfLight/bp_Imports/bp_Character` OtherActor))
  (set `/Game/PathOfLight/bp_Imports/bp_Character.Valve4Overlap?` false _asbp_character)
  (`self.DisableInput` (`GameplayStatics.GetPlayerController` 0))
  (`MeshComponent.SetOverlayMaterial` (`self.sm_Door_pTorus5`) null))

(event `/Game/PathOfLight/LD_Prototyping/JavonW/BPI_Interface.Interaction`
  (`self.Valve4Interact`))

(fn `UserConstructionScript`)