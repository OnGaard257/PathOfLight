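; SteamBlocker is the steam obstacle in the crypt riddle puzzle that removes itself once the puzzle's valve checks pass.
; Its DeleteSteam event finds PuzzleValve1 through PuzzleValve4 with GetActorOfClass and tests each one's RiddleCheck flag in nested branches.
; The actor is destroyed only when all four flags are true at the moment of the call, as there is no polling.
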(event `DeleteSteam`
  (bind _returnvalue (`GameplayStatics.GetActorOfClass` "/Game/PathOfLight/Blueprints/CryptRiddlePuzzle/PuzzleValve1.PuzzleValve1_C"))
  (if (`/Game/PathOfLight/Blueprints/CryptRiddlePuzzle/PuzzleValve1.RiddleCheck1` _returnvalue)
    (bind _returnvalue_2 (`GameplayStatics.GetActorOfClass` "/Game/PathOfLight/Blueprints/CryptRiddlePuzzle/PuzzleValve2.PuzzleValve2_C"))
    (if (`/Game/PathOfLight/Blueprints/CryptRiddlePuzzle/PuzzleValve2.RiddleCheck2` _returnvalue_2)
      (bind _returnvalue_3 (`GameplayStatics.GetActorOfClass` "/Game/PathOfLight/Blueprints/CryptRiddlePuzzle/PuzzleValve3.PuzzleValve3_C"))
      (if (`/Game/PathOfLight/Blueprints/CryptRiddlePuzzle/PuzzleValve3.RiddleCheck3` _returnvalue_3)
        (bind _returnvalue_4 (`GameplayStatics.GetActorOfClass` "/Game/PathOfLight/Blueprints/CryptRiddlePuzzle/PuzzleValve4.PuzzleValve4_C"))
        (if (`/Game/PathOfLight/Blueprints/CryptRiddlePuzzle/PuzzleValve4.RiddleCheck4` _returnvalue_4)
          (`|ExecutionSequence`
            (:`then_0`
              (`self.K2_DestroyActor`))))))))

(fn `UserConstructionScript`)