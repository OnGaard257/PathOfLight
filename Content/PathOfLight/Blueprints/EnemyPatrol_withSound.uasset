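; Enemy character that patrols, chases seen pawns, investigates sensed stimuli and ends the game when its collision touches the player.
; AIMoveTo loops through four patrol points, while the random-patrol variant is never started.
; PawnSensing triggers chases with retriggerable-delay returns to patrol, and AIPerception sends it to the player's stimulus location before resuming.
; Contact destroys the player and shows the game-over widget, while stun-object hits briefly disable movement.
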(event `Enemy Random Patrol`
  ;[1 1 1] Random Enemy Patrol (Michael F.)
  (set `CharacterMovementComponent.MaxWalkSpeed` 300.0 (`self.CharacterMovement`))
  (bind _randomlocation (`NavigationSystemV1.K2_GetRandomLocationInNavigableRadius` (`self.K2_GetActorLocation`) 2000.0 null null))
  (`|AIMoveTo` self _randomlocation null
    (:`OnSuccess`
      (`KismetSystemLibrary.Delay` 0.5)
      (`self.Enemy Random Patrol`))))

(event `self.ReceiveBeginPlay`
  (`self.EnemyPatrol`)
  (`GameplayStatics.PlaySoundAtLocation` "/Game/PathOfLight/Sounds/Monster_Growl.Monster_Growl" (0.0 0.0 0.0) (struct) 1.0 1.0 0.0 null null null null))

(event `EnemyPatrol`
  ;[1 1 1] Enemy Movement with Patrol Points
  (set `CharacterMovementComponent.MaxWalkSpeed` 400.0 (`self.CharacterMovement`))
  (`|AIMoveTo` self (`self.Patrol1`) null
    (:`OnSuccess`
      (`|AIMoveTo` self (`self.Patrol2`) null
        (:`OnSuccess`
          (`|AIMoveTo` self (`self.Patrol3`) null
            (:`OnSuccess`
              (`|AIMoveTo` self (`self.Patrol4`) null
                (:`OnSuccess`
                  (`self.EnemyPatrol`))))))))))

(event `self.GameOverCollision.OnComponentBeginOverlap`
  (params (OverlappedComponent :type "PrimitiveComponent Object Reference") (OtherActor :type "Actor Object Reference") (OtherComp :type "PrimitiveComponent Object Reference") (OtherBodyIndex :type Integer) (bFromSweep :type Boolean) (SweepResult :type "HitResult Structure (by ref)"))
  (bind _asbp_character (cast `/Game/PathOfLight/bp_Imports/bp_Character` OtherActor))
  (`self.K2_DestroyActor` _asbp_character)
  (bind _returnvalue (`|CreateWidget` "/Game/PathOfLight/Blueprints/bp_Game_Over.bp_Game_Over_C"))
  (`UserWidget.AddToViewport` _returnvalue 0)
  (set `PlayerController.bShowMouseCursor` true (`GameplayStatics.GetPlayerController` 0)))

(event `self.PawnSensing.OnSeePawn`
  (params (Pawn :type "Pawn Object Reference"))
  ;[1 1 1] Pawn Sensing
  (set `CharacterMovementComponent.MaxWalkSpeed` 350.0 (`self.CharacterMovement`))
  (`|AIMoveTo` self (0.0 0.0 0.0) Pawn
    (:`then`
      (`KismetSystemLibrary.RetriggerableDelay` 2.0)
      (`self.EnemyPatrol`))))

(event `self.AIPerception.OnTargetPerceptionUpdated`
  (params (Actor :type "Actor Object Reference") (Stimulus :type "AIStimulus Structure"))
  (bind (_age _expirationage _strength _stimuluslocation _receiverlocation _tag _bsuccessfullysensed) (break `AIStimulus` Stimulus))
  ;[1 1 1] AI Sound Interaction (Prototype) (Michael F.)
  ;;[1 1 1] AI Hears the Object Nearby
  (cast `/Game/PathOfLight/bp_Imports/bp_Character` Actor)
  (if _bsuccessfullysensed
    (set `self.Investigating?` true)
    (`|AIMoveTo` self _stimuluslocation null
      (:`OnSuccess`
        (`KismetSystemLibrary.Delay` 3.0)
        (`self.EnemyPatrol`)))))

(event `self.ReceiveHit`
  (params (MyComp :type "PrimitiveComponent Object Reference") (Other :type "Actor Object Reference") (OtherComp :type "PrimitiveComponent Object Reference") (bSelfMoved :type Boolean) (HitLocation :type "Vector Structure") (HitNormal :type "Vector Structure") (NormalImpulse :type "Vector Structure") (Hit :type "HitResult Structure (by ref)"))
  ;[1 1 1] Stun Interaction
  (bind _asbp_stun (cast `/Game/PathOfLight/Blueprints/bp_Stun` Other))
  (`self.K2_DestroyActor` _asbp_stun)
  (`CharacterMovementComponent.DisableMovement` (`self.CharacterMovement`))
  (`KismetSystemLibrary.Delay` 2.0)
  (`CharacterMovementComponent.SetMovementMode` (`self.CharacterMovement`) "MOVE_Walking" 0))

(fn `UserConstructionScript`)