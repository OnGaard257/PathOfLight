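; Blind enemy character that patrols between two points and hunts the player by AI hearing.
; Hearing updates from an uncrouched player build a detection counter; past a threshold, a looping locate mode decays it, triggering a chase at maximum or resuming patrol when low.
; SoundStun halts movement and disables hearing temporarily, then resumes patrol.
; Random roaming and instant investigation are left unhooked.
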(event `Sound Stun`
  ;[1 1 1] Sound Stun Mechanic
  (`AIPerceptionComponent.SetSenseEnabled` (`self.AIPerception (Blind Enemy Hearing)`) "/Script/AIModule.AISense_Hearing" false)
  (`MovementComponent.StopMovementImmediately` (`self.CharacterMovement`))
  (`NavMovementComponent.StopActiveMovement` (`self.CharacterMovement`))
  (set `self.ChasingMode` false)
  (`KismetSystemLibrary.PrintString` "Stunned")
  (`KismetSystemLibrary.Delay` 6.0)
  (`self.PatrolPathing`)
  (`AIPerceptionComponent.SetSenseEnabled` (`self.AIPerception (Blind Enemy Hearing)`) "/Script/AIModule.AISense_Hearing" true)
  (set `self.HearingDetection` 0))

(event `self.ReceiveBeginPlay`
  ;[1 1 1] Patrol Path
  (`self.PatrolPathing`))

(event `PatrolPathing`
  ;[1 1 1] Patrol Path
  (`|AIMoveTo` self (`self.Patrol Point_1`) null
    (:`OnSuccess`
      (`KismetSystemLibrary.Delay` 2.0)
      (`|AIMoveTo` self (`self.Patrol Point_2`) null
        (:`OnSuccess`
          (`KismetSystemLibrary.Delay` 2.0)
          (`self.PatrolPathing`))))))

(event `ChasePlayer`
  ;[1 1 1] Chasing Event Node
  (set `self.ChasingMode` true)
  (set `CharacterMovementComponent.MaxWalkSpeed` 500.0 (`self.CharacterMovement`))
  (bind _asbp_character (cast `/Game/PathOfLight/bp_Imports/bp_Character` (`GameplayStatics.GetPlayerCharacter` 0)))
  (`|AIMoveTo` self (`self.K2_GetActorLocation` _asbp_character) _asbp_character
    (:`OnSuccess`
      (`self.ChasePlayer`))))

(event `Random Blind Roam`
  ;[1 1 1] Random Movement for Blind Enemy AI
  (set `CharacterMovementComponent.MaxWalkSpeed` 500.0 (`self.CharacterMovement`))
  (`|AIMoveTo` self (`NavigationSystemV1.K2_GetRandomReachablePointInRadius` (`self.K2_GetActorLocation`) 1500.0 null null) null
    (:`OnSuccess`
      (`KismetSystemLibrary.Delay` (`KismetMathLibrary.RandomFloatInRange` 1.0 5.0))
      (if (not (`self.Investigating`))
        (`self.Random Blind Roam` :!label _label)))
    (:`OnFail`
      (goto _label))))

(event `self.ReceiveTick`
  (params (DeltaSeconds :type "Float (single-precision)")))

(event `self.AIPerception (Blind Enemy Hearing).OnTargetPerceptionUpdated`
  (params (Actor :type "Actor Object Reference") (Stimulus :type "AIStimulus Structure"))
  (bind _hearingdetection (`self.HearingDetection`))
  ;[1 1 1] Active Hearing (Build Up)
  (bind _asbp_character (cast `/Game/PathOfLight/bp_Imports/bp_Character` Actor))
  (if (not (`/Game/PathOfLight/bp_Imports/bp_Character.Crouched` _asbp_character))
    (`KismetSystemLibrary.Delay` 0.25)
    (bind _result (`/Engine/EditorBlueprintResources/StandardMacros.IncrementInt` _hearingdetection)
      (:`  `
        (if (>= _hearingdetection 5)
          (`self.LocaterMode`))))))

(event `LocaterMode`
  ;[1 1 1] Echo Locate Mode
  (set `self.Locating` true)
  (`KismetSystemLibrary.Delay` 0.75)
  (if (>= (`self.HearingDetection`) 10)
    (set `self.HearingDetection` 10)
    (`self.ChasePlayer`)
    (else
      (bind _result (`/Engine/EditorBlueprintResources/StandardMacros.DecrementInt` (`self.HearingDetection`))
        (:`  `
          (bind _output_get (set `self.HearingDetection` (`KismetMathLibrary.Clamp` _result 0 10)))
          (if (<= (`self.HearingDetection`) 2)
            (`self.PatrolPathing`)
            (set `self.HearingDetection` 0)
            (set `self.Locating` false)
            (else
              (`self.LocaterMode`))))))))

(fn `UserConstructionScript`)