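; GearMech_B is a gear mechanism whose five gears spin in two opposing groups once started.
; GearWallTurn pitches BGear, BGear3 and BGear4 one way, while GearV2WallTurn pitches BGear1 and BGear2 the other.
; Each custom event loops endlessly by re-calling itself after a short Delay, adding delta seconds to a fixed step rather than scaling it.
; Nothing in this Blueprint calls either event initially.
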(event `GearWallTurn`
  (`SceneComponent.K2_AddLocalRotation` (`self.B_Gear`) (`KismetMathLibrary.MakeRotator` 0.0 (+ (`GameplayStatics.GetWorldDeltaSeconds`) 1.0)) false false)
  (`SceneComponent.K2_AddLocalRotation` (`self.B_Gear3`) (`KismetMathLibrary.MakeRotator` 0.0 (+ (`GameplayStatics.GetWorldDeltaSeconds`) 1.0)) false false)
  (`SceneComponent.K2_AddLocalRotation` (`self.B_Gear4`) (`KismetMathLibrary.MakeRotator` 0.0 (+ (`GameplayStatics.GetWorldDeltaSeconds`) 1.0)) false false)
  (`KismetSystemLibrary.Delay` 0.01)
  (`self.GearWallTurn`))

(event `GearV2WallTurn`
  (`SceneComponent.K2_AddLocalRotation` (`self.B_Gear1`) (`KismetMathLibrary.MakeRotator` 0.0 (+ (`GameplayStatics.GetWorldDeltaSeconds`) -1.0)) false false)
  (`SceneComponent.K2_AddLocalRotation` (`self.B_Gear2`) (`KismetMathLibrary.MakeRotator` 0.0 (+ (`GameplayStatics.GetWorldDeltaSeconds`) -1.0)) false false)
  (`KismetSystemLibrary.Delay` 0.01)
  (`self.GearV2WallTurn`))

(fn `UserConstructionScript`)