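; GearMech_Y3 is a gear mechanism that spins five gear components around their pitch axis once started.
; GearWallTurn turns three gears one way and GearV2WallTurn turns two the opposite way; nothing in this graph calls either initially.
; Each event re-calls itself after a short Delay instead of using Tick, adding frame delta to a fixed step.
; GearWallTurn also spawns an attached, attenuated running-gear sound once via DoOnce.
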(event `GearWallTurn`
  (`SceneComponent.K2_AddLocalRotation` (`self.Y_Gear`) (`KismetMathLibrary.MakeRotator` 0.0 (+ (`GameplayStatics.GetWorldDeltaSeconds`) -1.0)) false false)
  (`SceneComponent.K2_AddLocalRotation` (`self.Y_Gear3`) (`KismetMathLibrary.MakeRotator` 0.0 (+ (`GameplayStatics.GetWorldDeltaSeconds`) -1.0)) false false)
  (`SceneComponent.K2_AddLocalRotation` (`self.Y_Gear4`) (`KismetMathLibrary.MakeRotator` 0.0 (+ (`GameplayStatics.GetWorldDeltaSeconds`) -1.0)) false false)
  (`KismetSystemLibrary.Delay` 0.01)
  (`self.GearWallTurn`)
  (`/Engine/EditorBlueprintResources/StandardMacros.DoOnce` false
    (:`Completed`
      (`GameplayStatics.SpawnSoundAttached` "/Game/PathOfLight/Sounds/running-gear-6403.running-gear-6403" (`self.DefaultSceneRoot`) "None" (0.0 0.0 0.0) (struct) "KeepRelativeOffset" false 1.0 1.0 0.0 "/Game/PathOfLight/VFX/Fire_and_smoke/VFX-k/Gears.Gears" null))))

(event `GearV2WallTurn`
  (`SceneComponent.K2_AddLocalRotation` (`self.Y_Gear1`) (`KismetMathLibrary.MakeRotator` 0.0 (+ (`GameplayStatics.GetWorldDeltaSeconds`) 1.0)) false false)
  (`SceneComponent.K2_AddLocalRotation` (`self.Y_Gear2`) (`KismetMathLibrary.MakeRotator` 0.0 (+ (`GameplayStatics.GetWorldDeltaSeconds`) 1.0)) false false)
  (`KismetSystemLibrary.Delay` 0.01)
  (`self.GearV2WallTurn`))

(fn `UserConstructionScript`)