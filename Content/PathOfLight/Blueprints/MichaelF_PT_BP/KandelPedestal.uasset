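; Statue-head puzzle pedestal for which the Kandel head is the correct piece.
; An overlap sphere toggles the outline and gates interact input, which passes through a FlipFlop with only A wired.
; Interacting spawns the head matching the character's PickupItem at the socket and clears the carried item.
; Kandel's head also attaches, plays a sound, increments PedestalStatue's CorrectHeads, calls PuzzleComplete and moves the pedestal along a timeline.
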(event `Move Down`
  (bind (_direction _y_position) (`Timeline|Timeline`)
    (:`Update`
      (bind _returnvalue_location (`KismetMathLibrary.BreakTransform` (`KismetMathLibrary.TLerp` (`self.Start Pos`) (`self.End Pos`) _y_position)))
      (`SceneComponent.K2_SetRelativeLocation` (`self.Pedestal`) _returnvalue_location false false))))

(event `self.ReceiveBeginPlay`
  (`self.EnableInput` (`GameplayStatics.GetPlayerController` 0)))

(event `EnhancedInput|/Game/PathOfLight/bp_Imports/ia_Interact`
  (params (ActionValue :type Boolean) (ElapsedSeconds :type "Float (double-precision)") (TriggeredSeconds :type "Float (double-precision)") (InputAction :type "InputAction Object Reference" :default "/Game/PathOfLight/bp_Imports/ia_Interact.ia_Interact"))
  (:`Triggered`
    (bind _asbp_character (cast `/Game/PathOfLight/bp_Imports/bp_Character` (`GameplayStatics.GetPlayerCharacter` 0)))
    (`/Engine/EditorBlueprintResources/StandardMacros.Gate` true :!label _label
      (:`Exit`
        (`/Engine/EditorBlueprintResources/StandardMacros.FlipFlop`
          (:`A`
            (bind _pickupitem_ (`/Game/PathOfLight/bp_Imports/bp_Character.PickupItem#` _asbp_character))
            (if (== _pickupitem_ 1)
              (`|SpawnActorFromClass` "/Game/PathOfLight/Blueprints/MichaelF_PT_BP/StatueHead_Otto_1.StatueHead_Otto_1_C" (`SceneComponent.K2_GetComponentToWorld` (`self.Socket`)) "Undefined" "MultiplyWithRoot" null null)
              (set `/Game/PathOfLight/bp_Imports/bp_Character.PickupItem#` 0 _asbp_character)
              (`SceneComponent.SetVisibility` (`/Game/PathOfLight/bp_Imports/bp_Character.Otto` _asbp_character) false false)
              (elif (== _pickupitem_ 2)
                (`|SpawnActorFromClass` "/Game/PathOfLight/Blueprints/MichaelF_PT_BP/StatueHead_Luxx_2.StatueHead_Luxx_2_C" (`SceneComponent.K2_GetComponentToWorld` (`self.Socket`)) "Undefined" "MultiplyWithRoot" null null)
                (set `/Game/PathOfLight/bp_Imports/bp_Character.PickupItem#` 0 _asbp_character)
                (`SceneComponent.SetVisibility` (`/Game/PathOfLight/bp_Imports/bp_Character.Luxx` _asbp_character) false false)
                (elif (== _pickupitem_ 3)
                  (`|SpawnActorFromClass` "/Game/PathOfLight/Blueprints/MichaelF_PT_BP/StatueHead_Solara_3.StatueHead_Solara_3_C" (`SceneComponent.K2_GetComponentToWorld` (`self.Socket`)) "Undefined" "MultiplyWithRoot" null null)
                  (set `/Game/PathOfLight/bp_Imports/bp_Character.PickupItem#` 0 _asbp_character)
                  (`SceneComponent.SetVisibility` (`/Game/PathOfLight/bp_Imports/bp_Character.Solara` _asbp_character) false false)
                  (elif (== _pickupitem_ 4)
                    (bind _returnvalue (`|SpawnActorFromClass` "/Game/PathOfLight/Blueprints/MichaelF_PT_BP/StatueHead_Kandel_4.StatueHead_Kandel_4_C" (`SceneComponent.K2_GetComponentToWorld` (`self.Socket`)) "Undefined" "MultiplyWithRoot" null null))
                    (`self.K2_AttachToComponent` _returnvalue (`self.Socket`) "None" "KeepWorld" "KeepWorld" "KeepWorld" true)
                    (set `/Game/PathOfLight/bp_Imports/bp_Character.PickupItem#` 0 _asbp_character)
                    (`SceneComponent.SetVisibility` (`/Game/PathOfLight/bp_Imports/bp_Character.Kandel` _asbp_character) false false)
                    (`GameplayStatics.PlaySound2D` "/Game/PathOfLight/Sounds/ColeSFX/StoneRotate.StoneRotate" 0.8 1.2 0.0 null null)
                    (`/Game/PathOfLight/Blueprints/MichaelF_PT_BP/StatueHead_Kandel_4.Yes` _returnvalue)
                    (bind _returnvalue_2 (`GameplayStatics.GetActorOfClass` "/Game/PathOfLight/Blueprints/MichaelF_PT_BP/PedestalStatue.PedestalStatue_C"))
                    (bind _output_get (set `/Game/PathOfLight/Blueprints/MichaelF_PT_BP/PedestalStatue.CorrectHeads` (+ (`/Game/PathOfLight/Blueprints/MichaelF_PT_BP/PedestalStatue.CorrectHeads` _returnvalue_2) 1) _returnvalue_2))
                    (`KismetSystemLibrary.PrintString` (`KismetStringLibrary.Conv_IntToString` _output_get))
                    (`/Game/PathOfLight/Blueprints/MichaelF_PT_BP/PedestalStatue.PuzzleComplete` _returnvalue_2)
                    (`self.Move Down`)))))))))))

(event `self.Interact Sphere.OnComponentBeginOverlap`
  (params (OverlappedComponent :type "PrimitiveComponent Object Reference") (OtherActor :type "Actor Object Reference") (OtherComp :type "PrimitiveComponent Object Reference") (OtherBodyIndex :type Integer) (bFromSweep :type Boolean) (SweepResult :type "HitResult Structure (by ref)"))
  (cast `/Game/PathOfLight/bp_Imports/bp_Character` OtherActor)
  (`MeshComponent.SetOverlayMaterial` (`self.Pedestal`) "/Game/PathOfLight/Materials/m_Outline_Inst.m_Outline_Inst")
  (goto _label :!via `Open`))

(event `self.Interact Sphere.OnComponentEndOverlap`
  (params (OverlappedComponent :type "PrimitiveComponent Object Reference") (OtherActor :type "Actor Object Reference") (OtherComp :type "PrimitiveComponent Object Reference") (OtherBodyIndex :type Integer))
  (cast `/Game/PathOfLight/bp_Imports/bp_Character` OtherActor)
  (`MeshComponent.SetOverlayMaterial` (`self.Pedestal`) null)
  (goto _label :!via `Close`))

(fn `UserConstructionScript`)