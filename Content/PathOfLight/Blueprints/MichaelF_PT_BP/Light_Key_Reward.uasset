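; Light Key Reward is a puzzle reward pedestal that spawns a light key pickup attached to its socket on BeginPlay.
; StatueProgress counts correct statues; at four it plays sounds and runs a timeline that lerps the pedestal to a new location.
; It also fires the OnGearsSolved dispatcher and opens the crypt door, found by class lookup.
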(event `self.ReceiveBeginPlay`
  ;[1 1 1] Spawns Light Orb
  (bind _returnvalue (`|SpawnActorFromClass` "/Game/PathOfLight/bp_Imports/BP_LightKey_Pickup.BP_LightKey_Pickup_C" (`SceneComponent.K2_GetComponentToWorld` (`self.Socket`)) "Undefined" "MultiplyWithRoot" null null))
  (set `self.CorrectStatues` 0)
  (`self.K2_AttachToComponent` _returnvalue (`self.Socket`) "None" "KeepWorld" "KeepWorld" "KeepWorld" true))

(event `StatueProgress`
  ;[1 1 1] Increment Progress towards Light Key Reward
  (bind _result (`/Engine/EditorBlueprintResources/StandardMacros.IncrementInt` (`self.CorrectStatues`))
    (:`  `
      (bind _output_get (set `self.CorrectStatues` _result))
      (if (== _output_get 4)
        (`GameplayStatics.PlaySound2D` "/Game/PathOfLight/Sounds/NickSFX/SFX_GetPower.SFX_GetPower" 0.6 1.0 0.0 null null)
        (`|ExecutionSequence`
          (:`then_0`
            (bind (_direction _descender) (`Timeline|Timeline`)
              (:`Update`
                (bind _returnvalue_location (`KismetMathLibrary.BreakTransform` (`KismetMathLibrary.TLerp` (`self.Current Location`) (`self.New Location`) _descender)))
                (`SceneComponent.K2_SetRelativeTransform` (`self.Pedestal`) (`KismetMathLibrary.MakeTransform` _returnvalue_location (struct) (`self.Current Scale`)) false false))))
          (:`then_1`
            (`self.OnGearsSolved`)
            (bind _returnvalue (`GameplayStatics.GetActorOfClass` "/Game/PathOfLight/Blueprints/MichaelF_PT_BP/bp_LCryptDoor.bp_LCryptDoor_C"))
            (`/Game/PathOfLight/Blueprints/MichaelF_PT_BP/bp_LCryptDoor.Door Open` _returnvalue))
          (:`then_2`
            (`/Engine/EditorBlueprintResources/StandardMacros.DoOnce` false
              (:`Completed`
                (`GameplayStatics.PlaySound2D` "/Game/PathOfLight/Sounds/ColeSFX/StoneRotate.StoneRotate" 2.0 1.3 0.0 null null)))))))))

(fn `UserConstructionScript`)