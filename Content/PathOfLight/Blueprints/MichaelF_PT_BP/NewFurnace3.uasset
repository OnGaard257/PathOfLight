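; A furnace actor whose rect and point lights switch between lit and dark.
; BeginPlay starts it unlit, and the ToggleFurnace event flips FurnaceLit and sets both light intensities to match.
; Player interaction, outline highlighting, coal and fuel counting, and opening the furnace door at three fueled furnaces remain only as disconnected logic; their event handlers are empty.
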(event `self.ReceiveBeginPlay`
  (set `self.FurnaceLit` false)
  (`LightComponent.SetIntensity` (`self.RectLight`) 0.0)
  (`LightComponent.SetIntensity` (`self.PointLight`) 0.0))

(event `ToggleFurnace`
  (if (`self.FurnaceLit`)
    (set `self.FurnaceLit` false)
    (`LightComponent.SetIntensity` (`self.RectLight`) 0.0)
    (`LightComponent.SetIntensity` (`self.PointLight`) 0.0)
    (else
      (set `self.FurnaceLit` true)
      (`LightComponent.SetIntensity` (`self.RectLight`) 30.0)
      (`LightComponent.SetIntensity` (`self.PointLight`) 15.0))))

(event `FuelComplete`
  ;[1 1 1] When all Three Furnaces have been fueled
)

(event `EnhancedInput|/Game/PathOfLight/bp_Imports/ia_Interact`
  (params (ActionValue :type Boolean) (ElapsedSeconds :type "Float (double-precision)") (TriggeredSeconds :type "Float (double-precision)") (InputAction :type "InputAction Object Reference" :default "/Game/PathOfLight/bp_Imports/ia_Interact.ia_Interact"))
  ;[1 1 1] Player Interaction Condition and Visuals
)

(event `self.Interact_Box.OnComponentBeginOverlap`
  (params (OverlappedComponent :type "PrimitiveComponent Object Reference") (OtherActor :type "Actor Object Reference") (OtherComp :type "PrimitiveComponent Object Reference") (OtherBodyIndex :type Integer) (bFromSweep :type Boolean) (SweepResult :type "HitResult Structure (by ref)"))
  ;[1 1 1] Player Interaction Condition and Visuals
)

(event `self.Interact_Box.OnComponentEndOverlap`
  (params (OverlappedComponent :type "PrimitiveComponent Object Reference") (OtherActor :type "Actor Object Reference") (OtherComp :type "PrimitiveComponent Object Reference") (OtherBodyIndex :type Integer))
  ;[1 1 1] Player Interaction Condition and Visuals
)

(fn `UserConstructionScript`)