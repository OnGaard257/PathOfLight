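; Furnace actor that starts unlit and switches between lit and unlit through a ToggleFurnace event.
; Toggling sets both lights' intensity, smoke visibility and the volume of a looping sound spawned at BeginPlay, with ignite and extinguish one-shots and short delays.
; Interaction, outline and three-furnace fuel logic that would open the furnace door is disconnected, leaving those events empty.
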(event `self.ReceiveBeginPlay`
  (set `self.FurnaceLit` false)
  (`LightComponent.SetIntensity` (`self.RectLight`) 0.0)
  (`LightComponent.SetIntensity` (`self.PointLight`) 0.0)
  (`SceneComponent.SetVisibility` (`self.Smoke2`) false false)
  (`SceneComponent.SetVisibility` (`self.Smoke`) false false)
  (bind _returnvalue (`GameplayStatics.SpawnSoundAtLocation` "/Game/PathOfLight/Sounds/NickSFX/4-7/SFX_FurnaceLoop.SFX_FurnaceLoop" (`SceneComponent.K2_GetComponentLocation` (`self.DefaultSceneRoot`)) (struct) 1.0 1.0 0.0 "/Game/PathOfLight/VFX/Fire_and_smoke/VFX-k/Steam.Steam" null)))

(event `ToggleFurnace`
  (bind _smoke2 (`self.Smoke2`))
  (if (`self.FurnaceLit`)
    (set `self.FurnaceLit` false)
    (`LightComponent.SetIntensity` (`self.RectLight`) 0.0)
    (`LightComponent.SetIntensity` (`self.PointLight`) 0.0)
    (`SceneComponent.SetVisibility` _smoke2 false false)
    (`SceneComponent.SetVisibility` (`self.Smoke`) false false)
    (`AudioComponent.SetVolumeMultiplier` (stale `self.ReceiveBeginPlay` _returnvalue) 0.0)
    (`KismetSystemLibrary.Delay` 0.2)
    (`GameplayStatics.PlaySound2D` "/Game/PathOfLight/Sounds/NickSFX/4-7/SFX_FurnaceExtinguish.SFX_FurnaceExtinguish" 0.9 1.0 0.0 null null)
    (else
      (set `self.FurnaceLit` true)
      (`LightComponent.SetIntensity` (`self.RectLight`) 30.0)
      (`LightComponent.SetIntensity` (`self.PointLight`) 15.0)
      (`SceneComponent.SetVisibility` _smoke2 true false)
      (`SceneComponent.SetVisibility` (`self.Smoke`) true false)
      (`GameplayStatics.PlaySound2D` "/Game/PathOfLight/Sounds/NickSFX/4-7/FurnaceStartShort.FurnaceStartShort" 0.7 1.0 0.4 null null)
      (`KismetSystemLibrary.Delay` 1.6)
      (`AudioComponent.SetVolumeMultiplier` (stale `self.ReceiveBeginPlay` _returnvalue) 1.5))))

(event `FuelComplete`
  ;[1 1 1] When all Three Furnaces have been fueled
)

(event `EnhancedInput|/Game/PathOfLight/bp_Imports/ia_Interact`
  (params (ActionValue :type Boolean) (ElapsedSeconds :type "Float (double-precision)") (TriggeredSeconds :type "Float (double-precision)") (InputAction :type "InputAction Object Reference" :default "/Game/PathOfLight/bp_Imports/ia_Interact.ia_Interact"))
  ;[1 1 1] Player Interaction Condition and Visuals
)

(event `self.Interact_Box.OnComponentBeginOverlap`
  (params (OverlappedComponent :type "PrimitiveComponent Object Reference") (OtherActor :type "Actor Object Reference") (OtherComp :type "PrimitiveComponent Object Reference") (OtherBodyIndex :type Integer) (bFromSweep :type Boolean) (SweepResult :type "HitResult Structure (by ref)"))
  ;[1 1 1] Player Interaction Condition and Visuals
)

(event `self.Interact_Box.OnComponentEndOverlap`
  (params (OverlappedComponent :type "PrimitiveComponent Object Reference") (OtherActor :type "Actor Object Reference") (OtherComp :type "PrimitiveComponent Object Reference") (OtherBodyIndex :type Integer))
  ;[1 1 1] Player Interaction Condition and Visuals
)

(fn `UserConstructionScript`)