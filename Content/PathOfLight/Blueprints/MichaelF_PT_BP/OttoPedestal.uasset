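; Otto's pedestal in a statue head puzzle, where the player places or swaps one of four character heads.
; Sphere overlap outlines the pedestal and opens a gate for OttoPedestalInteract.
; Interaction toggles head visibility on pedestal and character to swap with PickupItem; Otto's head marks it correct and calls PedestalStatue's PuzzleComplete.
; MoveDown lowers the pedestal by timeline and removes interaction; older spawn-based placement remains unconnected.
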(event `MoveDown`
  ;[1 1 1] Pedestal Animation
  (`|ExecutionSequence`
    (:`then_0`
      (bind (_direction _y_position) (`Timeline|Push Down` :!via `PlayFromStart`)
        (:`Update`
          (bind _returnvalue_location (`KismetMathLibrary.BreakTransform` (`KismetMathLibrary.TLerp` (`self.Starting Position`) (`self.End Position`) _y_position)))
          (`SceneComponent.K2_SetRelativeLocation` (`self.Pedestal`) _returnvalue_location false false))))
    (:`then_1`
      (`ActorComponent.K2_DestroyComponent` (`self.Interact Sphere`)))))

(event `Set Head Visibility`
  ;[1 1 1] Statue Head Logic for the Lumi
  (if (`SceneComponent.IsVisible` (`self.OttoHead1`))
    (bind _otto (`/Game/PathOfLight/bp_Imports/bp_Character.Otto` (stale `OttoPedestalInteract` _asbp_character)))
    (`SceneComponent.SetVisibility` _otto true false)
    (bind _luxx (`/Game/PathOfLight/bp_Imports/bp_Character.Luxx` (stale `OttoPedestalInteract` _asbp_character)))
    (`SceneComponent.SetVisibility` _luxx false false)
    (bind _solara (`/Game/PathOfLight/bp_Imports/bp_Character.Solara` (stale `OttoPedestalInteract` _asbp_character)))
    (`SceneComponent.SetVisibility` _solara false false)
    (bind _kandel (`/Game/PathOfLight/bp_Imports/bp_Character.Kandel` (stale `OttoPedestalInteract` _asbp_character)))
    (`SceneComponent.SetVisibility` _kandel false false)
    (set `/Game/PathOfLight/bp_Imports/bp_Character.PickupItem#` 1 (stale `OttoPedestalInteract` _asbp_character))
    (elif (`SceneComponent.IsVisible` (`self.LuxxHead2`))
      (`SceneComponent.SetVisibility` _luxx true false)
      (`SceneComponent.SetVisibility` _otto false false)
      (`SceneComponent.SetVisibility` _solara false false)
      (`SceneComponent.SetVisibility` _kandel false false)
      (set `/Game/PathOfLight/bp_Imports/bp_Character.PickupItem#` 2 (stale `OttoPedestalInteract` _asbp_character))
      (elif (`SceneComponent.IsVisible` (`self.SolaraHead3`))
        (`SceneComponent.SetVisibility` _solara true false)
        (`SceneComponent.SetVisibility` _otto false false)
        (`SceneComponent.SetVisibility` _luxx false false)
        (`SceneComponent.SetVisibility` _kandel false false)
        (set `/Game/PathOfLight/bp_Imports/bp_Character.PickupItem#` 3 (stale `OttoPedestalInteract` _asbp_character))
        (elif (`SceneComponent.IsVisible` (`self.KandelHead4`))
          (`SceneComponent.SetVisibility` _kandel true false)
          (`SceneComponent.SetVisibility` _otto false false)
          (`SceneComponent.SetVisibility` _luxx false false)
          (`SceneComponent.SetVisibility` _solara false false)
          (set `/Game/PathOfLight/bp_Imports/bp_Character.PickupItem#` 4 (stale `OttoPedestalInteract` _asbp_character))
          (else
            (`SceneComponent.SetVisibility` _otto false false)
            (`SceneComponent.SetVisibility` _luxx false false)
            (`SceneComponent.SetVisibility` _solara false false)
            (`SceneComponent.SetVisibility` _kandel false false)
            (set `/Game/PathOfLight/bp_Imports/bp_Character.PickupItem#` 0 (stale `OttoPedestalInteract` _asbp_character))))))))

(event `self.ReceiveBeginPlay`
  ;[1 1 1] Player Interactivity
  (`self.EnableInput` (`GameplayStatics.GetPlayerController` 0)))

(event `EnhancedInput|/Game/PathOfLight/bp_Imports/ia_Interact`
  (params (ActionValue :type Boolean) (ElapsedSeconds :type "Float (double-precision)") (TriggeredSeconds :type "Float (double-precision)") (InputAction :type "InputAction Object Reference" :default "/Game/PathOfLight/bp_Imports/ia_Interact.ia_Interact"))
  ;[1 1 1] Player Interactivity
)

(event `OttoPedestalInteract`
  ;[1 1 1] Player Interactivity
  (bind _asbp_character (cast `/Game/PathOfLight/bp_Imports/bp_Character` (`GameplayStatics.GetPlayerCharacter` 0)))
  (if (or (> (`/Game/PathOfLight/bp_Imports/bp_Character.PickupItem#` _asbp_character) 0) (`self.HeadPlaced`))
    (`/Engine/EditorBlueprintResources/StandardMacros.Gate` true :!label _label
      (:`Exit`
        (`/Game/PathOfLight/bp_Imports/bp_Character.Interact` _asbp_character)
        (`KismetSystemLibrary.Delay` 0.5)
        (`KismetSystemLibrary.DelayUntilNextTick`)
        (bind _pickupitem_ (`/Game/PathOfLight/bp_Imports/bp_Character.PickupItem#` _asbp_character))
        ;[1 1 1] Logic for which Head is Placed
        (if (== _pickupitem_ 1)
          (`self.Set Head Visibility`)
          (`SceneComponent.SetVisibility` (`self.OttoHead1`) true false)
          (`SceneComponent.SetVisibility` (`self.LuxxHead2`) false false)
          (`SceneComponent.SetVisibility` (`self.SolaraHead3`) false false)
          (`SceneComponent.SetVisibility` (`self.KandelHead4`) false false)
          (set `self.PlacedHead` "Correct")
          (set `self.HeadPlaced` true)
          (bind _returnvalue (`GameplayStatics.GetActorOfClass` "/Game/PathOfLight/Blueprints/MichaelF_PT_BP/PedestalStatue.PedestalStatue_C"))
          (`/Game/PathOfLight/Blueprints/MichaelF_PT_BP/PedestalStatue.PuzzleComplete` _returnvalue)
          (`KismetSystemLibrary.PrintString` "Correct")
          (elif (== _pickupitem_ 2)
            (`self.Set Head Visibility`)
            (`SceneComponent.SetVisibility` (`self.OttoHead1`) false false)
            (`SceneComponent.SetVisibility` (`self.LuxxHead2`) true false)
            (`SceneComponent.SetVisibility` (`self.SolaraHead3`) false false)
            (`SceneComponent.SetVisibility` (`self.KandelHead4`) false false)
            (set `self.PlacedHead` "Incorrect")
            (set `self.HeadPlaced` true)
            (elif (== _pickupitem_ 3)
              (`self.Set Head Visibility`)
              (`SceneComponent.SetVisibility` (`self.OttoHead1`) false false)
              (`SceneComponent.SetVisibility` (`self.LuxxHead2`) false false)
              (`SceneComponent.SetVisibility` (`self.SolaraHead3`) true false)
              (`SceneComponent.SetVisibility` (`self.KandelHead4`) false false)
              (set `self.PlacedHead` "Incorrect")
              (set `self.HeadPlaced` true)
              (elif (== _pickupitem_ 4)
                (`self.Set Head Visibility`)
                (`SceneComponent.SetVisibility` (`self.OttoHead1`) false false)
                (`SceneComponent.SetVisibility` (`self.LuxxHead2`) false false)
                (`SceneComponent.SetVisibility` (`self.SolaraHead3`) false false)
                (`SceneComponent.SetVisibility` (`self.KandelHead4`) true false)
                (set `self.PlacedHead` "Incorrect")
                (set `self.HeadPlaced` true)
                (elif (== _pickupitem_ 0)
                  (`self.Set Head Visibility`)
                  (`SceneComponent.SetVisibility` (`self.OttoHead1`) false false)
                  (`SceneComponent.SetVisibility` (`self.LuxxHead2`) false false)
                  (`SceneComponent.SetVisibility` (`self.SolaraHead3`) false false)
                  (`SceneComponent.SetVisibility` (`self.KandelHead4`) false false)
                  (set `self.PlacedHead` "Incorrect")
                  (set `self.HeadPlaced` false))))))))))

(event `self.Interact Sphere.OnComponentBeginOverlap`
  (params (OverlappedComponent :type "PrimitiveComponent Object Reference") (OtherActor :type "Actor Object Reference") (OtherComp :type "PrimitiveComponent Object Reference") (OtherBodyIndex :type Integer) (bFromSweep :type Boolean) (SweepResult :type "HitResult Structure (by ref)"))
  ;[1 1 1] Player Interactivity
  (bind _asbp_character (cast `/Game/PathOfLight/bp_Imports/bp_Character` OtherActor))
  (set `/Game/PathOfLight/bp_Imports/bp_Character.NorthOverlap?` true _asbp_character)
  (`MeshComponent.SetOverlayMaterial` (`self.Pedestal`) "/Game/PathOfLight/Materials/m_Outline_Inst.m_Outline_Inst")
  (goto _label :!via `Open`))

(event `self.Interact Sphere.OnComponentEndOverlap`
  (params (OverlappedComponent :type "PrimitiveComponent Object Reference") (OtherActor :type "Actor Object Reference") (OtherComp :type "PrimitiveComponent Object Reference") (OtherBodyIndex :type Integer))
  ;[1 1 1] Player Interactivity
  (bind _asbp_character (cast `/Game/PathOfLight/bp_Imports/bp_Character` OtherActor))
  (set `/Game/PathOfLight/bp_Imports/bp_Character.NorthOverlap?` false _asbp_character)
  (`MeshComponent.SetOverlayMaterial` (`self.Pedestal`) null)
  (goto _label :!via `Close`))

(fn `UserConstructionScript`)