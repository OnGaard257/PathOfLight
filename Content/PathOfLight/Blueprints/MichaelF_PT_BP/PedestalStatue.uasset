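; PedestalStatue checks completion of the four-head pedestal puzzle (Otto, Luxx, Solara, Kandel) and triggers its reward.
; PuzzleComplete finds each pedestal by class and tests whether every PlacedHead is "Correct".
; On success it lowers ThrowRewardPedestal and the four head pedestals, plays a power sound, and calls OnPedestalSolved after each head pedestal's move.
; A statue-rotation timeline exists but is never triggered.
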(event `PuzzleComplete`
  (`|ExecutionSequence`
    (:`then_0`
      (bind _returnvalue (`GameplayStatics.GetActorOfClass` "/Game/PathOfLight/Blueprints/MichaelF_PT_BP/OttoPedestal.OttoPedestal_C")))
    (:`then_1`
      (bind _returnvalue_2 (`GameplayStatics.GetActorOfClass` "/Game/PathOfLight/Blueprints/MichaelF_PT_BP/LuxxPedestal.LuxxPedestal_C")))
    (:`then_2`
      (bind _returnvalue_3 (`GameplayStatics.GetActorOfClass` "/Game/PathOfLight/Blueprints/MichaelF_PT_BP/SolaraPedestal.SolaraPedestal_C")))
    (:`then_3`
      (bind _returnvalue_4 (`GameplayStatics.GetActorOfClass` "/Game/PathOfLight/Blueprints/MichaelF_PT_BP/KandelPedestal.KandelPedestal_C"))))
  (if (and (`KismetStringLibrary.EqualEqual_StrStr` (`/Game/PathOfLight/Blueprints/MichaelF_PT_BP/OttoPedestal.PlacedHead` _returnvalue) "Correct") (`KismetStringLibrary.EqualEqual_StrStr` (`/Game/PathOfLight/Blueprints/MichaelF_PT_BP/LuxxPedestal.PlacedHead` _returnvalue_2) "Correct") (`KismetStringLibrary.EqualEqual_StrStr` (`/Game/PathOfLight/Blueprints/MichaelF_PT_BP/SolaraPedestal.PlacedHead` _returnvalue_3) "Correct") (`KismetStringLibrary.EqualEqual_StrStr` (`/Game/PathOfLight/Blueprints/MichaelF_PT_BP/KandelPedestal.PlacedHead` _returnvalue_4) "Correct"))
    (bind _returnvalue_5 (`GameplayStatics.GetActorOfClass` "/Game/PathOfLight/Blueprints/MichaelF_PT_BP/ThrowRewardPedestal.ThrowRewardPedestal_C"))
    (`/Game/PathOfLight/Blueprints/MichaelF_PT_BP/ThrowRewardPedestal.MoveDown` _returnvalue_5)
    (`GameplayStatics.PlaySound2D` "/Game/PathOfLight/Sounds/NickSFX/SFX_GetPower.SFX_GetPower" 1.0 1.0 0.0 null null)
    (`|ExecutionSequence`
      (:`then_0`
        (bind _returnvalue_6 (`GameplayStatics.GetActorOfClass` "/Game/PathOfLight/Blueprints/MichaelF_PT_BP/OttoPedestal.OttoPedestal_C"))
        (`/Game/PathOfLight/Blueprints/MichaelF_PT_BP/OttoPedestal.MoveDown` _returnvalue_6))
      (:`then_1`
        (bind _returnvalue_7 (`GameplayStatics.GetActorOfClass` "/Game/PathOfLight/Blueprints/MichaelF_PT_BP/LuxxPedestal.LuxxPedestal_C"))
        (`/Game/PathOfLight/Blueprints/MichaelF_PT_BP/LuxxPedestal.Move Down` _returnvalue_7))
      (:`then_2`
        (bind _returnvalue_8 (`GameplayStatics.GetActorOfClass` "/Game/PathOfLight/Blueprints/MichaelF_PT_BP/SolaraPedestal.SolaraPedestal_C"))
        (`/Game/PathOfLight/Blueprints/MichaelF_PT_BP/SolaraPedestal.Move Down` _returnvalue_8))
      (:`then_3`
        (bind _returnvalue_9 (`GameplayStatics.GetActorOfClass` "/Game/PathOfLight/Blueprints/MichaelF_PT_BP/KandelPedestal.KandelPedestal_C"))
        (`/Game/PathOfLight/Blueprints/MichaelF_PT_BP/KandelPedestal.Move Down` _returnvalue_9)))
    (`self.OnPedestalSolved`)))

(fn `UserConstructionScript`)