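; Scrap rubble pickup that the player character collects with the interact input to add one to its scrap count.
; Overlapping the sphere puts an outline overlay material on the three rubble pieces and opens a Gate; leaving clears both.
; The actor enables input on itself at BeginPlay, and an interact press passes only through the open Gate, destroying the rubble and incrementing ScrapAmount on bp_Character.
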(event `self.ReceiveBeginPlay`
  (`self.EnableInput` (`GameplayStatics.GetPlayerController` 0)))

(event `EnhancedInput|/Game/PathOfLight/bp_Imports/ia_Interact`
  (params (ActionValue :type Boolean) (ElapsedSeconds :type "Float (double-precision)") (TriggeredSeconds :type "Float (double-precision)") (InputAction :type "InputAction Object Reference" :default "/Game/PathOfLight/bp_Imports/ia_Interact.ia_Interact"))
  (:`Triggered`
    (bind _asbp_character (cast `/Game/PathOfLight/bp_Imports/bp_Character` (`GameplayStatics.GetPlayerPawn` 0)))
    (`/Engine/EditorBlueprintResources/StandardMacros.Gate` true :!label _label
      (:`Exit`
        (`self.K2_DestroyActor`)
        (`/Engine/EditorBlueprintResources/StandardMacros.IncrementInt` (`/Game/PathOfLight/bp_Imports/bp_Character.ScrapAmount` _asbp_character))))))

(event `self.Sphere.OnComponentBeginOverlap`
  (params (OverlappedComponent :type "PrimitiveComponent Object Reference") (OtherActor :type "Actor Object Reference") (OtherComp :type "PrimitiveComponent Object Reference") (OtherBodyIndex :type Integer) (bFromSweep :type Boolean) (SweepResult :type "HitResult Structure (by ref)"))
  (cast `/Game/PathOfLight/bp_Imports/bp_Character` OtherActor)
  (`MeshComponent.SetOverlayMaterial` (`self.Piece #1`) "/Game/PathOfLight/Materials/m_Outline_Inst.m_Outline_Inst")
  (`MeshComponent.SetOverlayMaterial` (`self.Piece #2`) "/Game/PathOfLight/Materials/m_Outline_Inst.m_Outline_Inst")
  (`MeshComponent.SetOverlayMaterial` (`self.Piece #3`) "/Game/PathOfLight/Materials/m_Outline_Inst.m_Outline_Inst")
  (goto _label :!via `Open`))

(event `self.Sphere.OnComponentEndOverlap`
  (params (OverlappedComponent :type "PrimitiveComponent Object Reference") (OtherActor :type "Actor Object Reference") (OtherComp :type "PrimitiveComponent Object Reference") (OtherBodyIndex :type Integer))
  (cast `/Game/PathOfLight/bp_Imports/bp_Character` OtherActor)
  (`MeshComponent.SetOverlayMaterial` (`self.Piece #1`) null)
  (`MeshComponent.SetOverlayMaterial` (`self.Piece #2`) null)
  (`MeshComponent.SetOverlayMaterial` (`self.Piece #3`) null)
  (goto _label :!via `Close`))

(fn `UserConstructionScript`)