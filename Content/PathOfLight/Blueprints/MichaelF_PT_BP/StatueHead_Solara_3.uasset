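; Pickup actor for the Solara statue head, which the player collects or swaps with another carried head.
; A sphere overlap toggles an outline and a Gate, letting Interact work while the character's Rock is hidden.
; Pickup shows the character's Solara mesh, sets PickupItem and destroys the actor, first spawning any held Kandel, Luxx or Otto head in its place.
; The Correct! event removes the pickup sphere.
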(event `self.ReceiveBeginPlay`
  ;[1 1 1] Enable Player Input
  (`self.EnableInput` (`GameplayStatics.GetPlayerController` 0)))

(event `Correct!`
  (`ActorComponent.K2_DestroyComponent` (`self.Pickup Sphere`)))

(event `EnhancedInput|/Game/PathOfLight/bp_Imports/ia_Interact`
  (params (ActionValue :type Boolean) (ElapsedSeconds :type "Float (double-precision)") (TriggeredSeconds :type "Float (double-precision)") (InputAction :type "InputAction Object Reference" :default "/Game/PathOfLight/bp_Imports/ia_Interact.ia_Interact"))
  (bind _defaultsceneroot (`self.DefaultSceneRoot`))
  (bind _returnvalue (`SceneComponent.K2_GetComponentLocation` _defaultsceneroot))
  (bind _returnvalue_2 (`SceneComponent.K2_GetComponentRotation` _defaultsceneroot))
  (:`Triggered`
    (bind _asbp_character (cast `/Game/PathOfLight/bp_Imports/bp_Character` (`GameplayStatics.GetPlayerCharacter` 0)))
    (if (not (`SceneComponent.IsVisible` (`/Game/PathOfLight/bp_Imports/bp_Character.Rock` _asbp_character)))
      (`/Engine/EditorBlueprintResources/StandardMacros.Gate` true :!label _label
        (:`Exit`
          (if (== (`/Game/PathOfLight/bp_Imports/bp_Character.PickupItem#` _asbp_character) 0)
            (`SceneComponent.SetVisibility` (`/Game/PathOfLight/bp_Imports/bp_Character.Solara` _asbp_character) true false :!label _label_2)
            (set `/Game/PathOfLight/bp_Imports/bp_Character.PickupItem#` 3 _asbp_character)
            (`self.K2_DestroyActor`)
            (else
              (bind _kandel (`/Game/PathOfLight/bp_Imports/bp_Character.Kandel` _asbp_character))
              (if (`SceneComponent.IsVisible` _kandel)
                (`|SpawnActorFromClass` "/Game/PathOfLight/Blueprints/MichaelF_PT_BP/StatueHead_Kandel_4.StatueHead_Kandel_4_C" (`KismetMathLibrary.MakeTransform` _returnvalue _returnvalue_2) "Undefined" "MultiplyWithRoot" null null)
                (`SceneComponent.SetVisibility` _kandel false false)
                (`KismetSystemLibrary.DelayUntilNextTick` :!label _label_3)
                (goto _label_2)
                (else
                  (bind _luxx (`/Game/PathOfLight/bp_Imports/bp_Character.Luxx` _asbp_character))
                  (if (`SceneComponent.IsVisible` _luxx)
                    (`|SpawnActorFromClass` "/Game/PathOfLight/Blueprints/MichaelF_PT_BP/StatueHead_Luxx_2.StatueHead_Luxx_2_C" (`KismetMathLibrary.MakeTransform` _returnvalue _returnvalue_2) "Undefined" "MultiplyWithRoot" null null)
                    (`SceneComponent.SetVisibility` _luxx false false)
                    (goto _label_3)
                    (else
                      (bind _otto (`/Game/PathOfLight/bp_Imports/bp_Character.Otto` _asbp_character))
                      (if (`SceneComponent.IsVisible` _otto)
                        (`|SpawnActorFromClass` "/Game/PathOfLight/Blueprints/MichaelF_PT_BP/StatueHead_Otto_1.StatueHead_Otto_1_C" (`KismetMathLibrary.MakeTransform` _returnvalue _returnvalue_2) "Undefined" "MultiplyWithRoot" null null)
                        (`SceneComponent.SetVisibility` _otto false false)
                        (goto _label_3)))))))))))))

(event `self.Pickup Sphere.OnComponentBeginOverlap`
  (params (OverlappedComponent :type "PrimitiveComponent Object Reference") (OtherActor :type "Actor Object Reference") (OtherComp :type "PrimitiveComponent Object Reference") (OtherBodyIndex :type Integer) (bFromSweep :type Boolean) (SweepResult :type "HitResult Structure (by ref)"))
  (cast `/Game/PathOfLight/bp_Imports/bp_Character` OtherActor)
  (`MeshComponent.SetOverlayMaterial` (`self.Solara_Head`) "/Game/PathOfLight/Materials/m_Outline_Inst.m_Outline_Inst")
  (goto _label :!via `Open`))

(event `self.Pickup Sphere.OnComponentEndOverlap`
  (params (OverlappedComponent :type "PrimitiveComponent Object Reference") (OtherActor :type "Actor Object Reference") (OtherComp :type "PrimitiveComponent Object Reference") (OtherBodyIndex :type Integer))
  (cast `/Game/PathOfLight/bp_Imports/bp_Character` OtherActor)
  (`MeshComponent.SetOverlayMaterial` (`self.Solara_Head`) null)
  (goto _label :!via `Close`))

(fn `UserConstructionScript`)