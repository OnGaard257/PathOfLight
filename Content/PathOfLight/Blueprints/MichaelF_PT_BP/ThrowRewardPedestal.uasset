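; A reward pedestal Blueprint whose MoveDown event lowers the pedestal with a stone-rotation sound.
; The PushDown timeline drives a lerp between the start and end transforms, applying only the location to the Pedestal's relative position.
; Disconnected logic that would spawn a throw-key test actor and attach it to the Socket never runs.
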(event `self.ReceiveBeginPlay`)

(event `MoveDown`
  (`GameplayStatics.PlaySound2D` "/Game/PathOfLight/Sounds/ColeSFX/StoneRotate.StoneRotate" 2.0 1.2 0.0 null null)
  (bind (_direction _y_position) (`Timeline|Push Down` :!via `PlayFromStart`)
    (:`Update`
      (bind _returnvalue_location (`KismetMathLibrary.BreakTransform` (`KismetMathLibrary.TLerp` (`self.Starting Position`) (`self.End Position`) _y_position)))
      (`SceneComponent.K2_SetRelativeLocation` (`self.Pedestal`) _returnvalue_location false false))))

(fn `UserConstructionScript`)