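; Cavern gate Blueprint that swings a pair of gate doors open when its OpenTheGates event is called.
; The event plays a 2D creak sound and starts the GateOpenAnim timeline.
; Each timeline update lerps the left and right gate relative rotations between their stored start and end rotators.
; The file holds no closing logic or trigger of its own.
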(event `self.ReceiveBeginPlay`)

(event `10-8/OpenTheGates`
  (`GameplayStatics.PlaySound2D` "/Game/PathOfLight/Sounds/NickSFX/4-13/SFX_Creak.SFX_Creak" 1.2 0.7 0.0 null null)
  (bind (_direction _newtrack_0) (`Timeline|GateOpenAnim`)
    (:`Update`
      (`SceneComponent.K2_SetRelativeRotation` (`self.GateLeft`) (`KismetMathLibrary.RLerp` (`self.LeftDoorStart`) (`self.LeftDoorEnd`) _newtrack_0) false false)
      (`SceneComponent.K2_SetRelativeRotation` (`self.GateRight`) (`KismetMathLibrary.RLerp` (`self.RightDoorStart`) (`self.RightDoorEnd`) _newtrack_0) false false))))

(fn `UserConstructionScript`)