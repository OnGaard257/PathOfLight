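; Coal bowl pickup that lets the player take one piece of coal to carry, apparently for fueling furnaces.
; Box overlap outlines the bowl and opens a gate for the interact input, which requires no visible gear, no held scrap and fewer than three fueled furnaces.
; A pickup shows the character's coal, increments ScrapAmount and hides a random coal mesh through CoalVisibilityChart.
; Only one random branch checks for a full Furnace to destroy the trigger box.
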(event `self.ReceiveBeginPlay`
  (`self.EnableInput` (`GameplayStatics.GetPlayerController` 0)))

(event `EnhancedInput|/Game/PathOfLight/bp_Imports/ia_Interact`
  (params (ActionValue :type Boolean) (ElapsedSeconds :type "Float (double-precision)") (TriggeredSeconds :type "Float (double-precision)") (InputAction :type "InputAction Object Reference" :default "/Game/PathOfLight/bp_Imports/ia_Interact.ia_Interact"))
  (:`Triggered`
    (bind _asbp_character (cast `/Game/PathOfLight/bp_Imports/bp_Character` (`GameplayStatics.GetPlayerCharacter` 0)))
    (if (not (`SceneComponent.bVisible` (`/Game/PathOfLight/bp_Imports/bp_Character.Gear` _asbp_character)))
      (bind _scrapamount (`/Game/PathOfLight/bp_Imports/bp_Character.ScrapAmount` _asbp_character))
      (if (< _scrapamount 1)
        (if (< (`/Game/PathOfLight/bp_Imports/bp_Character.FurnacesFueled` _asbp_character) 3)
          (`/Engine/EditorBlueprintResources/StandardMacros.Gate` true :!label _label
            (:`Exit`
              (`/Game/PathOfLight/bp_Imports/bp_Character.Interact` _asbp_character)
              (`SceneComponent.SetVisibility` (`/Game/PathOfLight/bp_Imports/bp_Character.Coal` _asbp_character) true false)
              (`/Engine/EditorBlueprintResources/StandardMacros.IncrementInt` _scrapamount
                (:`  `
                  (switch `int` (`KismetMathLibrary.RandomIntegerInRange` 0 6)
                    (:`0`
                      (`SceneComponent.SetVisibility` (`self.Coal#2`) false false))
                    (:`1`
                      (`SceneComponent.SetVisibility` (`self.Coal#4`) false false))
                    (:`2`
                      (`SceneComponent.SetVisibility` (`self.Coal#8`) false false))
                    (:`3`
                      (`SceneComponent.SetVisibility` (`self.Coal#6`) false false))
                    (:`4`
                      (`SceneComponent.SetVisibility` (`self.Coal#7`) false false))
                    (:`5`
                      (`SceneComponent.SetVisibility` (`self.Coal#9`) false false))
                    (:`6`
                      (`SceneComponent.SetVisibility` (`self.Coal#11`) false false)))
                  (bind _returnvalue (`GameplayStatics.GetActorOfClass` "/Game/PathOfLight/Blueprints/MichaelF_PT_BP/Furnace.Furnace_C"))
                  (if (`/Game/PathOfLight/Blueprints/MichaelF_PT_BP/Furnace.FurnaceFull` _returnvalue)
                    (`ActorComponent.K2_DestroyComponent` (`self.Box`))))))))))))

(event `self.Box.OnComponentBeginOverlap`
  (params (OverlappedComponent :type "PrimitiveComponent Object Reference") (OtherActor :type "Actor Object Reference") (OtherComp :type "PrimitiveComponent Object Reference") (OtherBodyIndex :type Integer) (bFromSweep :type Boolean) (SweepResult :type "HitResult Structure (by ref)"))
  (cast `/Game/PathOfLight/bp_Imports/bp_Character` OtherActor)
  (`MeshComponent.SetOverlayMaterial` (`self.Bowl`) "/Game/PathOfLight/Materials/m_Outline_Inst.m_Outline_Inst")
  (goto _label :!via `Open`))

(event `self.Box.OnComponentEndOverlap`
  (params (OverlappedComponent :type "PrimitiveComponent Object Reference") (OtherActor :type "Actor Object Reference") (OtherComp :type "PrimitiveComponent Object Reference") (OtherBodyIndex :type Integer))
  (cast `/Game/PathOfLight/bp_Imports/bp_Character` OtherActor)
  (`MeshComponent.SetOverlayMaterial` (`self.Bowl`) null)
  (goto _label :!via `Close`))

(fn `UserConstructionScript`)