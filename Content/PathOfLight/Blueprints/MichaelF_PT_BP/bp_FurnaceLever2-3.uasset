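; Lever actor that toggles two furnaces when the player presses Interact while inside its trigger box.
; It enables player input on BeginPlay, and overlap with bp_Character opens and closes a Gate that filters the Interact action.
; Each press looks up NewFurnace2 and NewFurnace3 with GetActorOfClass and calls ToggleFurnace on both, so the targets are fixed by class rather than assigned references.
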(event `self.ReceiveBeginPlay`
  (`self.EnableInput` (`GameplayStatics.GetPlayerController` 0)))

(event `EnhancedInput|/Game/PathOfLight/bp_Imports/ia_Interact`
  (params (ActionValue :type Boolean) (ElapsedSeconds :type "Float (double-precision)") (TriggeredSeconds :type "Float (double-precision)") (InputAction :type "InputAction Object Reference" :default "/Game/PathOfLight/bp_Imports/ia_Interact.ia_Interact"))
  (:`Triggered`
    (`/Engine/EditorBlueprintResources/StandardMacros.Gate` true :!label _label
      (:`Exit`
        (`|ExecutionSequence`
          (:`then_0`
            (bind _returnvalue (`GameplayStatics.GetActorOfClass` "/Game/PathOfLight/Blueprints/MichaelF_PT_BP/NewFurnace2.NewFurnace2_C"))
            (`/Game/PathOfLight/Blueprints/MichaelF_PT_BP/NewFurnace2.ToggleFurnace` _returnvalue))
          (:`then_1`
            (bind _returnvalue_2 (`GameplayStatics.GetActorOfClass` "/Game/PathOfLight/Blueprints/MichaelF_PT_BP/NewFurnace3.NewFurnace3_C"))
            (`/Game/PathOfLight/Blueprints/MichaelF_PT_BP/NewFurnace3.ToggleFurnace` _returnvalue_2)))))))

(event `self.Box.OnComponentBeginOverlap`
  (params (OverlappedComponent :type "PrimitiveComponent Object Reference") (OtherActor :type "Actor Object Reference") (OtherComp :type "PrimitiveComponent Object Reference") (OtherBodyIndex :type Integer) (bFromSweep :type Boolean) (SweepResult :type "HitResult Structure (by ref)"))
  (cast `/Game/PathOfLight/bp_Imports/bp_Character` OtherActor)
  (goto _label :!via `Open`))

(event `self.Box.OnComponentEndOverlap`
  (params (OverlappedComponent :type "PrimitiveComponent Object Reference") (OtherActor :type "Actor Object Reference") (OtherComp :type "PrimitiveComponent Object Reference") (OtherBodyIndex :type Integer))
  (cast `/Game/PathOfLight/bp_Imports/bp_Character` OtherActor)
  (goto _label :!via `Close`))

(fn `UserConstructionScript`)