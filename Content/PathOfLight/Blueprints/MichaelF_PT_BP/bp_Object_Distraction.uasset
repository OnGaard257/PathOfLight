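; Distraction object, apparently a rock given its impact sound, that lures a blind enemy to where it hits.
; Its first hit on anything but the player plays the sound and reports a noise event with the player as instigator.
; After a short delay it finds the nearest "Enemy"-tagged actor and, if close enough and a BP_BlindEnemy, sends it to the hit location directly.
; The object then destroys itself.
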(event `self.ReceiveHit`
  (params (MyComp :type "PrimitiveComponent Object Reference") (Other :type "Actor Object Reference") (OtherComp :type "PrimitiveComponent Object Reference") (bSelfMoved :type Boolean) (HitLocation :type "Vector Structure") (HitNormal :type "Vector Structure") (NormalImpulse :type "Vector Structure") (Hit :type "HitResult Structure (by ref)"))
  (bind _returnvalue (`GameplayStatics.GetPlayerCharacter` 0))
  (bind _returnvalue_2 (`self.K2_GetActorLocation`))
  ;[1 1 1] Sound Spawn Collision
  (if (!= Other _returnvalue)
    (`/Engine/EditorBlueprintResources/StandardMacros.DoOnce` false
      (:`Completed`
        (`GameplayStatics.PlaySoundAtLocation` "/Game/PathOfLight/Sounds/ThrowSFX/Rock_Hit_Ground.Rock_Hit_Ground" _returnvalue_2 (struct) 1.0 1.0 0.4 null null null null)
        (`AISense_Hearing.ReportNoiseEvent` _returnvalue_2 1.0 _returnvalue 300.0)
        (`KismetSystemLibrary.Delay` 1.0)
        (`|ExecutionSequence`
          (:`then_0`
            (bind _outactors (`GameplayStatics.GetAllActorsWithTag` "Enemy"))
            (bind (_distance _returnvalue_3) (`GameplayStatics.FindNearestActor` HitLocation _outactors))
            (if (not (>= _distance 1500.0))
              (bind _asbp_blind_enemy (cast `/Game/PathOfLight/LD_Prototyping/JavonW/Enemies/BP_BlindEnemy` _returnvalue_3))
              (set `/Game/PathOfLight/LD_Prototyping/JavonW/Enemies/BP_BlindEnemy.Distraction Location` HitLocation _asbp_blind_enemy)
              (`/Game/PathOfLight/LD_Prototyping/JavonW/Enemies/BP_BlindEnemy.GoToDistraction` _asbp_blind_enemy)))
          (:`then_1`
            (`self.K2_DestroyActor`)))))))

(fn `UserConstructionScript`)