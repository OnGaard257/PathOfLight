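; Gear-puzzle pedestal that accepts a gear from the player and treats only the green one as the correct solution.
; Sphere overlap outlines the terminal and opens a gate, letting the debounced interaction swap the carried gear with the placed one, tracked through component visibility.
; A green gear destroys the sphere, starts self-recursive Delay rotation loops, and triggers both G4 gear mechanisms, the green statue, reward progress and staggered steam effects.
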(event `GearTurn`
  ;[1 1 1] Gear Turning Function
  (`SceneComponent.K2_AddLocalRotation` (`self.GreenGear`) (`KismetMathLibrary.MakeRotator` 0.0 (+ (`GameplayStatics.GetWorldDeltaSeconds`) -1.0)) false false)
  (`KismetSystemLibrary.Delay` 0.01)
  (`self.GearTurn`)
  (`self.GearV2Turn`))

(event `SetGearVisibility`
  ;[1 1 1] Gear Swap Functionality
  (if (`SceneComponent.IsVisible` (`self.GreenGear`))
    (bind _gear (`/Game/PathOfLight/bp_Imports/bp_Character.Gear` (stale `SetGear` _asbp_character)))
    (`PrimitiveComponent.SetMaterial` _gear 0 "/Game/PathOfLight/Materials/Test_MM_Green_Gear.Test_MM_Green_Gear")
    (`SceneComponent.SetVisibility` _gear true false)
    (set `/Game/PathOfLight/bp_Imports/bp_Character.HUD#` 2 (stale `SetGear` _asbp_character))
    (set `/Game/PathOfLight/bp_Imports/bp_Character.PickupItem#` 4 (stale `SetGear` _asbp_character))
    (`GameplayStatics.PlaySound2D` "/Game/PathOfLight/Sounds/NickSFX/4-7/SFX_ThrowPickup.SFX_ThrowPickup" 0.5 0.8 0.0 null null :!label _label)
    (elif (`SceneComponent.IsVisible` (`self.RedGear`))
      (`PrimitiveComponent.SetMaterial` _gear 0 "/Game/PathOfLight/Materials/Test_MM_Red_Gear.Test_MM_Red_Gear")
      (`SceneComponent.SetVisibility` _gear true false)
      (set `/Game/PathOfLight/bp_Imports/bp_Character.HUD#` 3 (stale `SetGear` _asbp_character))
      (set `/Game/PathOfLight/bp_Imports/bp_Character.PickupItem#` 2 (stale `SetGear` _asbp_character))
      (goto _label)
      (elif (`SceneComponent.IsVisible` (`self.YellowGear`))
        (`PrimitiveComponent.SetMaterial` _gear 0 "/Game/PathOfLight/Materials/Test_MM_Yellow_Gear_Inst.Test_MM_Yellow_Gear_Inst")
        (`SceneComponent.SetVisibility` _gear true false)
        (set `/Game/PathOfLight/bp_Imports/bp_Character.HUD#` 4 (stale `SetGear` _asbp_character))
        (set `/Game/PathOfLight/bp_Imports/bp_Character.PickupItem#` 3 (stale `SetGear` _asbp_character))
        (goto _label)
        (elif (`SceneComponent.IsVisible` (`self.BlueGear`))
          (`PrimitiveComponent.SetMaterial` _gear 0 "/Game/PathOfLight/Materials/Test_MM_BlueGear_Inst.Test_MM_BlueGear_Inst")
          (`SceneComponent.SetVisibility` _gear true false)
          (set `/Game/PathOfLight/bp_Imports/bp_Character.HUD#` 1 (stale `SetGear` _asbp_character))
          (set `/Game/PathOfLight/bp_Imports/bp_Character.PickupItem#` 1 (stale `SetGear` _asbp_character))
          (goto _label)
          (else
            (`SceneComponent.SetVisibility` _gear false false)
            (set `/Game/PathOfLight/bp_Imports/bp_Character.HUD#` 0 (stale `SetGear` _asbp_character))
            (set `/Game/PathOfLight/bp_Imports/bp_Character.PickupItem#` 0 (stale `SetGear` _asbp_character))))))))

(event `/Game/PathOfLight/LD_Prototyping/JavonW/BPI_Interface.Interaction`
  ;[1 1 1] Event Interaction
  (`self.G4Interact`))

(event `G4Interact`
  (`/Engine/EditorBlueprintResources/StandardMacros.DoOnce` false :!label _label_2
    (:`Completed`
      (`self.SetGear`)
      (`KismetSystemLibrary.Delay` 2.0)
      (goto _label_2 :!via `Reset`))))

(event `GearV2Turn`
  ;[1 1 1] Gear Turning Function
  (`SceneComponent.K2_AddLocalRotation` (`self.GreenGearPiece-1`) (`KismetMathLibrary.MakeRotator` 0.0 (+ (`GameplayStatics.GetWorldDeltaSeconds`) 1.0)) false false)
  (`SceneComponent.K2_AddLocalRotation` (`self.GreenGearPiece-2`) (`KismetMathLibrary.MakeRotator` 0.0 (+ (`GameplayStatics.GetWorldDeltaSeconds`) 1.0)) false false)
  (`KismetSystemLibrary.Delay` 0.01)
  (`self.GearV2Turn`))

(event `self.ReceiveBeginPlay`
  ;[1 1 1] Pedestal Interaction
  (`self.EnableInput` (`GameplayStatics.GetPlayerController` 0)))

(event `SetGear`
  (bind _defaultsceneroot (`self.DefaultSceneRoot`))
  ;[1 1 1] Pedestal Interaction
  (bind _asbp_character (cast `/Game/PathOfLight/bp_Imports/bp_Character` (`GameplayStatics.GetPlayerCharacter` 0)))
  (if (or (> (`/Game/PathOfLight/bp_Imports/bp_Character.PickupItem#` _asbp_character) 0) (`self.Gear?`))
    (`/Engine/EditorBlueprintResources/StandardMacros.Gate` true :!label _label_3
      (:`Exit`
        (bind _cooldownuiref (`/Game/PathOfLight/bp_Imports/bp_Character.CooldownUIRef` _asbp_character))
        (`/Game/PathOfLight/bp_Imports/HUD_UI.GearHide` _cooldownuiref)
        (`/Game/PathOfLight/bp_Imports/bp_Character.Interact` _asbp_character)
        (`KismetSystemLibrary.Delay` 0.5)
        (`SceneComponent.SetVisibility` (`/Game/PathOfLight/bp_Imports/bp_Character.Gear` _asbp_character) false false)
        (`KismetSystemLibrary.DelayUntilNextTick`)
        (bind _pickupitem_ (`/Game/PathOfLight/bp_Imports/bp_Character.PickupItem#` _asbp_character))
        ;[1 1 1] If the Player has picked up either blue or red cubes
        (if (== _pickupitem_ 4)
          (`self.SetGearVisibility`)
          (`/Game/PathOfLight/bp_Imports/HUD_UI.GearVisibility` _cooldownuiref)
          (`SceneComponent.SetVisibility` (`self.YellowGear`) false false)
          (`SceneComponent.SetVisibility` (`self.BlueGear`) false false)
          (`SceneComponent.SetVisibility` (`self.RedGear`) false false)
          (`SceneComponent.SetVisibility` (`self.GreenGear`) true false)
          (set `self.PlacedItem` "Correct")
          (`ActorComponent.K2_DestroyComponent` (`self.Sphere`))
          (`GameplayStatics.PlaySound2D` "/Game/PathOfLight/Sounds/NickSFX/4-7/SFX_ThrowPickup.SFX_ThrowPickup" 0.6 1.0 0.0 null null)
          (`KismetSystemLibrary.Delay` 0.5)
          (`self.GearTurn`)
          (`KismetSystemLibrary.Delay` 0.5)
          (`|ExecutionSequence`
            (:`then_0`
              (bind _returnvalue (`GameplayStatics.GetActorOfClass` "/Game/PathOfLight/Blueprints/MichaelF_PT_BP/GearMech_G4.GearMech_G4_C"))
              (`/Game/PathOfLight/Blueprints/MichaelF_PT_BP/GearMech_G4.GearWallTurn` _returnvalue)
              (`/Game/PathOfLight/Blueprints/MichaelF_PT_BP/GearMech_G4.GearV2WallTurn` _returnvalue))
            (:`then_1`
              (bind _returnvalue_2 (`GameplayStatics.GetActorOfClass` "/Game/PathOfLight/Blueprints/MichaelF_PT_BP/GearMech_G4_2.GearMech_G4_2_C"))
              (`/Game/PathOfLight/Blueprints/MichaelF_PT_BP/GearMech_G4_2.GearWallTurn` _returnvalue_2)
              (`/Game/PathOfLight/Blueprints/MichaelF_PT_BP/GearMech_G4_2.GearV2WallTurn` _returnvalue_2))
            (:`then_2`
              (bind _returnvalue_3 (`GameplayStatics.GetActorOfClass` "/Game/PathOfLight/Blueprints/MichaelF_PT_BP/bp_Statue_Green.bp_Statue_Green_C"))
              (`/Game/PathOfLight/Blueprints/MichaelF_PT_BP/bp_Statue_Green.CorrectRotation` _returnvalue_3)
              (bind _returnvalue_4 (`GameplayStatics.GetActorOfClass` "/Game/PathOfLight/Blueprints/MichaelF_PT_BP/Light_Key_Reward.Light_Key_Reward_C"))
              (`/Game/PathOfLight/Blueprints/MichaelF_PT_BP/Light_Key_Reward.StatueProgress` _returnvalue_4)
              (`ActorComponent.Activate` (`self.Steam-1`) false)
              (`GameplayStatics.SpawnSoundAttached` "/Game/StarterContent/Audio/Steam01_Cue.Steam01_Cue" _defaultsceneroot "None" (0.0 0.0 0.0) (struct) "KeepRelativeOffset" false 0.2 1.0 0.0 "/Game/PathOfLight/VFX/Fire_and_smoke/VFX-k/Steam.Steam" null)
              (`KismetSystemLibrary.Delay` 1.0)
              (`ActorComponent.Activate` (`self.Steam-2`) false)
              (`GameplayStatics.SpawnSoundAttached` "/Game/StarterContent/Audio/Steam01_Cue.Steam01_Cue" _defaultsceneroot "None" (0.0 0.0 0.0) (struct) "KeepRelativeOffset" false 0.2 1.0 0.0 "/Game/PathOfLight/VFX/Fire_and_smoke/VFX-k/Steam.Steam" null)
              (`KismetSystemLibrary.Delay` 1.0)
              (`ActorComponent.Activate` (`self.Steam-3`) false)
              (`GameplayStatics.SpawnSoundAttached` "/Game/StarterContent/Audio/Steam01_Cue.Steam01_Cue" _defaultsceneroot "None" (0.0 0.0 0.0) (struct) "KeepRelativeOffset" false 0.2 1.0 0.0 "/Game/PathOfLight/VFX/Fire_and_smoke/VFX-k/Steam.Steam" null)))
          (elif (== _pickupitem_ 1)
            (`self.SetGearVisibility`)
            (`/Game/PathOfLight/bp_Imports/HUD_UI.GearVisibility` _cooldownuiref)
            (`SceneComponent.SetVisibility` (`self.YellowGear`) false false)
            (`SceneComponent.SetVisibility` (`self.BlueGear`) true false)
            (`SceneComponent.SetVisibility` (`self.RedGear`) false false)
            (`SceneComponent.SetVisibility` (`self.GreenGear`) false false)
            (set `self.PlacedItem` "False")
            (`GameplayStatics.PlaySound2D` "/Game/PathOfLight/Sounds/NickSFX/SFX_Gear.SFX_Gear" 0.4 1.0 0.0 null null)
            (set `self.Gear?` true)
            (elif (== _pickupitem_ 2)
              (`self.SetGearVisibility`)
              (`/Game/PathOfLight/bp_Imports/HUD_UI.GearVisibility` _cooldownuiref)
              (`SceneComponent.SetVisibility` (`self.YellowGear`) false false)
              (`SceneComponent.SetVisibility` (`self.BlueGear`) false false)
              (`SceneComponent.SetVisibility` (`self.RedGear`) true false)
              (`SceneComponent.SetVisibility` (`self.GreenGear`) false false)
              (set `self.PlacedItem` "False")
              (`GameplayStatics.PlaySound2D` "/Game/PathOfLight/Sounds/NickSFX/SFX_Gear.SFX_Gear" 0.4 1.0 0.0 null null)
              (set `self.Gear?` true)
              (elif (== _pickupitem_ 3)
                (`self.SetGearVisibility`)
                (`/Game/PathOfLight/bp_Imports/HUD_UI.GearVisibility` _cooldownuiref)
                (`SceneComponent.SetVisibility` (`self.YellowGear`) true false)
                (`SceneComponent.SetVisibility` (`self.BlueGear`) false false)
                (`SceneComponent.SetVisibility` (`self.RedGear`) false false)
                (`SceneComponent.SetVisibility` (`self.GreenGear`) false false)
                (set `self.PlacedItem` "False")
                (`GameplayStatics.PlaySound2D` "/Game/PathOfLight/Sounds/NickSFX/SFX_Gear.SFX_Gear" 0.4 1.0 0.0 null null)
                (set `self.Gear?` true)
                (elif (== _pickupitem_ 0)
                  (`self.SetGearVisibility`)
                  (`/Game/PathOfLight/bp_Imports/HUD_UI.GearVisibility` _cooldownuiref)
                  (`SceneComponent.SetVisibility` (`self.YellowGear`) false false)
                  (`SceneComponent.SetVisibility` (`self.BlueGear`) false false)
                  (`SceneComponent.SetVisibility` (`self.RedGear`) false false)
                  (`SceneComponent.SetVisibility` (`self.GreenGear`) false false)
                  (set `self.PlacedItem` "None")
                  (set `self.Gear?` false))))))))))

(event `self.Sphere.OnComponentBeginOverlap`
  (params (OverlappedComponent :type "PrimitiveComponent Object Reference") (OtherActor :type "Actor Object Reference") (OtherComp :type "PrimitiveComponent Object Reference") (OtherBodyIndex :type Integer) (bFromSweep :type Boolean) (SweepResult :type "HitResult Structure (by ref)"))
  ;[1 1 1] Pedestal Interaction
  (bind _asbp_character (cast `/Game/PathOfLight/bp_Imports/bp_Character` OtherActor))
  (set `/Game/PathOfLight/bp_Imports/bp_Character.G4Overlap?` true _asbp_character)
  (`MeshComponent.SetOverlayMaterial` (`self.Terminal`) "/Game/PathOfLight/Materials/m_Outline_Inst.m_Outline_Inst")
  (goto _label_3 :!via `Open`))

(event `self.Sphere.OnComponentEndOverlap`
  (params (OverlappedComponent :type "PrimitiveComponent Object Reference") (OtherActor :type "Actor Object Reference") (OtherComp :type "PrimitiveComponent Object Reference") (OtherBodyIndex :type Integer))
  ;[1 1 1] Pedestal Interaction
  (bind _asbp_character (cast `/Game/PathOfLight/bp_Imports/bp_Character` OtherActor))
  (set `/Game/PathOfLight/bp_Imports/bp_Character.G4Overlap?` false _asbp_character)
  (`MeshComponent.SetOverlayMaterial` (`self.Terminal`) null)
  (goto _label_3 :!via `Close`))

(fn `UserConstructionScript`)