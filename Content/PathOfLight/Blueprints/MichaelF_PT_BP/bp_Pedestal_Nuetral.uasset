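; Neutral pedestal where the player places a carried blue, red, yellow or green pickup.
; A sphere overlap with bp_Character outlines the cube and opens a Gate, so Interact only works in range while an item is held.
; A FlipFlop alternates between spawning the matching pickup at the socket while zeroing the character's PickupItem, and setting PlacedItem to None.
; The second branch does not destroy the spawned pickup.
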(event `self.ReceiveBeginPlay`
  ;[1 1 1] Pedestal Interaction
  (`self.EnableInput` (`GameplayStatics.GetPlayerController` 0)))

(event `EnhancedInput|/Game/PathOfLight/bp_Imports/ia_Interact`
  (params (ActionValue :type Boolean) (ElapsedSeconds :type "Float (double-precision)") (TriggeredSeconds :type "Float (double-precision)") (InputAction :type "InputAction Object Reference" :default "/Game/PathOfLight/bp_Imports/ia_Interact.ia_Interact"))
  ;[1 1 1] Pedestal Interaction
  (:`Triggered`
    (bind _asbp_character (cast `/Game/PathOfLight/bp_Imports/bp_Character` (`GameplayStatics.GetPlayerCharacter` 0)))
    (if (> (`/Game/PathOfLight/bp_Imports/bp_Character.PickupItem#` _asbp_character) 0)
      (`/Engine/EditorBlueprintResources/StandardMacros.Gate` true :!label _label
        (:`Exit`
          (`/Engine/EditorBlueprintResources/StandardMacros.FlipFlop`
            (:`A`
              (bind _pickupitem_ (`/Game/PathOfLight/bp_Imports/bp_Character.PickupItem#` _asbp_character))
              ;[1 1 1] If the Player has picked up either blue or red cubes
              (if (== _pickupitem_ 1)
                (`|SpawnActorFromClass` "/Game/PathOfLight/Blueprints/MichaelF_PT_BP/bp_BluePickup.bp_BluePickup_C" (`SceneComponent.K2_GetComponentToWorld` (`self.Socket`)) "Undefined" "MultiplyWithRoot" null null)
                (set `/Game/PathOfLight/bp_Imports/bp_Character.PickupItem#` 0 _asbp_character)
                (elif (== _pickupitem_ 2)
                  (`|SpawnActorFromClass` "/Game/PathOfLight/Blueprints/MichaelF_PT_BP/bp_RedPickup.bp_RedPickup_C" (`SceneComponent.K2_GetComponentToWorld` (`self.Socket`)) "Undefined" "MultiplyWithRoot" null null)
                  (set `/Game/PathOfLight/bp_Imports/bp_Character.PickupItem#` 0 _asbp_character)
                  (elif (== _pickupitem_ 3)
                    (`|SpawnActorFromClass` "/Game/PathOfLight/Blueprints/MichaelF_PT_BP/bp_YellowPickup.bp_YellowPickup_C" (`SceneComponent.K2_GetComponentToWorld` (`self.Socket`)) "Undefined" "MultiplyWithRoot" null null)
                    (set `/Game/PathOfLight/bp_Imports/bp_Character.PickupItem#` 0 _asbp_character)
                    (elif (== _pickupitem_ 4)
                      (`|SpawnActorFromClass` "/Game/PathOfLight/Blueprints/MichaelF_PT_BP/bp_GreenPickup.bp_GreenPickup_C" (`SceneComponent.K2_GetComponentToWorld` (`self.Socket`)) "Undefined" "MultiplyWithRoot" null null)
                      (set `/Game/PathOfLight/bp_Imports/bp_Character.PickupItem#` 0 _asbp_character))))))
            (:`B`
              ;[1 1 1] Player AbIlity to take off placed item
              (set `self.PlacedItem` "None"))))))))

(event `self.Sphere.OnComponentBeginOverlap`
  (params (OverlappedComponent :type "PrimitiveComponent Object Reference") (OtherActor :type "Actor Object Reference") (OtherComp :type "PrimitiveComponent Object Reference") (OtherBodyIndex :type Integer) (bFromSweep :type Boolean) (SweepResult :type "HitResult Structure (by ref)"))
  ;[1 1 1] Pedestal Interaction
  (cast `/Game/PathOfLight/bp_Imports/bp_Character` OtherActor)
  (`MeshComponent.SetOverlayMaterial` (`self.Cube`) "/Game/PathOfLight/Materials/m_Outline_Inst.m_Outline_Inst")
  (goto _label :!via `Open`))

(event `self.Sphere.OnComponentEndOverlap`
  (params (OverlappedComponent :type "PrimitiveComponent Object Reference") (OtherActor :type "Actor Object Reference") (OtherComp :type "PrimitiveComponent Object Reference") (OtherBodyIndex :type Integer))
  ;[1 1 1] Pedestal Interaction
  (cast `/Game/PathOfLight/bp_Imports/bp_Character` OtherActor)
  (`MeshComponent.SetOverlayMaterial` (`self.Cube`) null)
  (goto _label :!via `Close`))

(fn `UserConstructionScript`)