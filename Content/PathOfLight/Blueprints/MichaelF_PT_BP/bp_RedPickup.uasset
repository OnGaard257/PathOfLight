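; Red puzzle pickup that the player collects with the interact input while standing in range.
; Overlap with the Sphere toggles an outline overlay material on the Gear and opens or closes a Gate that guards the interaction.
; If bp_Character holds no item, interacting destroys the actor and sets the character's PickupItem to the red item's ID.
; RedShutdown destroys the Sphere to disable interactivity on puzzle completion.
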(event `self.ReceiveBeginPlay`
  ;[1 1 1] Enables Player Input
  (`self.EnableInput` (`GameplayStatics.GetPlayerController` 0)))

(event `RedShutdown`
  ;[1 1 1] Destroys Interactivity upon Puzzle Completion
  (`ActorComponent.K2_DestroyComponent` (`self.Sphere`)))

(event `EnhancedInput|/Game/PathOfLight/bp_Imports/ia_Interact`
  (params (ActionValue :type Boolean) (ElapsedSeconds :type "Float (double-precision)") (TriggeredSeconds :type "Float (double-precision)") (InputAction :type "InputAction Object Reference" :default "/Game/PathOfLight/bp_Imports/ia_Interact.ia_Interact"))
  ;[1 1 1] Red Cube Pickup Cube Interactions
  (:`Triggered`
    (bind _asbp_character (cast `/Game/PathOfLight/bp_Imports/bp_Character` (`GameplayStatics.GetPlayerPawn` 0)))
    (if (== (`/Game/PathOfLight/bp_Imports/bp_Character.PickupItem#` _asbp_character) 0)
      (`/Engine/EditorBlueprintResources/StandardMacros.Gate` true :!label _label
        (:`Exit`
          (`self.K2_DestroyActor`)
          (set `/Game/PathOfLight/bp_Imports/bp_Character.PickupItem#` 2 _asbp_character))))))

(event `self.Sphere.OnComponentBeginOverlap`
  (params (OverlappedComponent :type "PrimitiveComponent Object Reference") (OtherActor :type "Actor Object Reference") (OtherComp :type "PrimitiveComponent Object Reference") (OtherBodyIndex :type Integer) (bFromSweep :type Boolean) (SweepResult :type "HitResult Structure (by ref)"))
  ;[1 1 1] Red Cube Pickup Cube Interactions
  (cast `/Game/PathOfLight/bp_Imports/bp_Character` OtherActor)
  (`MeshComponent.SetOverlayMaterial` (`self.Gear`) "/Game/PathOfLight/Materials/m_Outline_Inst.m_Outline_Inst")
  (goto _label :!via `Open`))

(event `self.Sphere.OnComponentEndOverlap`
  (params (OverlappedComponent :type "PrimitiveComponent Object Reference") (OtherActor :type "Actor Object Reference") (OtherComp :type "PrimitiveComponent Object Reference") (OtherBodyIndex :type Integer))
  ;[1 1 1] Red Cube Pickup Cube Interactions
  (cast `/Game/PathOfLight/bp_Imports/bp_Character` OtherActor)
  (`MeshComponent.SetOverlayMaterial` (`self.Gear`) null)
  (goto _label :!via `Close`))

(fn `UserConstructionScript`)