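; Shield actor with a ShieldVFX effect and a ShieldBounce overlap component, apparently an unfinished or disabled defense against patrolling enemies.
; On BeginPlay it doubles the effect's custom time dilation; the overlap and ShieldDelay events are empty.
; Disconnected logic would stun and launch an EnemyPatrol_withSound, or briefly reveal ShieldBounce after a delay, but none of it runs.
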(event `self.ReceiveBeginPlay`
  (`NiagaraComponent.SetCustomTimeDilation` (`self.Shield_VFX`) 2.0))

(event `Shield Delay`)

(event `self.Shield Bounce.OnComponentBeginOverlap`
  (params (OverlappedComponent :type "PrimitiveComponent Object Reference") (OtherActor :type "Actor Object Reference") (OtherComp :type "PrimitiveComponent Object Reference") (OtherBodyIndex :type Integer) (bFromSweep :type Boolean) (SweepResult :type "HitResult Structure (by ref)")))

(fn `UserConstructionScript`)