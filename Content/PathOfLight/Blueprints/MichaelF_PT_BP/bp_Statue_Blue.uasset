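; Blue statue puzzle actor that rotates to a correct or incorrect orientation depending on the colored cube event it receives.
; Timelines lerp the statue's relative rotation: blue turns it to the correct rotation with a one-time stone sound, while yellow, red and green turn it to wrong ones.
; RotateBackToDefault reads the character's PickupItem to choose which incorrect-rotation timeline to reverse.
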(event `CorrectRotation(BlueCube)`
  ;[1 1 1] Correct Rotation (Blue Cube PT)
  (bind (_direction _incorrect_rotation) (`Timeline|Timeline_0` :!via `PlayFromStart`)
    (:`Update`
      (`SceneComponent.K2_SetRelativeRotation` (`self.Statue_Blue`) (`KismetMathLibrary.RLerp` (`self.Starting Rotation`) (`self.Correct Rotation`) _incorrect_rotation true) false false)
      (`/Engine/EditorBlueprintResources/StandardMacros.DoOnce` false
        (:`Completed`
          (`GameplayStatics.PlaySound2D` "/Game/PathOfLight/Sounds/ColeSFX/StoneRotate.StoneRotate" 1.0 1.3 0.0 null null false))))))

(event `IncorrectRotation(Yellow Cube)`
  ;[1 1 1] Incorrect Rotation for Statue (Yellow Cube PT)
  (bind (_direction _incorrect_rotation) (`Timeline|Timeline_1` :!label _label)
    (:`Update`
      (`SceneComponent.K2_SetRelativeRotation` (`self.Statue_Blue`) (`KismetMathLibrary.RLerp` (`self.Starting Rotation`) (`self.Incorrect Rotation_0`) _incorrect_rotation true) false false))))

(event `RotateBackToDefault`
  ;[1 1 1] Comment
  (bind _returnvalue (`GameplayStatics.GetActorOfClass` "/Game/PathOfLight/bp_Imports/bp_Character.bp_Character_C"))
  (bind _pickupitem_ (`/Game/PathOfLight/bp_Imports/bp_Character.PickupItem#` _returnvalue))
  (if (== _pickupitem_ 3)
    (goto _label :!via `Reverse`)
    (elif (== _pickupitem_ 2)
      ;[1 1 1] Incorrect Rotation for Statue (Red Cube PT)
      (bind (_direction _incorrect_rotation) (`Timeline|Timeline` :!via `Reverse` :!label _label_2)
        (:`Update`
          (`SceneComponent.K2_SetRelativeRotation` (`self.Statue_Blue`) (`KismetMathLibrary.RLerp` (`self.Starting Rotation`) (`self.Incorrect Rotation`) _incorrect_rotation true) false false)))
      (elif (== _pickupitem_ 4)
        (bind (_direction_2 _incorrect_rotation_2) (`Timeline|Timeline_2` :!via `Reverse` :!label _label_3)
          (:`Update`
            (`SceneComponent.K2_SetRelativeRotation` (`self.Statue_Blue`) (`KismetMathLibrary.RLerp` (`self.Starting Rotation`) (`self.Incorrect Rotation`) _incorrect_rotation_2 true) false false)))))))

(event `IncorrectRotation(RedCube)`
  ;[1 1 1] Incorrect Rotation for Statue (Red Cube PT)
  (goto _label_2))

(event `Incorrect Rotation (Green Cube)`
  (goto _label_3))

(fn `UserConstructionScript`)