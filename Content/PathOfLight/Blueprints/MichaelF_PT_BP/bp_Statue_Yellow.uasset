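; Yellow statue puzzle actor that rotates in response to colored cube events.
; The correct-rotation event lerps the statue to its solved angle on a timeline and plays a stone sound, while incorrect-cube events only play a gear sound.
; RotateBack reads the character's PickupItem to choose which incorrect-rotation timeline to reverse.
; Disconnected Bp_Pedestal_R2 checks for an empty pedestal never run.
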(event `CorrectRotation`
  ;[1 1 1] Correct Rotation (Red Cube PT)
  (bind (_direction _rotation) (`Timeline|Timeline_0` :!via `PlayFromStart`)
    (:`Update`
      (`SceneComponent.K2_SetRelativeRotation` (`self.Statue_Yellow`) (`KismetMathLibrary.RLerp` (`self.Starting Rotation`) (`self.Correct Rotation`) _rotation) false false)
      (`/Engine/EditorBlueprintResources/StandardMacros.DoOnce` false
        (:`Completed`
          (`GameplayStatics.PlaySound2D` "/Game/PathOfLight/Sounds/ColeSFX/StoneRotate.StoneRotate" 1.0 1.3 0.0 null null false))))))

(event `IncorrectRotation (Red Cube)`
  ;[1 1 1] Incorrect Rotation (Red Cube)
  (`GameplayStatics.PlaySound2D` "/Game/PathOfLight/Sounds/NickSFX/SFX_Gear.SFX_Gear" 0.4 1.0 0.0 null null))

(event `Rotate Back`
  (bind _returnvalue (`GameplayStatics.GetActorOfClass` "/Game/PathOfLight/bp_Imports/bp_Character.bp_Character_C"))
  (bind _pickupitem_ (`/Game/PathOfLight/bp_Imports/bp_Character.PickupItem#` _returnvalue))
  (if (== _pickupitem_ 2)
    ;[1 1 1] Incorrect Rotation (Red Cube)
    (bind (_direction _rotation) (`Timeline|Timeline_1` :!via `Reverse`)
      (:`Update`
        (`SceneComponent.K2_SetRelativeRotation` (`self.Statue_Yellow`) (`KismetMathLibrary.RLerp` (`self.Starting Rotation`) (`self.Incorrect Rotation_0`) _rotation true) false false)))
    (elif (== _pickupitem_ 1)
      ;[1 1 1] Incorrect Rotation (Blue Cube PT)
      (bind (_direction_2 _rotation_2) (`Timeline|Timeline` :!via `Reverse`)
        (:`Update`
          (`SceneComponent.K2_SetRelativeRotation` (`self.Statue_Yellow`) (`KismetMathLibrary.RLerp` (`self.Starting Rotation`) (`self.Incorrect Rotation`) _rotation_2 true) false false)))
      (elif (== _pickupitem_ 4)
        (bind (_direction_3 _rotation_3) (`Timeline|Timeline_2` :!via `Reverse`)
          (:`Update`
            (`SceneComponent.K2_SetRelativeRotation` (`self.Statue_Yellow`) (`KismetMathLibrary.RLerp` (`self.Starting Rotation`) (`self.Incorrect Rotation_0`) _rotation_3 true) false false)))))))

(event `IncorrectRotation(BlueCube)`
  ;[1 1 1] Incorrect Rotation (Blue Cube PT)
  (`GameplayStatics.PlaySound2D` "/Game/PathOfLight/Sounds/NickSFX/SFX_Gear.SFX_Gear" 0.4 1.0 0.0 null null))

(event `IncorrectRoation(Green Cube)`
  (`GameplayStatics.PlaySound2D` "/Game/PathOfLight/Sounds/NickSFX/SFX_Gear.SFX_Gear" 0.4 1.0 0.0 null null))

(fn `UserConstructionScript`)