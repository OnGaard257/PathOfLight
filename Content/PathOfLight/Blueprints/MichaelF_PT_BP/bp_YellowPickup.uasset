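; Yellow gear pickup for a puzzle, which the player collects with the interact input while standing inside its overlap sphere.
; Sphere overlap toggles an outline overlay on the gear and opens or closes a gate on the input.
; Pickup sets the character's PickupItem and yellow gear visual, then destroys itself, first spawning any carried blue, red or green pickup in its place as a swap.
; YellowShutdown removes the sphere when the puzzle completes.
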(event `YellowShutdown`
  ;[1 1 1] Destroys Interactivity upon Puzzle Conmpletion
  (`ActorComponent.K2_DestroyComponent` (`self.Sphere`)))

(event `self.ReceiveBeginPlay`
  ;[1 1 1] Enables Player Interaction
  (`self.EnableInput` (`GameplayStatics.GetPlayerController` 0)))

(event `EnhancedInput|/Game/PathOfLight/bp_Imports/ia_Interact`
  (params (ActionValue :type Boolean) (ElapsedSeconds :type "Float (double-precision)") (TriggeredSeconds :type "Float (double-precision)") (InputAction :type "InputAction Object Reference" :default "/Game/PathOfLight/bp_Imports/ia_Interact.ia_Interact"))
  (bind _defaultsceneroot (`self.DefaultSceneRoot`))
  (bind _returnvalue (`SceneComponent.K2_GetComponentRotation` _defaultsceneroot))
  (bind _returnvalue_2 (`SceneComponent.K2_GetComponentLocation` _defaultsceneroot))
  (:`Triggered`
    (bind _asbp_character (cast `/Game/PathOfLight/bp_Imports/bp_Character` (`GameplayStatics.GetPlayerPawn` 0)))
    (`/Engine/EditorBlueprintResources/StandardMacros.Gate` true :!label _label
      (:`Exit`
        (if (== (`/Game/PathOfLight/bp_Imports/bp_Character.PickupItem#` _asbp_character) 0)
          (set `/Game/PathOfLight/bp_Imports/bp_Character.PickupItem#` 3 _asbp_character :!label _label_2)
          (bind _gear (`/Game/PathOfLight/bp_Imports/bp_Character.Gear` _asbp_character))
          (`PrimitiveComponent.SetMaterial` _gear 0 "/Game/PathOfLight/Materials/Test_MM_Yellow_Gear_Inst.Test_MM_Yellow_Gear_Inst")
          (`SceneComponent.SetVisibility` _gear true false)
          (`self.K2_DestroyActor`)
          (else
            (bind _pickupitem_ (`/Game/PathOfLight/bp_Imports/bp_Character.PickupItem#` _asbp_character))
            (if (== _pickupitem_ 1)
              (`|SpawnActorFromClass` "/Game/PathOfLight/Blueprints/MichaelF_PT_BP/bp_BluePickup.bp_BluePickup_C" (`KismetMathLibrary.MakeTransform` _returnvalue_2 _returnvalue) "AlwaysSpawn" "MultiplyWithRoot" null null)
              (`KismetSystemLibrary.DelayUntilNextTick` :!label _label_3)
              (goto _label_2)
              (elif (== _pickupitem_ 2)
                (`|SpawnActorFromClass` "/Game/PathOfLight/Blueprints/MichaelF_PT_BP/bp_RedPickup.bp_RedPickup_C" (`KismetMathLibrary.MakeTransform` _returnvalue_2 _returnvalue) "AlwaysSpawn" "MultiplyWithRoot" null null)
                (goto _label_3)
                (elif (== _pickupitem_ 4)
                  (`|SpawnActorFromClass` "/Game/PathOfLight/Blueprints/MichaelF_PT_BP/bp_GreenPickup.bp_GreenPickup_C" (`KismetMathLibrary.MakeTransform` _returnvalue_2 _returnvalue) "AlwaysSpawn" "MultiplyWithRoot" null null)
                  (goto _label_3))))))))))

(event `self.Sphere.OnComponentBeginOverlap`
  (params (OverlappedComponent :type "PrimitiveComponent Object Reference") (OtherActor :type "Actor Object Reference") (OtherComp :type "PrimitiveComponent Object Reference") (OtherBodyIndex :type Integer) (bFromSweep :type Boolean) (SweepResult :type "HitResult Structure (by ref)"))
  (cast `/Game/PathOfLight/bp_Imports/bp_Character` OtherActor)
  (`MeshComponent.SetOverlayMaterial` (`self.Gear`) "/Game/PathOfLight/Materials/m_Outline_Inst.m_Outline_Inst")
  (goto _label :!via `Open`))

(event `self.Sphere.OnComponentEndOverlap`
  (params (OverlappedComponent :type "PrimitiveComponent Object Reference") (OtherActor :type "Actor Object Reference") (OtherComp :type "PrimitiveComponent Object Reference") (OtherBodyIndex :type Integer))
  (cast `/Game/PathOfLight/bp_Imports/bp_Character` OtherActor)
  (`MeshComponent.SetOverlayMaterial` (`self.Gear`) null)
  (goto _label :!via `Close`))

(fn `UserConstructionScript`)