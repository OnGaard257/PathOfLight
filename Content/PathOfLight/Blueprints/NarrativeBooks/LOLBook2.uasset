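; Interactable narrative book (LOL Book 2) that the player opens and closes to read a page widget on screen.
; Box overlap flags the character as near the book, toggles actor input and applies an outline overlay to the mesh.
; Interaction calls Book2Interact, which toggles the Wbp_LOLBook2 widget with a pickup sound on open.
; While open, it shows the cursor, locks movement and look, and disables shield, dash, throw and stun-statue prayer, restoring them on close.
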(event `self.Box_0.OnComponentBeginOverlap`
  (params (OverlappedComponent :type "PrimitiveComponent Object Reference") (OtherActor :type "Actor Object Reference") (OtherComp :type "PrimitiveComponent Object Reference") (OtherBodyIndex :type Integer) (bFromSweep :type Boolean) (SweepResult :type "HitResult Structure (by ref)"))
  ;[1 1 1] Allows Player to Interact with Book when Near
  (bind _asbp_character (cast `/Game/PathOfLight/bp_Imports/bp_Character` OtherActor))
  (set `/Game/PathOfLight/bp_Imports/bp_Character.Book2Overlap?` true _asbp_character)
  (`self.EnableInput` (`GameplayStatics.GetPlayerController` 0))
  (`MeshComponent.SetOverlayMaterial` (`self.Book`) "/Game/PathOfLight/Materials/m_Outline_Inst.m_Outline_Inst"))

(event `self.Box_0.OnComponentEndOverlap`
  (params (OverlappedComponent :type "PrimitiveComponent Object Reference") (OtherActor :type "Actor Object Reference") (OtherComp :type "PrimitiveComponent Object Reference") (OtherBodyIndex :type Integer))
  ;[1 1 1] Allows Player to Interact with Book when Near
  (bind _asbp_character (cast `/Game/PathOfLight/bp_Imports/bp_Character` OtherActor))
  (set `/Game/PathOfLight/bp_Imports/bp_Character.Book2Overlap?` false _asbp_character)
  (`self.DisableInput` (`GameplayStatics.GetPlayerController` 0))
  (`MeshComponent.SetOverlayMaterial` (`self.Book`) null))

(event `Book2Interact`
  (bind _returnvalue (`GameplayStatics.GetPlayerController` 0))
  (bind _returnvalue_2 (`GameplayStatics.GetPlayerCharacter` 0))
  (bind _returnvalue_3 (`GameplayStatics.GetPlayerController` 0))
  (bind _lol2pages (`self.LOL2Pages`))
  ;[1 1 1] Interact Event
  (`/Engine/EditorBlueprintResources/StandardMacros.IsValid` (`self.LOL2Pages`)
    (:`Is Valid`
      ;[1 1 1] Remove Book From Screen
      (`Widget.RemoveFromParent` (`self.LOL2Pages`))
      (set `self.LOL2Pages` null)
      ;[1 1 1] Restores Player Control
      (`WidgetBlueprintLibrary.SetInputMode_GameOnly` _returnvalue_3)
      (set `PlayerController.bShowMouseCursor` false _returnvalue_3)
      (`CharacterMovementComponent.SetMovementMode` (`Character.CharacterMovement` _returnvalue_2) "MOVE_Walking" 0)
      (`Controller.SetIgnoreLookInput` _returnvalue false)
      (bind _asbp_character (cast `/Game/PathOfLight/bp_Imports/bp_Character` (`GameplayStatics.GetPlayerCharacter` 0)))
      (set `/Game/PathOfLight/bp_Imports/bp_Character.CanUseShield?` true _asbp_character)
      (set `/Game/PathOfLight/bp_Imports/bp_Character.PrayAtStunStatue?` true _asbp_character)
      (set `/Game/PathOfLight/bp_Imports/bp_Character.CanDash?` true _asbp_character)
      (set `/Game/PathOfLight/bp_Imports/bp_Character.AbletoThrow?` true _asbp_character))
    (:`Is Not Valid`
      (`GameplayStatics.PlaySound2D` "/Game/PathOfLight/Sounds/NickSFX/SFX_PickupBook.SFX_PickupBook" 0.6 1.0 0.0 null null)
      ;[1 1 1] Adds Book to Screen
      (bind _returnvalue_4 (`|CreateWidget` "/Game/PathOfLight/UI/Journal_Pages/JournalSwitchers/wbp_LOLBook2.wbp_LOLBook2_C"))
      (bind _output_get (set `self.LOL2Pages` _returnvalue_4))
      (`UserWidget.AddToViewport` _output_get 0)
      ;[1 1 1] Removes Player Control (UI Only)
      (`WidgetBlueprintLibrary.SetInputMode_GameAndUIEx` _returnvalue_3 null)
      (`Widget.SetUserFocus` _lol2pages _returnvalue_3)
      (`Widget.SetKeyboardFocus` _lol2pages)
      (set `PlayerController.bShowMouseCursor` true _returnvalue_3)
      (`CharacterMovementComponent.DisableMovement` (`Character.CharacterMovement` _returnvalue_2))
      (`Controller.SetIgnoreLookInput` _returnvalue true)
      (bind _asbp_character_2 (cast `/Game/PathOfLight/bp_Imports/bp_Character` (`GameplayStatics.GetPlayerCharacter` 0)))
      (set `/Game/PathOfLight/bp_Imports/bp_Character.CanUseShield?` false _asbp_character_2)
      (set `/Game/PathOfLight/bp_Imports/bp_Character.PrayAtStunStatue?` false _asbp_character_2)
      (set `/Game/PathOfLight/bp_Imports/bp_Character.CanDash?` false _asbp_character_2)
      (set `/Game/PathOfLight/bp_Imports/bp_Character.AbletoThrow?` false _asbp_character_2))))

(event `/Game/PathOfLight/LD_Prototyping/JavonW/BPI_Interface.Interaction`
  (`self.Book2Interact`))

(fn `UserConstructionScript`)