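; Readable Matriarch narrative book that opens a page-switcher journal widget for the player.
; Box overlap outlines the book, enables input and sets the character's MatriarchBookOverlap flag.
; MatriarchBookInteract shows the widget unless a journal is already on screen, freezing movement and look and disabling shield, dash, throw and statue prayer.
; Close keys remove the widget and restore control, re-enabling those abilities after a short delay.
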(event OnComponentBeginOverlap(Box)
  (params (OverlappedComponent :type Primitive%20Component%20Object%20Reference) (OtherActor :type Actor%20Object%20Reference) (OtherComp :type Primitive%20Component%20Object%20Reference) (OtherBodyIndex :type Integer) (bFromSweep :type Boolean) (SweepResult :type Hit%20Result%20Structure%20%28by%20ref%29))
  ;[1 1 1] Allows Player to Interact with Book when Near
  (bind _asbp_character (Utilities|Casting|CastTobp_Character OtherActor))
  (Variables|/Game/PathOfLight/bp_Imports/bp_Character.bp_Character_C|SetMatriarchBookOverlap? _asbp_character true)
  (Input|EnableInput (Game|GetPlayerController 0))
  (Rendering|Material|SetOverlayMaterial (Variables|Default|GetBook) "/Game/PathOfLight/Materials/m_Outline_Inst.m_Outline_Inst" :!class /Script/Engine.MeshComponent))

(event OnComponentEndOverlap(Box)
  (params (OverlappedComponent :type Primitive%20Component%20Object%20Reference) (OtherActor :type Actor%20Object%20Reference) (OtherComp :type Primitive%20Component%20Object%20Reference) (OtherBodyIndex :type Integer))
  ;[1 1 1] Allows Player to Interact with Book when Near
  (bind _asbp_character (Utilities|Casting|CastTobp_Character OtherActor))
  (Variables|/Game/PathOfLight/bp_Imports/bp_Character.bp_Character_C|SetMatriarchBookOverlap? _asbp_character false)
  (Input|DisableInput (Game|GetPlayerController 0))
  (Rendering|Material|SetOverlayMaterial (Variables|Default|GetBook) 0 :!class /Script/Engine.MeshComponent))

(event Custom|MatriarchBookInteract
  (bind _returnvalue (Game|GetPlayerController 0))
  ;[1 1 1] Adds Book to Screen
  (bind _asbp_character (Utilities|Casting|CastTobp_Character (Game|GetPlayerCharacter 0)))
  (if (not (and (UserInterface|Viewport|IsinViewport (Variables|/Game/PathOfLight/bp_Imports/bp_Character.bp_Character_C|GetCurrentJournal _asbp_character)) (Utilities|IsValid (Variables|/Game/PathOfLight/bp_Imports/bp_Character.bp_Character_C|GetCurrentJournal _asbp_character))))
    (Audio|PlaySound2D "/Game/PathOfLight/Sounds/NickSFX/SFX_PickupBook.SFX_PickupBook" 0.6 1.0 0.0 0 0)
    (bind _returnvalue_2 (UserInterface|CreateWidget "/Game/PathOfLight/UI/Journal_Pages/JournalSwitchers/wbp_switcher_NB.wbp_switcher_NB_C"))
    (bind _output_get (Variables|Default|SetActivePages _returnvalue_2))
    (UserInterface|Viewport|AddtoViewport _output_get 0)
    (Variables|/Game/PathOfLight/bp_Imports/bp_Character.bp_Character_C|SetCurrentJournal _asbp_character _returnvalue_2)
    ;[1 1 1] Removes Player Control (UI Only)
    (Input|SetInputModeGameandUI _returnvalue 0 "DoNotLock" true false)
    (Class|Widget|SetUserFocus (Variables|Default|GetActivePages) _returnvalue)
    (Widget|SetKeyboardFocus (Variables|Default|GetActivePages))
    (Variables|/Script/Engine.PlayerController|SetbShowMouseCursor _returnvalue true)
    (Pawn|Components|CharacterMovement|DisableMovement (Variables|/Script/Engine.Character|GetCharacterMovement (Game|GetPlayerCharacter 0)))
    (Input|SetIgnoreLookInput (Game|GetPlayerController 0) true)
    (bind _asbp_character_2 (Utilities|Casting|CastTobp_Character (Game|GetPlayerCharacter 0)))
    (Variables|/Game/PathOfLight/bp_Imports/bp_Character.bp_Character_C|SetCanUseShield? _asbp_character_2 false)
    (Variables|/Game/PathOfLight/bp_Imports/bp_Character.bp_Character_C|SetPrayAtStunStatue? _asbp_character_2 false)
    (Variables|/Game/PathOfLight/bp_Imports/bp_Character.bp_Character_C|SetCanDash? _asbp_character_2 false)
    (Variables|/Game/PathOfLight/bp_Imports/bp_Character.bp_Character_C|SetAbletoThrow? _asbp_character_2 false)))

(event Input|KeyboardEvents|DebugKeyF
  (params (Key :type Key%20Structure :default "None") (ActionValue :type Input%20Action%20Value%20Structure))
  (bind _returnvalue (Game|GetPlayerController 0))
  ;[1 1 1] Remove Book From Screen
  (:Pressed
    (Widget|RemovefromParent (Variables|Default|GetActivePages))
    (Variables|Default|SetActivePages 0)
    ;[1 1 1] Restores Player Control
    (Input|SetInputModeGameOnly _returnvalue false)
    (Variables|/Script/Engine.PlayerController|SetbShowMouseCursor _returnvalue false)
    (Pawn|Components|CharacterMovement|SetMovementMode (Variables|/Script/Engine.Character|GetCharacterMovement (Game|GetPlayerCharacter 0)) "MOVE_Walking" 0)
    (Input|SetIgnoreLookInput (Game|GetPlayerController 0) false)
    (bind _asbp_character (Utilities|Casting|CastTobp_Character (Game|GetPlayerCharacter 0)))
    (Utilities|FlowControl|Delay 0.2)
    (Variables|/Game/PathOfLight/bp_Imports/bp_Character.bp_Character_C|SetCanUseShield? _asbp_character true)
    (Variables|/Game/PathOfLight/bp_Imports/bp_Character.bp_Character_C|SetPrayAtStunStatue? _asbp_character true)
    (Variables|/Game/PathOfLight/bp_Imports/bp_Character.bp_Character_C|SetCanDash? _asbp_character true)
    (Variables|/Game/PathOfLight/bp_Imports/bp_Character.bp_Character_C|SetAbletoThrow? _asbp_character true)))

(event Input|GamepadEvents|GamepadFaceButtonRight
  (params (Key :type Key%20Structure :default "None"))
  (bind _returnvalue (Game|GetPlayerController 0))
  ;[1 1 1] Remove Book From Screen
  (:Pressed
    (Widget|RemovefromParent (Variables|Default|GetActivePages))
    (Variables|Default|SetActivePages 0)
    ;[1 1 1] Restores Player Control
    (Input|SetInputModeGameOnly _returnvalue false)
    (Variables|/Script/Engine.PlayerController|SetbShowMouseCursor _returnvalue false)
    (Pawn|Components|CharacterMovement|SetMovementMode (Variables|/Script/Engine.Character|GetCharacterMovement (Game|GetPlayerCharacter 0)) "MOVE_Walking" 0)
    (Input|SetIgnoreLookInput (Game|GetPlayerController 0) false)
    (bind _asbp_character (Utilities|Casting|CastTobp_Character (Game|GetPlayerCharacter 0)))
    (Utilities|FlowControl|Delay 0.2)
    (Variables|/Game/PathOfLight/bp_Imports/bp_Character.bp_Character_C|SetCanUseShield? _asbp_character true)
    (Variables|/Game/PathOfLight/bp_Imports/bp_Character.bp_Character_C|SetPrayAtStunStatue? _asbp_character true)
    (Variables|/Game/PathOfLight/bp_Imports/bp_Character.bp_Character_C|SetCanDash? _asbp_character true)
    (Variables|/Game/PathOfLight/bp_Imports/bp_Character.bp_Character_C|SetAbletoThrow? _asbp_character true)))

(event Input|KeyboardEvents|Escape
  (params (Key :type Key%20Structure :default "None"))
  (bind _returnvalue (Game|GetPlayerController 0))
  ;[1 1 1] Remove Book From Screen
  (:Pressed
    (Widget|RemovefromParent (Variables|Default|GetActivePages))
    (Variables|Default|SetActivePages 0)
    ;[1 1 1] Restores Player Control
    (Input|SetInputModeGameOnly _returnvalue false)
    (Variables|/Script/Engine.PlayerController|SetbShowMouseCursor _returnvalue false)
    (Pawn|Components|CharacterMovement|SetMovementMode (Variables|/Script/Engine.Character|GetCharacterMovement (Game|GetPlayerCharacter 0)) "MOVE_Walking" 0)
    (Input|SetIgnoreLookInput (Game|GetPlayerController 0) false)
    (bind _asbp_character (Utilities|Casting|CastTobp_Character (Game|GetPlayerCharacter 0)))
    (Utilities|FlowControl|Delay 0.2)
    (Variables|/Game/PathOfLight/bp_Imports/bp_Character.bp_Character_C|SetCanUseShield? _asbp_character true)
    (Variables|/Game/PathOfLight/bp_Imports/bp_Character.bp_Character_C|SetPrayAtStunStatue? _asbp_character true)
    (Variables|/Game/PathOfLight/bp_Imports/bp_Character.bp_Character_C|SetCanDash? _asbp_character true)
    (Variables|/Game/PathOfLight/bp_Imports/bp_Character.bp_Character_C|SetAbletoThrow? _asbp_character true)))

(fn ConstructionScript)