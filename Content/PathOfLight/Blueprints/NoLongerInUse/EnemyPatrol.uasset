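; Enemy character that patrols, chases seen pawns and can be stunned, stored in a NoLongerInUse folder.
; Chained AIMoveTo calls loop through four patrol points, and a growl plays at world origin on BeginPlay.
; PawnSensing triggers a faster chase, with a retriggerable delay resuming patrol shortly after the last sighting.
; A bp_Stun hit destroys that actor and briefly disables movement before restoring walking.
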(event `self.ReceiveBeginPlay`
  (`self.EnemyPatrol`)
  (`GameplayStatics.PlaySoundAtLocation` "/Game/PathOfLight/Sounds/Monster_Growl.Monster_Growl" (0.0 0.0 0.0) (struct) 0.7 1.0 0.0 null null null null))

(event `EnemyPatrol`
  (set `CharacterMovementComponent.MaxWalkSpeed` 200.0 (`self.CharacterMovement`))
  (`|AIMoveTo` self (`self.Patrol1`) null
    (:`OnSuccess`
      (`|AIMoveTo` self (`self.Patrol2`) null
        (:`OnSuccess`
          (`|AIMoveTo` self (`self.Patrol3`) null
            (:`OnSuccess`
              (`|AIMoveTo` self (`self.Patrol4`) null
                (:`OnSuccess`
                  (`self.EnemyPatrol`))))))))))

(event `self.PawnSensing.OnSeePawn`
  (params (Pawn :type "Pawn Object Reference"))
  (set `CharacterMovementComponent.MaxWalkSpeed` 350.0 (`self.CharacterMovement`))
  (`|AIMoveTo` self (0.0 0.0 0.0) Pawn
    (:`then`
      (`KismetSystemLibrary.RetriggerableDelay` 2.0)
      (`self.EnemyPatrol`))))

(event `self.ReceiveHit`
  (params (MyComp :type "PrimitiveComponent Object Reference") (Other :type "Actor Object Reference") (OtherComp :type "PrimitiveComponent Object Reference") (bSelfMoved :type Boolean) (HitLocation :type "Vector Structure") (HitNormal :type "Vector Structure") (NormalImpulse :type "Vector Structure") (Hit :type "HitResult Structure (by ref)"))
  (bind _asbp_stun (cast `/Game/PathOfLight/Blueprints/bp_Stun` Other))
  (`self.K2_DestroyActor` _asbp_stun)
  (`CharacterMovementComponent.DisableMovement` (`self.CharacterMovement`))
  (`KismetSystemLibrary.Delay` 2.0)
  (`CharacterMovementComponent.SetMovementMode` (`self.CharacterMovement`) "MOVE_Walking" 0))

(fn `UserConstructionScript`)