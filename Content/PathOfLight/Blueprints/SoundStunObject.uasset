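; SoundStunObject is an interactable noise source that stuns the blind enemy (BP_BlindPT) while it is chasing.
; InteractCollider overlaps with the player character open and close a gate on the ia_Interact input.
; Interacting enables overlap events on LoudNoiseCollider for a few seconds, then disables them again.
; A BP_BlindPT that begins overlapping that collider gets its Stunned flag set if ChasingMode is on.
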(event `self.ReceiveBeginPlay`
  (`self.EnableInput` (`GameplayStatics.GetPlayerController` 0))
  (set `PrimitiveComponent.bGenerateOverlapEvents` false (`self.Loud Noise Collider`)))

(event `EnhancedInput|/Game/PathOfLight/bp_Imports/ia_Interact`
  (params (ActionValue :type Boolean) (ElapsedSeconds :type "Float (double-precision)") (TriggeredSeconds :type "Float (double-precision)") (InputAction :type "InputAction Object Reference" :default "/Game/PathOfLight/bp_Imports/ia_Interact.ia_Interact"))
  (bind _loud_noise_collider (`self.Loud Noise Collider`))
  (:`Triggered`
    (cast `/Game/PathOfLight/bp_Imports/bp_Character` (`GameplayStatics.GetPlayerCharacter` 0))
    (`/Engine/EditorBlueprintResources/StandardMacros.Gate` true :!label _label
      (:`Exit`
        (set `PrimitiveComponent.bGenerateOverlapEvents` true _loud_noise_collider)
        (`KismetSystemLibrary.Delay` 3.0)
        (set `PrimitiveComponent.bGenerateOverlapEvents` false _loud_noise_collider)))))

(event `self.Interact Collider.OnComponentBeginOverlap`
  (params (OverlappedComponent :type "PrimitiveComponent Object Reference") (OtherActor :type "Actor Object Reference") (OtherComp :type "PrimitiveComponent Object Reference") (OtherBodyIndex :type Integer) (bFromSweep :type Boolean) (SweepResult :type "HitResult Structure (by ref)"))
  (cast `/Game/PathOfLight/bp_Imports/bp_Character` OtherActor)
  (goto _label :!via `Open`))

(event `self.Interact Collider.OnComponentEndOverlap`
  (params (OverlappedComponent :type "PrimitiveComponent Object Reference") (OtherActor :type "Actor Object Reference") (OtherComp :type "PrimitiveComponent Object Reference") (OtherBodyIndex :type Integer))
  (cast `/Game/PathOfLight/bp_Imports/bp_Character` OtherActor)
  (goto _label :!via `Close`))

(event `self.Loud Noise Collider.OnComponentBeginOverlap`
  (params (OverlappedComponent :type "PrimitiveComponent Object Reference") (OtherActor :type "Actor Object Reference") (OtherComp :type "PrimitiveComponent Object Reference") (OtherBodyIndex :type Integer) (bFromSweep :type Boolean) (SweepResult :type "HitResult Structure (by ref)"))
  (bind _asbp_blind_pt (cast `/Game/PathOfLight/Blueprints/BP_BlindPT` OtherActor))
  (if (`/Game/PathOfLight/Blueprints/BP_BlindPT.ChasingMode` _asbp_blind_pt)
    (set `/Game/PathOfLight/Blueprints/BP_BlindPT.Stunned` true _asbp_blind_pt)))

(fn `UserConstructionScript`)