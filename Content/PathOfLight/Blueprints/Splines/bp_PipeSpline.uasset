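; Pipe spline Blueprint whose construction script spawns a spline mesh component for each fixed-length section along its spline.
; Section length can follow actor X scale, and a flag limits the pieces to full-length sections or allows one extra.
; Helper functions compute each section's local start and end positions and length-clamped tangents, but the nodes applying these and the collision setting are not connected to execution.
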(fn `Get_End_Pos/Tangent`
  (params (Index :type Integer))
  (returns (Position :type "Vector Structure") (Tangent :type "Vector Structure"))
  (bind _spline (`self.Spline`))
  (bind _returnvalue (* (+ Index 1) (`self.Section Length`)))
  (return (`SplineComponent.GetLocationAtDistanceAlongSpline` _spline _returnvalue "Local") (`KismetMathLibrary.ClampVectorSize` (`SplineComponent.GetTangentAtDistanceAlongSpline` _spline _returnvalue "Local") 0.0 (`self.Section Length`))))

(fn `Get_Start_Pos/Tangent`
  (params (Index :type Integer))
  (returns (Position :type "Vector Structure") (Tangent :type "Vector Structure"))
  (bind _spline (`self.Spline`))
  (bind _returnvalue (* Index (`self.Section Length`)))
  (return (`SplineComponent.GetLocationAtDistanceAlongSpline` _spline _returnvalue "Local") (`KismetMathLibrary.ClampVectorSize` (`SplineComponent.GetTangentAtDistanceAlongSpline` _spline _returnvalue "Local") 0.0 (`self.Section Length`))))

(fn `UserConstructionScript`
  (bind _returnvalue_x (`KismetMathLibrary.BreakVector` (`self.GetActorScale3D`)))
  (if (`self.Allow Scaling?`)
    (set `self.Section Length` (* _returnvalue_x 100.0)))
  (if (`self.MustBeFullLengthMeshes?`)
    (for _index (range (`KismetMathLibrary.FTrunc` (/ (`SplineComponent.GetSplineLength` (`self.Spline`)) (`self.Section Length`))))
      (set `self.Loop Index` _index)
      (bind _returnvalue (`AddComponent|NODE_AddSplineMeshComponent-0` :!label _label))
      (`StaticMeshComponent.SetStaticMesh` _returnvalue (`self.SplineMesh`))
      (`SplineMeshComponent.SetForwardAxis` _returnvalue "X" true)
      (bind (_position _tangent) (`self.Get_Start_Pos/Tangent` (`self.Loop Index`)))
      (bind (_position_2 _tangent_2) (`self.Get_End_Pos/Tangent` (`self.Loop Index`))))
    (else
      (for _index_2 (range (+ (`KismetMathLibrary.FTrunc` (/ (`SplineComponent.GetSplineLength` (`self.Spline`)) (`self.Section Length`))) 1))
        (set `self.Loop Index` _index_2)
        (goto _label)))))