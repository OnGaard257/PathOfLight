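; Tutorial trigger actor that shows the shield tutorial pop-up while the player character is inside its volume, then removes itself.
; Overlap begin on bp_Character creates WBP_ShieldTutorial and adds it to the viewport through a DoOnce, then resets a second DoOnce.
; Overlap end fires that second DoOnce, which removes the widget and destroys the actor after a short delay.
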(event `self.Trigger.OnComponentBeginOverlap`
  (params (OverlappedComponent :type "PrimitiveComponent Object Reference") (OtherActor :type "Actor Object Reference") (OtherComp :type "PrimitiveComponent Object Reference") (OtherBodyIndex :type Integer) (bFromSweep :type Boolean) (SweepResult :type "HitResult Structure (by ref)"))
  (cast `/Game/PathOfLight/bp_Imports/bp_Character` OtherActor)
  (`/Engine/EditorBlueprintResources/StandardMacros.DoOnce` false :!label _label
    (:`Completed`
      (bind _returnvalue (`|CreateWidget` "/Game/PathOfLight/UI/Tutorials/WBP_ShieldTutorial.WBP_ShieldTutorial_C"))
      (bind _output_get (set `self.ShieldTut` _returnvalue))
      (`UserWidget.AddToViewport` _output_get 0)
      (goto _label_2 :!via `Reset`))))

(event `self.Trigger.OnComponentEndOverlap`
  (params (OverlappedComponent :type "PrimitiveComponent Object Reference") (OtherActor :type "Actor Object Reference") (OtherComp :type "PrimitiveComponent Object Reference") (OtherBodyIndex :type Integer))
  (cast `/Game/PathOfLight/bp_Imports/bp_Character` OtherActor)
  (`/Engine/EditorBlueprintResources/StandardMacros.DoOnce` false :!label _label_2
    (:`Completed`
      (`Widget.RemoveFromParent` (`self.ShieldTut`))
      (`KismetSystemLibrary.Delay` 2.0)
      (`self.K2_DestroyActor`)
      (goto _label :!via `Reset`))))

(fn `UserConstructionScript`)