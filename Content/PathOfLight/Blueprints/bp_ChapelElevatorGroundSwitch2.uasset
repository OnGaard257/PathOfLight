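; Ground-floor call button for the second chapel elevator, which brings the elevator down when the player interacts with it.
; A box overlap with the player character sets its Ground2Overlap flag, enables input on the switch and outlines the button mesh, and leaving reverses all three.
; The interact event finds BP_ChapelElevator2 by class and triggers its ground-button event only if it is up, otherwise printing a debug message.
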(event `GroundSwitch2Interact`
  (bind _returnvalue (`GameplayStatics.GetActorOfClass` "/Game/PathOfLight/Blueprints/BP_ChapelElevator2.BP_ChapelElevator2_C"))
  (if (`/Game/PathOfLight/Blueprints/BP_ChapelElevator2.IsUp` _returnvalue)
    (`KismetSystemLibrary.PrintString` "ComingDown")
    (`/Game/PathOfLight/Blueprints/BP_ChapelElevator2.GroundButtonTriggered` _returnvalue)
    (else
      (`KismetSystemLibrary.PrintString` "AlreadyDown"))))

(event `self.Box.OnComponentBeginOverlap`
  (params (OverlappedComponent :type "PrimitiveComponent Object Reference") (OtherActor :type "Actor Object Reference") (OtherComp :type "PrimitiveComponent Object Reference") (OtherBodyIndex :type Integer) (bFromSweep :type Boolean) (SweepResult :type "HitResult Structure (by ref)"))
  (bind _asbp_character (cast `/Game/PathOfLight/bp_Imports/bp_Character` OtherActor))
  (set `/Game/PathOfLight/bp_Imports/bp_Character.Ground2Overlap?` true _asbp_character)
  (`self.EnableInput` (`GameplayStatics.GetPlayerController` 0))
  (`MeshComponent.SetOverlayMaterial` (`self.sm_ButtonDown`) "/Game/PathOfLight/Materials/m_Outline_Inst.m_Outline_Inst"))

(event `self.Box.OnComponentEndOverlap`
  (params (OverlappedComponent :type "PrimitiveComponent Object Reference") (OtherActor :type "Actor Object Reference") (OtherComp :type "PrimitiveComponent Object Reference") (OtherBodyIndex :type Integer))
  (bind _asbp_character (cast `/Game/PathOfLight/bp_Imports/bp_Character` OtherActor))
  (set `/Game/PathOfLight/bp_Imports/bp_Character.Ground2Overlap?` false _asbp_character)
  (`self.DisableInput` null)
  (`MeshComponent.SetOverlayMaterial` (`self.sm_ButtonDown`) null))

(fn `UserConstructionScript`)