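; Sleeping crow enemy that snores, wakes to chase the player, and returns to Point1 when it loses them.
; Per-tick line and sphere traces, plus a hearing overlap checking WalkingNoise, trigger the AI MoveTo chase.
; An attack overlap opens a timed swing window in which the Kill overlap destroys a non-invincible player and shows game over.
; Flash orbs stun it briefly; patrol logic is present but unused.
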(event `self.ReceiveBeginPlay`
  (`GameplayStatics.SpawnSoundAttached` "/Game/PathOfLight/Sounds/Crow_Snore.Crow_Snore" (`self.CapsuleComponent`) "None" (0.0 0.0 0.0) (struct) "KeepRelativeOffset" false (`self.Volume Multiplier`) 1.0 0.0 "/Game/PathOfLight/Sounds/GrowlSoundAttenuation.GrowlSoundAttenuation" null))

(event `self.GameOver.OnComponentBeginOverlap`
  (params (OverlappedComponent :type "PrimitiveComponent Object Reference") (OtherActor :type "Actor Object Reference") (OtherComp :type "PrimitiveComponent Object Reference") (OtherBodyIndex :type Integer) (bFromSweep :type Boolean) (SweepResult :type "HitResult Structure (by ref)"))
  ;[1 1 1] Game Over
  (if (`self.ActorHasTag` OtherActor "Player")
    (set `self.Attacking?` true)
    (`KismetSystemLibrary.Delay` 0.4)
    (`GameplayStatics.PlaySoundAtLocation` "/Game/PathOfLight/Sounds/monster-snarl-3-105348.monster-snarl-3-105348" (0.0 0.0 0.0) (struct) 0.6 1.0 0.0 null null null null)
    (set `self.Swinging` true)
    (`KismetSystemLibrary.Delay` 0.3)
    (set `self.Attacking?` false)
    (set `self.Swinging` false)
    (`self.Player Chase`)))

(event `Player Chase`
  ;[1 1 1] Player Chase
  (set `self.Volume Multiplier` 0.0)
  (set `self.Chase?` true)
  (bind _asbp_character (cast `/Game/PathOfLight/bp_Imports/bp_Character` (`GameplayStatics.GetPlayerPawn` 0)))
  (set `CharacterMovementComponent.MaxWalkSpeed` 400.0 (`self.CharacterMovement`))
  (`|AIMoveTo` self (0.0 0.0 0.0) _asbp_character
    (:`then`
      (`KismetSystemLibrary.RetriggerableDelay` 6.0)
      (if (`/Game/PathOfLight/bp_Imports/bp_Character.WalkingNoise` (stale `self.HearingAid.OnComponentBeginOverlap` _asbp_character))
        (`self.Player Chase` :!label _label)
        (elif (`self.ActorHasTag` (`.HitActor` (`GameplayStatics.BreakHitResult` (stale `self.ReceiveTick` _outhit_2))) "Player")
          (goto _label)
          (else
            (`self.Go Schleep`)))))))

(event `self.Kill.OnComponentBeginOverlap`
  (params (OverlappedComponent :type "PrimitiveComponent Object Reference") (OtherActor :type "Actor Object Reference") (OtherComp :type "PrimitiveComponent Object Reference") (OtherBodyIndex :type Integer) (bFromSweep :type Boolean) (SweepResult :type "HitResult Structure (by ref)"))
  ;[1 1 1] Game Over
  (bind _asbp_character (cast `/Game/PathOfLight/bp_Imports/bp_Character` OtherActor))
  (if (`self.Swinging`)
    (if (not (`/Game/PathOfLight/bp_Imports/bp_Character.IsInvincible?` _asbp_character))
      (`self.K2_DestroyActor` _asbp_character)
      (bind _returnvalue (`|CreateWidget` "/Game/PathOfLight/Blueprints/bp_Game_Over.bp_Game_Over_C"))
      (`UserWidget.AddToViewport` _returnvalue 0)
      (set `PlayerController.bShowMouseCursor` true (`GameplayStatics.GetPlayerController` 0)))))

(event `Go Schleep`
  ;[1 1 1] Go Schleep
  (set `CharacterMovementComponent.MaxWalkSpeed` 200.0 (`self.CharacterMovement`))
  (`|AIMoveTo` self (`self.Point1`) null
    (:`OnSuccess`
      (set `self.Chase?` false)
      (set `self.Volume Multiplier` 0.8))))

(event `Crow Step`
  ;[1 1 1] Crow Walk
  (`GameplayStatics.PlaySoundAtLocation` (`KismetArrayLibrary.Array_Random` (`self.CrowWalk`)) (`self.K2_GetActorLocation`) (struct) 0.4 1.0 0.0 "/Game/PathOfLight/Sounds/NewSoundAttenuation.NewSoundAttenuation" null null null))

(event `Random Patrol`
  ;[1 1 1] random patrol
)

(event `self.PawnSensing.OnSeePawn`
  (params (Pawn :type "Pawn Object Reference"))
  ;[1 1 1] Pawn Sensing
)

(event `self.ReceiveHit`
  (params (MyComp :type "PrimitiveComponent Object Reference") (Other :type "Actor Object Reference") (OtherComp :type "PrimitiveComponent Object Reference") (bSelfMoved :type Boolean) (HitLocation :type "Vector Structure") (HitNormal :type "Vector Structure") (NormalImpulse :type "Vector Structure") (Hit :type "HitResult Structure (by ref)"))
  ;[1 1 1] Stun Interation
)

(event `self.ReceiveActorBeginOverlap`
  (params (OtherActor :type "Actor Object Reference"))
  ;[1 1 1] Stun Interation
  (cast `/Game/PathOfLight/Blueprints/bp_Flash_Orb` OtherActor)
  (set `self.Stunned?` true)
  (`CharacterMovementComponent.DisableMovement` (`self.CharacterMovement`))
  (`AIPerceptionComponent.SetSenseEnabled` (`self.AIPerception`) "/Script/AIModule.AISense_Hearing" false)
  (`PawnSensingComponent.SetSensingUpdatesEnabled` (`self.PawnSensing`) false)
  (`KismetSystemLibrary.Delay` 4.0)
  (set `self.Stunned?` false)
  (`CharacterMovementComponent.SetMovementMode` (`self.CharacterMovement`) "MOVE_Walking" 0)
  (`AIPerceptionComponent.SetSenseEnabled` (`self.AIPerception`) "/Script/AIModule.AISense_Hearing" true)
  (`PawnSensingComponent.SetSensingUpdatesEnabled` (`self.PawnSensing`) true)
  (`KismetSystemLibrary.Delay` 0.2)
  (if (`self.ActorHasTag` (`.HitActor` (`GameplayStatics.BreakHitResult` (stale `self.ReceiveTick` _outhit_2))) "Player")
    (`self.Player Chase`)
    (else
      (`self.Go Schleep`))))

(event `self.ReceiveTick`
  (params (DeltaSeconds :type "Float (single-precision)"))
  (bind _eyesight2 (`self.eyesight2`))
  (bind _eyesight (`self.eyesight`))
  (bind _returnvalue (`SceneComponent.K2_GetComponentLocation` _eyesight))
  (bind _returnvalue_2 (`SceneComponent.K2_GetComponentLocation` _eyesight2))
  ;[1 1 1] Collision Tracing
  (bind _outactors (`GameplayStatics.GetAllActorsWithTag` "Enemy"))
  (bind (_outhit _returnvalue_3) (`KismetSystemLibrary.LineTraceSingleByProfile` _returnvalue (+ _returnvalue (* (`SceneComponent.GetForwardVector` _eyesight) 2000.0)) "Pawn" false _outactors))
  (bind (_outhit_2 _returnvalue_4) (`KismetSystemLibrary.SphereTraceSingle` _returnvalue_2 (+ _returnvalue_2 (* (`SceneComponent.GetForwardVector` _eyesight2) 700.0)) 75.0 "TraceTypeQuery1"))
  (`|ExecutionSequence`
    (:`then_0`
      (if _returnvalue_3
        (if (`self.ActorHasTag` (`.HitActor` (`GameplayStatics.BreakHitResult` _outhit)) "Player")
          (`/Engine/EditorBlueprintResources/StandardMacros.DoOnce` false
            (:`Completed`
              (`KismetSystemLibrary.PrintText` "Hit")
              (`GameplayStatics.GetActorOfClass` "bp_CrowUnderground_C")
              (`self.Player Chase`))))))
    (:`then_1`
      (if _returnvalue_4
        (if (`self.ActorHasTag` (`.HitActor` (`GameplayStatics.BreakHitResult` _outhit_2)) "Player")
          (`/Engine/EditorBlueprintResources/StandardMacros.DoOnce` false
            (:`Completed`
              (`KismetSystemLibrary.PrintText` "Hit")
              (`GameplayStatics.GetActorOfClass` "bp_CrowUnderground_C")
              (`self.Player Chase`))))))))

(event `Enemy Patrol`
  ;[1 1 1] Set Patrol
  (set `CharacterMovementComponent.MaxWalkSpeed` 200.0 (`self.CharacterMovement`))
  (`|AIMoveTo` self (`self.Point1`) null
    (:`OnSuccess`
      (`|AIMoveTo` self (`self.Point2`) null
        (:`OnSuccess`
          (`|AIMoveTo` self (`self.Point3`) null
            (:`OnSuccess`
              (`|AIMoveTo` self (`self.Point4`) null
                (:`then`
                  (`self.Enemy Patrol`))))))))))

(event `self.HearingAid.OnComponentBeginOverlap`
  (params (OverlappedComponent :type "PrimitiveComponent Object Reference") (OtherActor :type "Actor Object Reference") (OtherComp :type "PrimitiveComponent Object Reference") (OtherBodyIndex :type Integer) (bFromSweep :type Boolean) (SweepResult :type "HitResult Structure (by ref)"))
  (bind _asbp_character (cast `/Game/PathOfLight/bp_Imports/bp_Character` OtherActor))
  (if (`/Game/PathOfLight/bp_Imports/bp_Character.WalkingNoise` _asbp_character)
    (`self.Player Chase`)))

(fn `UserConstructionScript`)