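; Stealth enemy for Path of Light that roams the navmesh, hunts the player, and triggers game over when its attack kills them.
; Eyesight traces and PawnSensing hearing, affected by crouching and dashing, fill a decaying detection meter.
; A full meter triggers a notice pause and chase; giving up leads into a waypoint patrol.
; Flash orbs temporarily disable movement and senses, after which it re-checks for the player.
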(event `NewPatrolInOrder`)

(event `Step1`
  ;[1 1 1] Footsteps
  (`GameplayStatics.PlaySoundAtLocation` (`KismetArrayLibrary.Array_Random` (`self.Footsteps`)) (`self.K2_GetActorLocation`) (struct) 0.4 1.0 0.0 "/Game/PathOfLight/Sounds/GrowlSoundAttenuation.GrowlSoundAttenuation" null null null))

(event `Step2`
  ;[1 1 1] Footsteps
  (`GameplayStatics.PlaySoundAtLocation` (`KismetArrayLibrary.Array_Random` (`self.Footsteps`)) (`self.K2_GetActorLocation`) (struct) 0.4 1.0 0.0 "/Game/PathOfLight/Sounds/GrowlSoundAttenuation.GrowlSoundAttenuation" null null null))

(event `Set Patrol`
  (bind _stunned_ (`self.Stunned?`))
  (bind _returnvalue (>= (`self.DetectionTest1`) 10))
  ;[1 1 1] Set Patrol
  (`|ExecutionSequence`
    (:`then_0`
      (set `CharacterMovementComponent.MaxWalkSpeed` (`self.Max Walk Speed`) (`self.CharacterMovement`))
      (`|AIMoveTo` self (`self.Point1`) null
        (:`OnSuccess`
          (if _returnvalue
            (`self.NoticesYou` :!label _label)
            (else
              (bind _returnvalue_2 (`self.ActorHasTag` (`.HitActor` (`GameplayStatics.BreakHitResult` (stale `self.ReceiveTick` _outhit_4))) "Player"))
              (if _returnvalue_2
                (goto _label)
                (else
                  (`|AIMoveTo` self (`self.Point2`) null
                    (:`OnSuccess`
                      (`KismetSystemLibrary.Delay` 0.2)
                      (if _returnvalue
                        (`self.NoticesYou` :!label _label_2)
                        (elif _returnvalue_2
                          (goto _label_2)
                          (else
                            (`|AIMoveTo` self (`self.Point3`) null
                              (:`OnSuccess`
                                (set `self.LookAround?` true)
                                (`KismetSystemLibrary.Delay` 8.0)
                                (set `self.LookAround?` false)
                                (if _returnvalue
                                  (`self.NoticesYou` :!label _label_3)
                                  (elif _returnvalue_2
                                    (goto _label_3)
                                    (else
                                      (`|AIMoveTo` self (`self.Point4`) null
                                        (:`OnSuccess`
                                          (set `self.LookAround?` true)
                                          (`KismetSystemLibrary.Delay` 8.0)
                                          (set `self.LookAround?` false)
                                          (if _returnvalue
                                            (`self.NoticesYou` :!label _label_4)
                                            (elif _returnvalue_2
                                              (goto _label_4)
                                              (else
                                                (`|AIMoveTo` self (`self.Point5`) null
                                                  (:`OnSuccess`
                                                    (`KismetSystemLibrary.Delay` 0.2)
                                                    (if _returnvalue
                                                      (`self.NoticesYou` :!label _label_5)
                                                      (elif _returnvalue_2
                                                        (goto _label_5)
                                                        (else
                                                          (`|AIMoveTo` self (`self.Point6`) null
                                                            (:`OnSuccess`
                                                              (if _returnvalue
                                                                (`self.NoticesYou` :!label _label_6)
                                                                (elif _returnvalue_2
                                                                  (goto _label_6)
                                                                  (else
                                                                    (`self.Give Up`)))))))))))))))))))))))))))))))))
    (:`then_1`
      (goto _label_7 :!via `Reset`))
    (:`then_2`
      (`KismetSystemLibrary.Delay` 1.0)
      (goto _label_8 :!via `Reset`))))

(event `Give Up`
  ;[1 1 1] GIve Up
  (`/Engine/EditorBlueprintResources/StandardMacros.DoOnce` false :!label _label_7
    (:`Completed`
      (`CharacterMovementComponent.SetMovementMode` (`self.CharacterMovement`) "MOVE_None" 0)
      (set `self.Give Up?1` true)
      (`KismetSystemLibrary.Delay` 2.0)
      (`CharacterMovementComponent.SetMovementMode` (`self.CharacterMovement`) "MOVE_Walking" 0)
      (set `self.Give Up?1` false)
      (if (not (`self.Stunned?`))
        (`self.Set Patrol`)))))

(event `NoticesYou`
  ;[1 1 1] Notices You
  (set `self.LookAround?` false)
  (`/Engine/EditorBlueprintResources/StandardMacros.DoOnce` false :!label _label_8
    (:`Completed`
      (bind _asbp_character (cast `/Game/PathOfLight/bp_Imports/bp_Character` (`GameplayStatics.GetPlayerPawn` 0)))
      (`self.K2_SetActorRotation` (`KismetMathLibrary.Conv_VectorToRotator` (`SceneComponent.K2_GetComponentLocation` (`Character.Mesh` _asbp_character))))
      (`CharacterMovementComponent.SetMovementMode` (`self.CharacterMovement`) "MOVE_None" 0)
      (set `self.Noticed?1` true)
      (`KismetSystemLibrary.Delay` 2.0)
      (`CharacterMovementComponent.SetMovementMode` (`self.CharacterMovement`) "MOVE_Walking" 0)
      (set `self.Noticed?1` false)
      (if (not (`self.Stunned?`))
        (`self.Player Chase`)))))

(event `InitializeEnemy2`)

(event `self.ReceiveBeginPlay`
  (`self.Random Patrol`)
  (if (>= (`self.DetectionTest1`) 0)
    (set `self.DetectionTest1` 0)))

(event `Random Patrol`
  ;[1 1 1] random patrol
  (set `CharacterMovementComponent.MaxWalkSpeed` 200.0 (`self.CharacterMovement`))
  (bind _randomlocation (`NavigationSystemV1.K2_GetRandomLocationInNavigableRadius` (`self.K2_GetActorLocation`) 10000.0 null null))
  (`|AIMoveTo` self _randomlocation null 50.0
    (:`OnSuccess`
      (`self.Random Patrol`))))

(event `self.GameOver.OnComponentBeginOverlap`
  (params (OverlappedComponent :type "PrimitiveComponent Object Reference") (OtherActor :type "Actor Object Reference") (OtherComp :type "PrimitiveComponent Object Reference") (OtherBodyIndex :type Integer) (bFromSweep :type Boolean) (SweepResult :type "HitResult Structure (by ref)"))
  ;[1 1 1] Game Over
  (if (>= (`self.DetectionTest1`) 10)
    (if (`self.ActorHasTag` OtherActor "Player")
      (`KismetSystemLibrary.Delay` 0.2)
      (set `self.Attacking?` true)
      (`GameplayStatics.PlaySoundAtLocation` "/Game/PathOfLight/Sounds/monster-snarl-3-105348.monster-snarl-3-105348" (0.0 0.0 0.0) (struct) 0.6 1.0 0.0 null null null null)
      (`KismetSystemLibrary.Delay` 0.75)
      (set `self.Attacking?` false)
      (`self.NoticesYou`))))

(event `self.Kill.OnComponentBeginOverlap`
  (params (OverlappedComponent :type "PrimitiveComponent Object Reference") (OtherActor :type "Actor Object Reference") (OtherComp :type "PrimitiveComponent Object Reference") (OtherBodyIndex :type Integer) (bFromSweep :type Boolean) (SweepResult :type "HitResult Structure (by ref)"))
  ;[1 1 1] Game Over
  (bind _asbp_character (cast `/Game/PathOfLight/bp_Imports/bp_Character` OtherActor))
  (if (`self.Attacking?`)
    (if (not (`/Game/PathOfLight/bp_Imports/bp_Character.IsInvincible?` _asbp_character))
      (`self.K2_DestroyActor` _asbp_character)
      (bind _returnvalue (`|CreateWidget` "/Game/PathOfLight/Blueprints/bp_Game_Over.bp_Game_Over_C"))
      (`UserWidget.AddToViewport` _returnvalue 0)
      (set `PlayerController.bShowMouseCursor` true (`GameplayStatics.GetPlayerController` 0)))))

(event `Random Patrol Point`
  ;[1 1 1] Random patrol points
  (set `CharacterMovementComponent.MaxWalkSpeed` (`self.Max Walk Speed`) (`self.CharacterMovement`))
  (`|AIMoveTo` self (`KismetArrayLibrary.Array_Random` (`self.Patrol Array`)) null
    (:`OnSuccess`
      (`self.Random Patrol Point`))))

(event `Player Chase`
  ;[1 1 1] Player Chase
  (set `self.LookAround?` false)
  (bind _asbp_character (cast `/Game/PathOfLight/bp_Imports/bp_Character` (`GameplayStatics.GetPlayerPawn` 0)))
  (set `CharacterMovementComponent.MaxWalkSpeed` 450.0 (`self.CharacterMovement`))
  (set `self.Chasing1` true)
  (`|AIMoveTo` self (0.0 0.0 0.0) _asbp_character
    (:`then`
      (`KismetSystemLibrary.RetriggerableDelay` 6.0)
      (if (`self.ActorHasTag` (`.HitActor` (`GameplayStatics.BreakHitResult` (stale `self.ReceiveTick` _outhit_4))) "Player")
        (`self.NoticesYou`)
        (else
          (`self.Give Up`)
          (bind _output_get (set `self.Chasing1` false))
          (if _output_get
            (set `self.DetectionTest1` (- (`self.DetectionTest1`) 2))))))))

(event `self.ReceiveTick`
  (params (DeltaSeconds :type "Float (single-precision)"))
  (bind _eyesight2 (`self.eyesight2`))
  (bind _eyesight4 (`self.eyesight4`))
  (bind _eyesight3 (`self.eyesight3`))
  (bind _eyesight (`self.eyesight`))
  (bind _returnvalue (`SceneComponent.K2_GetComponentLocation` _eyesight4))
  (bind _returnvalue_2 (`SceneComponent.K2_GetComponentLocation` _eyesight2))
  (bind _returnvalue_3 (`SceneComponent.K2_GetComponentLocation` _eyesight))
  (bind _returnvalue_4 (`SceneComponent.K2_GetComponentLocation` _eyesight3))
  (`|ExecutionSequence`
    (:`then_0`
      ;[1 1 1] Collision Tracing
      (bind _outactors (`GameplayStatics.GetAllActorsWithTag` "Enemy"))
      (bind (_outhit _returnvalue_5) (`KismetSystemLibrary.LineTraceSingleByProfile` _returnvalue_3 (+ _returnvalue_3 (* (`SceneComponent.GetForwardVector` _eyesight) 2000.0)) "Pawn" false _outactors))
      (bind (_outhit_2 _returnvalue_6) (`KismetSystemLibrary.LineTraceSingleByProfile` _returnvalue_4 (+ _returnvalue_4 (* (`SceneComponent.GetForwardVector` _eyesight3) 2000.0)) "Pawn" false _outactors))
      (bind (_outhit_3 _returnvalue_7) (`KismetSystemLibrary.LineTraceSingleByProfile` _returnvalue (+ _returnvalue (* (`SceneComponent.GetForwardVector` _eyesight4) 2000.0)) "Pawn" false _outactors))
      (bind (_outhit_4 _returnvalue_8) (`KismetSystemLibrary.SphereTraceSingle` _returnvalue_2 (+ _returnvalue_2 (* (`SceneComponent.GetForwardVector` _eyesight2) 500.0)) 75.0 "TraceTypeQuery1" false _outactors))
      (`|ExecutionSequence`
        (:`then_0`
          (if _returnvalue_5
            (if (`self.ActorHasTag` (`.HitActor` (`GameplayStatics.BreakHitResult` _outhit)) "Player")
              (`/Engine/EditorBlueprintResources/StandardMacros.DoOnce` false :!label _label_9
                (:`Completed`
                  (set `self.LookAround?` false)
                  (set `self.DetectionTest1` (+ (`self.DetectionTest1`) 5))
                  (if (>= (`self.DetectionTest1`) 10)
                    (bind _returnvalue_9 (`GameplayStatics.GetActorOfClass` "bp_EnemyJavonThunderdome_C"))
                    (`self.NoticesYou` _returnvalue_9))
                  (`KismetSystemLibrary.Delay` 1.0)
                  (goto _label_9 :!via `Reset`))))))
        (:`then_1`
          (if _returnvalue_6
            (if (`self.ActorHasTag` (`.HitActor` (`GameplayStatics.BreakHitResult` _outhit_2)) "Player")
              (bind _asbp_character (cast `/Game/PathOfLight/bp_Imports/bp_Character` (`GameplayStatics.GetPlayerPawn` 0)))
              (if (not (`Character.bIsCrouched` _asbp_character))
                (`/Engine/EditorBlueprintResources/StandardMacros.DoOnce` false :!label _label_10
                  (:`Completed`
                    (set `self.LookAround?` false)
                    (set `self.DetectionTest1` (+ (`self.DetectionTest1`) 5))
                    (if (>= (`self.DetectionTest1`) 10)
                      (bind _returnvalue_10 (`GameplayStatics.GetActorOfClass` "bp_EnemyJavonThunderdome_C"))
                      (`self.NoticesYou` _returnvalue_10))
                    (`KismetSystemLibrary.Delay` 1.0)
                    (goto _label_10 :!via `Reset`)))))))
        (:`then_2`
          (if _returnvalue_7
            (if (`self.ActorHasTag` (`.HitActor` (`GameplayStatics.BreakHitResult` _outhit_3)) "Player")
              (bind _asbp_character_2 (cast `/Game/PathOfLight/bp_Imports/bp_Character` (`GameplayStatics.GetPlayerPawn` 0)))
              (if (not (`Character.bIsCrouched` _asbp_character_2))
                (`/Engine/EditorBlueprintResources/StandardMacros.DoOnce` false :!label _label_11
                  (:`Completed`
                    (set `self.LookAround?` false)
                    (set `self.DetectionTest1` (+ (`self.DetectionTest1`) 5))
                    (if (>= (`self.DetectionTest1`) 10)
                      (bind _returnvalue_11 (`GameplayStatics.GetActorOfClass` "bp_EnemyJavonThunderdome_C"))
                      (`self.NoticesYou` _returnvalue_11))
                    (`KismetSystemLibrary.Delay` 1.0)
                    (goto _label_11 :!via `Reset`)))))))
        (:`then_3`
          (if _returnvalue_8
            (if (`self.ActorHasTag` (`.HitActor` (`GameplayStatics.BreakHitResult` _outhit_4)) "Player")
              (`/Engine/EditorBlueprintResources/StandardMacros.DoOnce` false :!label _label_12
                (:`Completed`
                  (set `self.LookAround?` false)
                  (set `self.DetectionTest1` (+ (`self.DetectionTest1`) 5))
                  (if (>= (`self.DetectionTest1`) 10)
                    (bind _returnvalue_12 (`GameplayStatics.GetActorOfClass` "bp_EnemyJavonThunderdome_C"))
                    (`self.NoticesYou` _returnvalue_12))
                  (`KismetSystemLibrary.Delay` 1.0)
                  (goto _label_12 :!via `Reset`))))))))
    (:`then_1`
      (bind _asbp_character_3 (cast `/Game/PathOfLight/bp_Imports/bp_Character` (`GameplayStatics.GetPlayerPawn` 0)))
      (if (`/Game/PathOfLight/bp_Imports/bp_Character.IsDetected` _asbp_character_3)
        _
        (elif (`self.HearPlayer?1`)
          _
          (elif (not (<= (`self.DetectionTest1`) 0))
            (`KismetSystemLibrary.Delay` 0.5)
            (set `self.DetectionTest1` (- (`self.DetectionTest1`) 1))))))))

(event `DetectionCheck`
  (bind _returnvalue (`GameplayStatics.GetPlayerCharacter` 0))
  ;[1 1 1] DetectionCheck Event
  (if (or (>= (`self.DetectionTest1`) 10) (`self.Chasing1`))
    (bind _asbp_character (cast `/Game/PathOfLight/bp_Imports/bp_Character` _returnvalue))
    (set `/Game/PathOfLight/bp_Imports/bp_Character.IsDetected` true _asbp_character)
    (else
      (bind _asbp_character_2 (cast `/Game/PathOfLight/bp_Imports/bp_Character` _returnvalue))
      (set `/Game/PathOfLight/bp_Imports/bp_Character.IsDetected` false _asbp_character_2))))

(event `self.PawnSensing.OnSeePawn`
  (params (Pawn :type "Pawn Object Reference"))
  ;[1 1 1] Pawn Sensing
  (bind _asbp_character (cast `/Game/PathOfLight/bp_Imports/bp_Character` (`GameplayStatics.GetPlayerPawn` 0)))
  (if (`Character.bIsCrouched` _asbp_character)
    _
    (elif (>= (`self.DetectionTest1`) 10)
      (`self.NoticesYou`))))

(event `self.ReceiveHit`
  (params (MyComp :type "PrimitiveComponent Object Reference") (Other :type "Actor Object Reference") (OtherComp :type "PrimitiveComponent Object Reference") (bSelfMoved :type Boolean) (HitLocation :type "Vector Structure") (HitNormal :type "Vector Structure") (NormalImpulse :type "Vector Structure") (Hit :type "HitResult Structure (by ref)"))
  ;[1 1 1] stun interaction
)

(event `self.ReceiveActorBeginOverlap`
  (params (OtherActor :type "Actor Object Reference"))
  ;[1 1 1] stun interaction
  (cast `/Game/PathOfLight/Blueprints/bp_Flash_Orb` OtherActor)
  (set `self.Give Up?1` false)
  (set `self.LookAround?` false)
  (set `self.Noticed?1` false)
  (set `self.Stunned?` true)
  (`SceneComponent.SetVisibility` (`self.SpotLight`) false false)
  (`CharacterMovementComponent.DisableMovement` (`self.CharacterMovement`))
  (`AIPerceptionComponent.SetSenseEnabled` (`self.AIPerception`) "/Script/AIModule.AISense_Hearing" false)
  (`PawnSensingComponent.SetSensingUpdatesEnabled` (`self.PawnSensing`) false)
  (`KismetSystemLibrary.Delay` 4.0)
  (set `self.Stunned?` false)
  (`SceneComponent.SetVisibility` (`self.SpotLight`) false false)
  (`CharacterMovementComponent.SetMovementMode` (`self.CharacterMovement`) "MOVE_Walking" 0)
  (`AIPerceptionComponent.SetSenseEnabled` (`self.AIPerception`) "/Script/AIModule.AISense_Hearing" true)
  (`PawnSensingComponent.SetSensingUpdatesEnabled` (`self.PawnSensing`) true)
  (`KismetSystemLibrary.Delay` 0.2)
  (if (`self.ActorHasTag` (`.HitActor` (`GameplayStatics.BreakHitResult` (stale `self.ReceiveTick` _outhit_4))) "Player")
    (`self.NoticesYou`)
    (else
      (`self.Give Up`))))

(event `self.Hearing Aid.OnComponentBeginOverlap`
  (params (OverlappedComponent :type "PrimitiveComponent Object Reference") (OtherActor :type "Actor Object Reference") (OtherComp :type "PrimitiveComponent Object Reference") (OtherBodyIndex :type Integer) (bFromSweep :type Boolean) (SweepResult :type "HitResult Structure (by ref)"))
  (bind _asbp_character (cast `/Game/PathOfLight/bp_Imports/bp_Character` OtherActor)))

(event `self.PawnSensing.OnHearNoise`
  (params (Instigator :type "Pawn Object Reference") (Location :type "Vector Structure (by ref)") (Volume :type "Float (single-precision)"))
  (bind _returnvalue (>= (`self.DetectionTest1`) 10))
  ;[1 1 1] NEW Sound Detection, crouching acts as normal sound level for now
  (`|ExecutionSequence`
    (:`then_0`
      (bind _asbp_character (cast `/Game/PathOfLight/bp_Imports/bp_Character` Instigator))
      (if (`Character.bIsCrouched` _asbp_character)
        (set `self.DetectionTest1` (+ (`self.DetectionTest1`) 0))
        (`KismetSystemLibrary.Delay` 1.0)
        (if (>= (`self.DetectionTest1`) 10)
          (`self.NoticesYou`))
        (elif (`/Game/PathOfLight/bp_Imports/bp_Character.Dashing` _asbp_character)
          (if (not _returnvalue)
            (set `self.DetectionTest1` (+ (`self.DetectionTest1`) 4))
            (`KismetSystemLibrary.Delay` 1.0)
            (if (>= (`self.DetectionTest1`) 10)
              (`self.NoticesYou`)))
          (elif (not _returnvalue)
            (set `self.DetectionTest1` (+ (`self.DetectionTest1`) 2))
            (`KismetSystemLibrary.Delay` 1.0)
            (if (>= (`self.DetectionTest1`) 10)
              (`self.NoticesYou`))))))
    (:`then_1`
      (`/Engine/EditorBlueprintResources/StandardMacros.DoOnce` false :!label _label_13
        (:`Completed`
          (set `self.HearPlayer?1` true)
          (`KismetSystemLibrary.Delay` 1.0)
          (set `self.HearPlayer?1` false)
          (goto _label_13 :!via `Reset`))))))

(fn `UserConstructionScript`)