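; Patrolling monster enemy that loops six points, chases the player, and shows Game Over on overlap.
; Per-tick traces, some ignoring crouched players, fire one-shot chases on the first Bp_EnemyPatrol3 found, not necessarily itself.
; PawnSensing also starts chases on uncrouched players, while AIPerception sends it to investigate stimuli before resuming patrol.
; A bp_Stun hit destroys the stun actor and briefly disables movement and hearing.
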(event `self.ReceiveBeginPlay`
  (`self.Set Patrol`)
  (`GameplayStatics.SpawnSoundAttached` "/Game/PathOfLight/Sounds/Monster_Growl.Monster_Growl" (`self.CapsuleComponent`) "None" (0.0 0.0 0.0) (struct) "KeepRelativeOffset" false 1.0 1.0 0.0 null null))

(event `self.GameOver.OnComponentBeginOverlap`
  (params (OverlappedComponent :type "PrimitiveComponent Object Reference") (OtherActor :type "Actor Object Reference") (OtherComp :type "PrimitiveComponent Object Reference") (OtherBodyIndex :type Integer) (bFromSweep :type Boolean) (SweepResult :type "HitResult Structure (by ref)"))
  ;[1 1 1] Game Over
  (bind _asbp_character (cast `/Game/PathOfLight/bp_Imports/bp_Character` OtherActor))
  (`self.K2_DestroyActor` _asbp_character)
  (bind _returnvalue (`|CreateWidget` "/Game/PathOfLight/Blueprints/bp_Game_Over.bp_Game_Over_C"))
  (`UserWidget.AddToViewport` _returnvalue 0)
  (set `PlayerController.bShowMouseCursor` true (`GameplayStatics.GetPlayerController` 0)))

(event `Random Patrol`
  ;[1 1 1] random patrol
)

(event `Random Patrol Point`
  ;[1 1 1] Random patrol points
  (set `CharacterMovementComponent.MaxWalkSpeed` (`self.Max Walk Speed`) (`self.CharacterMovement`))
  (`|AIMoveTo` self (`KismetArrayLibrary.Array_Random` (`self.Patrol Array`)) null
    (:`OnSuccess`
      (`self.Random Patrol Point`))))

(event `Player Chase`
  (bind _returnvalue (`GameplayStatics.GetPlayerPawn` 0))
  ;[1 1 1] Player Chase
  (`|ExecutionSequence`
    (:`then_0`
      (bind _asbp_character_camera (cast `/Game/PathOfLight/LD_Prototyping/AshleyM/bp_character_camera` _returnvalue))
      (set `CharacterMovementComponent.MaxWalkSpeed` 400.0 (`self.CharacterMovement`))
      (`|AIMoveTo` self (0.0 0.0 0.0) _asbp_character_camera
        (:`then`
          (`KismetSystemLibrary.RetriggerableDelay` 2.0)
          (`self.Set Patrol`))))
    (:`then_1`
      (bind _asbp_character (cast `/Game/PathOfLight/bp_Imports/bp_Character` _returnvalue))
      (set `CharacterMovementComponent.MaxWalkSpeed` 400.0 (`self.CharacterMovement`))
      (`|AIMoveTo` self (0.0 0.0 0.0) _asbp_character
        (:`then`
          (`KismetSystemLibrary.RetriggerableDelay` 2.0)
          (`self.Set Patrol`))))))

(event `Set Patrol`
  ;[1 1 1] Set Patrol
  (set `CharacterMovementComponent.MaxWalkSpeed` (`self.Max Walk Speed`) (`self.CharacterMovement`))
  (`|AIMoveTo` self (`self.Point1`) null
    (:`OnSuccess`
      (`|AIMoveTo` self (`self.Point2`) null
        (:`OnSuccess`
          (`|AIMoveTo` self (`self.Point3`) null
            (:`OnSuccess`
              (`|AIMoveTo` self (`self.Point4`) null
                (:`OnSuccess`
                  (`|AIMoveTo` self (`self.Point5`) null
                    (:`OnSuccess`
                      (`|AIMoveTo` self (`self.Point6`) null
                        (:`OnSuccess`
                          (`self.Set Patrol`))))))))))))))

(event `self.ReceiveTick`
  (params (DeltaSeconds :type "Float (single-precision)"))
  (bind _eyesight (`self.eyesight`))
  (bind _eyesight2 (`self.eyesight2`))
  (bind _eyesight4 (`self.eyesight4`))
  (bind _eyesight3 (`self.eyesight3`))
  (bind _returnvalue (`SceneComponent.K2_GetComponentLocation` _eyesight4))
  (bind _returnvalue_2 (`SceneComponent.K2_GetComponentLocation` _eyesight2))
  (bind _returnvalue_3 (`SceneComponent.K2_GetComponentLocation` _eyesight))
  (bind _returnvalue_4 (`SceneComponent.K2_GetComponentLocation` _eyesight3))
  ;[1 1 1] Collision Tracing
  (bind _outactors (`GameplayStatics.GetAllActorsWithTag` "Enemy"))
  (bind (_outhit _returnvalue_5) (`KismetSystemLibrary.LineTraceSingleByProfile` _returnvalue_3 (+ _returnvalue_3 (* (`SceneComponent.GetForwardVector` _eyesight) 2000.0)) "Pawn" false _outactors "ForOneFrame"))
  (bind (_outhit_2 _returnvalue_6) (`KismetSystemLibrary.LineTraceSingleByProfile` _returnvalue_4 (+ _returnvalue_4 (* (`SceneComponent.GetForwardVector` _eyesight3) 2000.0)) "Pawn" false _outactors "ForOneFrame"))
  (bind (_outhit_3 _returnvalue_7) (`KismetSystemLibrary.LineTraceSingleByProfile` _returnvalue (+ _returnvalue (* (`SceneComponent.GetForwardVector` _eyesight4) 2000.0)) "Pawn" false _outactors "ForOneFrame"))
  (bind (_outhit_4 _returnvalue_8) (`KismetSystemLibrary.SphereTraceSingle` _returnvalue_2 (+ _returnvalue_2 (* (`SceneComponent.GetForwardVector` _eyesight2) 500.0)) 75.0 "TraceTypeQuery1" false _outactors "ForOneFrame"))
  (`|ExecutionSequence`
    (:`then_0`
      (if _returnvalue_5
        (if (`self.ActorHasTag` (`.HitActor` (`GameplayStatics.BreakHitResult` _outhit)) "Player")
          (`/Engine/EditorBlueprintResources/StandardMacros.DoOnce` false
            (:`Completed`
              (`KismetSystemLibrary.PrintText` "Hit")
              (bind _returnvalue_9 (`GameplayStatics.GetActorOfClass` "bp_EnemyPatrol3_C"))
              (`self.Player Chase` _returnvalue_9))))))
    (:`then_1`
      (if _returnvalue_6
        (if (`self.ActorHasTag` (`.HitActor` (`GameplayStatics.BreakHitResult` _outhit_2)) "Player")
          (bind _asbp_character (cast `/Game/PathOfLight/bp_Imports/bp_Character` (`GameplayStatics.GetPlayerPawn` 0)))
          (if (not (`Character.bIsCrouched` _asbp_character))
            (`/Engine/EditorBlueprintResources/StandardMacros.DoOnce` false
              (:`Completed`
                (`KismetSystemLibrary.PrintText` "Hit")
                (bind _returnvalue_10 (`GameplayStatics.GetActorOfClass` "bp_EnemyPatrol3_C"))
                (`self.Player Chase` _returnvalue_10)))))))
    (:`then_2`
      (if _returnvalue_7
        (if (`self.ActorHasTag` (`.HitActor` (`GameplayStatics.BreakHitResult` _outhit_3)) "Player")
          (bind _asbp_character_2 (cast `/Game/PathOfLight/bp_Imports/bp_Character` (`GameplayStatics.GetPlayerPawn` 0)))
          (if (not (`Character.bIsCrouched` _asbp_character_2))
            (`/Engine/EditorBlueprintResources/StandardMacros.DoOnce` false
              (:`Completed`
                (`KismetSystemLibrary.PrintText` "Hit")
                (bind _returnvalue_11 (`GameplayStatics.GetActorOfClass` "bp_EnemyPatrol3_C"))
                (`self.Player Chase` _returnvalue_11)))))))
    (:`then_3`
      (if _returnvalue_8
        (if (`self.ActorHasTag` (`.HitActor` (`GameplayStatics.BreakHitResult` _outhit_4)) "Player")
          (`/Engine/EditorBlueprintResources/StandardMacros.DoOnce` false
            (:`Completed`
              (`KismetSystemLibrary.PrintText` "Hit")
              (bind _returnvalue_12 (`GameplayStatics.GetActorOfClass` "bp_EnemyPatrol3_C"))
              (`self.Player Chase` _returnvalue_12))))))))

(event `self.PawnSensing.OnSeePawn`
  (params (Pawn :type "Pawn Object Reference"))
  ;[1 1 1] Pawn Sensing
  (bind _asbp_character (cast `/Game/PathOfLight/bp_Imports/bp_Character` (`GameplayStatics.GetPlayerPawn` 0)))
  (if (not (`Character.bIsCrouched` _asbp_character))
    (set `CharacterMovementComponent.MaxWalkSpeed` 400.0 (`self.CharacterMovement`))
    (`|AIMoveTo` self (0.0 0.0 0.0) Pawn
      (:`then`
        (`KismetSystemLibrary.RetriggerableDelay` 2.0)))))

(event `self.ReceiveHit`
  (params (MyComp :type "PrimitiveComponent Object Reference") (Other :type "Actor Object Reference") (OtherComp :type "PrimitiveComponent Object Reference") (bSelfMoved :type Boolean) (HitLocation :type "Vector Structure") (HitNormal :type "Vector Structure") (NormalImpulse :type "Vector Structure") (Hit :type "HitResult Structure (by ref)"))
  ;[1 1 1] stun interaction
  (bind _asbp_stun (cast `/Game/PathOfLight/Blueprints/bp_Stun` Other))
  (`self.K2_DestroyActor` _asbp_stun)
  (`CharacterMovementComponent.DisableMovement` (`self.CharacterMovement`))
  (`AIPerceptionComponent.SetSenseEnabled` (`self.AIPerception`) "/Script/AIModule.AISense_Hearing" false)
  (`KismetSystemLibrary.Delay` 4.0)
  (`CharacterMovementComponent.SetMovementMode` (`self.CharacterMovement`) "MOVE_Walking" 0)
  (`AIPerceptionComponent.SetSenseEnabled` (`self.AIPerception`) "/Script/AIModule.AISense_Hearing" true))

(event `self.AIPerception.OnTargetPerceptionUpdated`
  (params (Actor :type "Actor Object Reference") (Stimulus :type "AIStimulus Structure"))
  (bind (_age _expirationage _strength _stimuluslocation _receiverlocation _tag _bsuccessfullysensed) (break `AIStimulus` Stimulus))
  ;[1 1 1] AI Sound Interaction
  (cast `/Game/PathOfLight/bp_Imports/bp_Character` Actor)
  (if _bsuccessfullysensed
    (set `self.Investigating` true)
    (`|AIMoveTo` self _stimuluslocation null
      (:`OnSuccess`
        (`KismetSystemLibrary.Delay` 3.0)
        (`self.Set Patrol`)))))

(fn `UserConstructionScript`)