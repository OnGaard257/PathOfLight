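; Pickup object for PathOfLight that the player collects with the interact input while in range.
; Overlapping the interact collider with the player character shows a prompt widget, applies an outline overlay material to the mesh and opens a Gate, all reversed on exit.
; Interact input, enabled on BeginPlay, passes only through the open Gate to increment the character's ObjectAmount and destroy the actor.
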(event `self.ReceiveBeginPlay`
  (`self.EnableInput` (`GameplayStatics.GetPlayerController` 0)))

(event `EnhancedInput|/Game/PathOfLight/bp_Imports/ia_Interact`
  (params (ActionValue :type Boolean) (ElapsedSeconds :type "Float (double-precision)") (TriggeredSeconds :type "Float (double-precision)") (InputAction :type "InputAction Object Reference" :default "/Game/PathOfLight/bp_Imports/ia_Interact.ia_Interact"))
  ;[1 1 1] Pick Up Mechanic with UI Prompts
  (:`Triggered`
    (`/Engine/EditorBlueprintResources/StandardMacros.Gate` true :!label _label
      (:`Exit`
        (bind _result (`/Engine/EditorBlueprintResources/StandardMacros.IncrementInt` (`/Game/PathOfLight/bp_Imports/bp_Character.ObjectAmount` (stale `self.Interact Collider.OnComponentBeginOverlap` _asbp_character)))
          (:`  `
            (set `/Game/PathOfLight/bp_Imports/bp_Character.ObjectAmount` _result (stale `self.Interact Collider.OnComponentBeginOverlap` _asbp_character))
            (`self.K2_DestroyActor`)))))))

(event `self.Interact Collider.OnComponentBeginOverlap`
  (params (OverlappedComponent :type "PrimitiveComponent Object Reference") (OtherActor :type "Actor Object Reference") (OtherComp :type "PrimitiveComponent Object Reference") (OtherBodyIndex :type Integer) (bFromSweep :type Boolean) (SweepResult :type "HitResult Structure (by ref)"))
  ;[1 1 1] Pick Up Mechanic with UI Prompts
  (bind _asbp_character (cast `/Game/PathOfLight/bp_Imports/bp_Character` OtherActor))
  (`SceneComponent.SetVisibility` (`self.Widget`) true false)
  (`MeshComponent.SetOverlayMaterial` (`self.ObjectSM`) "/Game/PathOfLight/Materials/m_Outline_Inst.m_Outline_Inst")
  (goto _label :!via `Open`))

(event `self.Interact Collider.OnComponentEndOverlap`
  (params (OverlappedComponent :type "PrimitiveComponent Object Reference") (OtherActor :type "Actor Object Reference") (OtherComp :type "PrimitiveComponent Object Reference") (OtherBodyIndex :type Integer))
  ;[1 1 1] Pick Up Mechanic with UI Prompts
  (cast `/Game/PathOfLight/bp_Imports/bp_Character` OtherActor)
  (`SceneComponent.SetVisibility` (`self.Widget`) false false)
  (`MeshComponent.SetOverlayMaterial` (`self.ObjectSM`) null)
  (goto _label :!via `Close`))

(fn `UserConstructionScript`)