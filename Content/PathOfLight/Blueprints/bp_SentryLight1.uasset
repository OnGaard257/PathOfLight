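; Sentry light that detects the player in its beam and alerts the enemy crow.
; Each tick it line traces forward from its arrow, sphere traces at the impact point for bp_Character, and writes the hit location to the crow's blackboard.
; A DoOnce-gated alert plays the crow call, maxes detection on crows near the light and changes AI state, resetting after a delay.
; Back-and-forth rotation logic is disconnected.
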(event `Back and Forth`
  ;[1 1 1] Back and Forth
)

(event `self.ReceiveBeginPlay`
  (bind _returnvalue (`GameplayStatics.GetActorOfClass` "/Game/PathOfLight/LD_Prototyping/JavonW/Enemies/BP_EnemyCrow.BP_EnemyCrow_C"))
  (`|ExecutionSequence`
    (:`then_0`
      (set `self.BigCrowRef` _returnvalue))))

(event `self.ReceiveTick`
  (params (DeltaSeconds :type "Float (single-precision)"))
  (bind _arrow1 (`self.Arrow1`))
  (bind _returnvalue (`SceneComponent.K2_GetComponentLocation` _arrow1))
  ;[1 1 1] Collision Tracing
  (bind _outhit (`KismetSystemLibrary.LineTraceSingle` _returnvalue (+ _returnvalue (* (`SceneComponent.GetForwardVector` _arrow1) 4000.0)) "TraceTypeQuery1" false (`|MakeArray` (`self.BigCrowRef`) :!type "Actor Object Reference")))
  (bind (_bblockinghit _binitialoverlap _time _distance _location _impactpoint) (`GameplayStatics.BreakHitResult` _outhit))
  (bind _outhits (`KismetSystemLibrary.SphereTraceMultiByProfile` _location _impactpoint (`self.Sensing Radius`) "Pawn" false (`|MakeArray` (`self.BigCrowRef`) :!type "Actor Object Reference")))
  (for _array_element _outhits
    (bind (_bblockinghit_2 _binitialoverlap_2 _time_2 _distance_2 _location_2 _impactpoint_2 _normal _impactnormal _physmat _hitactor) (`GameplayStatics.BreakHitResult` _array_element))
    (`/Engine/EditorBlueprintResources/StandardMacros.IsValid` _hitactor
      (:`Is Valid`
        (cast `/Game/PathOfLight/bp_Imports/bp_Character` _hitactor)
        (`BlackboardComponent.SetValueAsVector` (`AIController.Blackboard` (`AIBlueprintHelperLibrary.GetAIController` (`self.BigCrowRef`))) (`self.Poi`) _location_2)
        (`/Engine/EditorBlueprintResources/StandardMacros.DoOnce` false :!label _label
          (:`Completed`
            (`GameplayStatics.PlaySound2D` "/Game/PathOfLight/Sounds/Crow_Call.Crow_Call" 1.0 1.0 0.2 null null)
            (bind (_outactors _returnvalue_2) (`KismetSystemLibrary.SphereOverlapActors` (`SceneComponent.K2_GetComponentLocation` (`self.Cylinder`)) 500.0 (`|MakeArray` "ObjectTypeQuery3" :!type "EObjectTypeQuery Enum") "/Game/PathOfLight/LD_Prototyping/JavonW/Enemies/BP_EnemyCrow.BP_EnemyCrow_C" (`|MakeArray` self :!type "Actor Object Reference")))
            (if _returnvalue_2
              (for _array_element_2 _outactors
                (bind _asbp_enemy_crow (cast `/Game/PathOfLight/LD_Prototyping/JavonW/Enemies/BP_EnemyCrow` _array_element_2))
                (`/Game/PathOfLight/LD_Prototyping/JavonW/Enemies/BP_EnemyCrow.DetectMax` _asbp_enemy_crow)
                (`BlackboardComponent.SetValueAsEnum` (`AIController.Blackboard` (`AIBlueprintHelperLibrary.GetAIController` (`self.BigCrowRef`))) (`self.Key`) (enumliteral `/Game/PathOfLight/LD_Prototyping/JavonW/Enemies/AI/Enums/E_AIStates` "NewEnumerator3"))
                (`KismetSystemLibrary.Delay` 1.3)
                (goto _label :!via `Reset`)))))))))

(fn `UserConstructionScript`)