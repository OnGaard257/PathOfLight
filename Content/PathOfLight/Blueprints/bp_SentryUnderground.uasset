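; Underground sentry that watches for the player and raises the alarm with the underground crow.
; Every Tick it casts two line traces and a capsule trace forward from three arrows, ignoring Enemy-tagged actors.
; A Player-tagged hit plays a crow call and calls SetDetection on Bp_UndergroundCrow, throttled per trace by a DoOnce reset after a short delay.
; The back-and-forth rotation logic is disconnected and never runs.
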(event `self.ReceiveBeginPlay`)

(event `Back and Forth`
  ;[1 1 1] Back and Forth
)

(event `self.ReceiveTick`
  (params (DeltaSeconds :type "Float (single-precision)"))
  (bind _arrow1 (`self.Arrow1`))
  (bind _arrow2 (`self.Arrow2`))
  (bind _arrow (`self.Arrow`))
  (bind _returnvalue (`SceneComponent.K2_GetComponentLocation` _arrow1))
  (bind _returnvalue_2 (`SceneComponent.K2_GetComponentLocation` _arrow))
  (bind _returnvalue_3 (`SceneComponent.K2_GetComponentLocation` _arrow2))
  ;[1 1 1] Collision Tracing
  (bind _outactors (`GameplayStatics.GetAllActorsWithTag` "Enemy"))
  (bind (_outhit _returnvalue_4) (`KismetSystemLibrary.LineTraceSingleByProfile` _returnvalue (+ _returnvalue (* (`SceneComponent.GetForwardVector` _arrow1) 3000.0)) "Pawn" false _outactors))
  (bind (_outhit_2 _returnvalue_5) (`KismetSystemLibrary.CapsuleTraceSingle` _returnvalue_2 (+ _returnvalue_2 (* (`SceneComponent.GetForwardVector` _arrow) 3000.0)) 60.0 120.0 "TraceTypeQuery1" false _outactors))
  (bind (_outhit_3 _returnvalue_6) (`KismetSystemLibrary.LineTraceSingleByProfile` _returnvalue_3 (+ _returnvalue_3 (* (`SceneComponent.GetForwardVector` _arrow2) 3000.0)) "Pawn" false _outactors))
  (`|ExecutionSequence`
    (:`then_0`
      (if _returnvalue_4
        (bind (_bblockinghit _binitialoverlap _time _distance _location _impactpoint _normal _impactnormal _physmat _hitactor) (`GameplayStatics.BreakHitResult` _outhit))
        (`/Engine/EditorBlueprintResources/StandardMacros.IsValid` _hitactor
          (:`Is Valid`
            (if (`self.ActorHasTag` _hitactor "Player")
              (`/Engine/EditorBlueprintResources/StandardMacros.DoOnce` false :!label _label
                (:`Completed`
                  (`GameplayStatics.PlaySound2D` "/Game/PathOfLight/Sounds/Crow_Call.Crow_Call" 1.0 1.0 0.2 null null)
                  (bind _returnvalue_7 (`GameplayStatics.GetActorOfClass` "/Game/PathOfLight/Blueprints/bp_UndergroundCrow.bp_UndergroundCrow_C"))
                  (`/Game/PathOfLight/Blueprints/bp_UndergroundCrow.SetDetection` _returnvalue_7)
                  (`KismetSystemLibrary.Delay` 1.3)
                  (goto _label :!via `Reset`))))))))
    (:`then_1`
      (if _returnvalue_5
        (if (`self.ActorHasTag` (`.HitActor` (`GameplayStatics.BreakHitResult` _outhit_2)) "Player")
          (`/Engine/EditorBlueprintResources/StandardMacros.DoOnce` false :!label _label_2
            (:`Completed`
              (`GameplayStatics.PlaySound2D` "/Game/PathOfLight/Sounds/Crow_Call.Crow_Call" 1.0 1.0 0.2 null null)
              (bind _returnvalue_8 (`GameplayStatics.GetActorOfClass` "/Game/PathOfLight/Blueprints/bp_UndergroundCrow.bp_UndergroundCrow_C"))
              (`/Game/PathOfLight/Blueprints/bp_UndergroundCrow.SetDetection` _returnvalue_8)
              (`KismetSystemLibrary.Delay` 1.3)
              (goto _label_2 :!via `Reset`))))))
    (:`then_2`
      (if _returnvalue_6
        (if (`self.ActorHasTag` (`.HitActor` (`GameplayStatics.BreakHitResult` _outhit_3)) "Player")
          (`/Engine/EditorBlueprintResources/StandardMacros.DoOnce` false :!label _label_3
            (:`Completed`
              (`GameplayStatics.PlaySound2D` "/Game/PathOfLight/Sounds/Crow_Call.Crow_Call" 1.0 1.0 0.2 null null)
              (bind _returnvalue_9 (`GameplayStatics.GetActorOfClass` "/Game/PathOfLight/Blueprints/bp_UndergroundCrow.bp_UndergroundCrow_C"))
              (`/Game/PathOfLight/Blueprints/bp_UndergroundCrow.SetDetection` _returnvalue_9)
              (`KismetSystemLibrary.Delay` 1.3)
              (goto _label_3 :!via `Reset`))))))))

(fn `UserConstructionScript`)