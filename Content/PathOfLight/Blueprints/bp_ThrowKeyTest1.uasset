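; Colored throwable key pickup that the player collects with the Interact input.
; Collider overlap toggles an outline and a gate that allows pickup.
; Pickup updates the character's held-item state, stops movement, maps the actor's color tag to throwable material and ColorIndex, then calls ReturnFromPickup.
; The key then destroys itself, first spawning an object pickup at the nearest Bp_ThrowKeyTest if the character has a DistractionObject.
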(event `self.ReceiveBeginPlay`
  (`self.EnableInput` (`GameplayStatics.GetPlayerController` 0)))

(event `EnhancedInput|/Game/PathOfLight/bp_Imports/ia_Interact`
  (params (ActionValue :type Boolean) (ElapsedSeconds :type "Float (double-precision)") (TriggeredSeconds :type "Float (double-precision)") (InputAction :type "InputAction Object Reference" :default "/Game/PathOfLight/bp_Imports/ia_Interact.ia_Interact"))
  ;[1 1 1] Pick Up Mechanic with UI Prompts
  (:`Triggered`
    (bind _asbp_character (cast `/Game/PathOfLight/bp_Imports/bp_Character` (`GameplayStatics.GetPlayerPawn` 0)))
    (if (`/Game/PathOfLight/bp_Imports/bp_Character.CanPickupAgain` _asbp_character)
      (if (`/Game/PathOfLight/bp_Imports/bp_Character.NoHeldItem` _asbp_character)
        (`/Engine/EditorBlueprintResources/StandardMacros.Gate` true :!label _label
          (:`Exit`
            (bind _result (`/Engine/EditorBlueprintResources/StandardMacros.IncrementInt` (`/Game/PathOfLight/bp_Imports/bp_Character.ObjectAmount` (stale `self.Interact Collider_0.OnComponentBeginOverlap` _asbp_character)))
              (:`  `
                (set `/Game/PathOfLight/bp_Imports/bp_Character.ObjectAmount` _result (stale `self.Interact Collider_0.OnComponentBeginOverlap` _asbp_character))
                (set `/Game/PathOfLight/bp_Imports/bp_Character.ThrowKey` true (stale `self.Interact Collider_0.OnComponentBeginOverlap` _asbp_character))
                (set `/Game/PathOfLight/bp_Imports/bp_Character.NoHeldItem` false (stale `self.Interact Collider_0.OnComponentBeginOverlap` _asbp_character))
                (set `/Game/PathOfLight/bp_Imports/bp_Character.CanThrow` true _asbp_character)
                (`CharacterMovementComponent.SetMovementMode` (`Character.CharacterMovement` _asbp_character) "MOVE_None" 0)
                (if (`self.ActorHasTag` "Red")
                  (bind _throwable (`/Game/PathOfLight/bp_Imports/bp_Character.Throwable` _asbp_character))
                  (`PrimitiveComponent.SetMaterial` _throwable 0 "/Game/PathOfLight/Materials/Material_Instances/MM_ThrowKeyRed.MM_ThrowKeyRed")
                  (set `/Game/PathOfLight/bp_Imports/bp_Character.ColorIndex` 1 _asbp_character)
                  (elif (`self.ActorHasTag` "Blue")
                    (`PrimitiveComponent.SetMaterial` _throwable 0 "/Game/PathOfLight/Materials/Material_Instances/MM_ThrowKeyBlue.MM_ThrowKeyBlue")
                    (set `/Game/PathOfLight/bp_Imports/bp_Character.ColorIndex` 2 _asbp_character)
                    (elif (`self.ActorHasTag` "Green")
                      (`PrimitiveComponent.SetMaterial` _throwable 0 "/Game/PathOfLight/Materials/Material_Instances/MM_ThrowKeyGreen.MM_ThrowKeyGreen")
                      (set `/Game/PathOfLight/bp_Imports/bp_Character.ColorIndex` 3 _asbp_character)
                      (elif (`self.ActorHasTag` "Yellow")
                        (`PrimitiveComponent.SetMaterial` _throwable 0 "/Game/PathOfLight/Materials/Material_Instances/MM_ThrowKeyYellow.MM_ThrowKeyYellow")
                        (set `/Game/PathOfLight/bp_Imports/bp_Character.ColorIndex` 4 _asbp_character)
                        (else
                          (`PrimitiveComponent.SetMaterial` _throwable 0 "/Game/PathOfLight/Materials/Material_Instances/MM_ThrowKeyPurple.MM_ThrowKeyPurple")
                          (set `/Game/PathOfLight/bp_Imports/bp_Character.ColorIndex` 0 _asbp_character))))))
                (`/Game/PathOfLight/bp_Imports/bp_Character.ReturnFromPickup` _asbp_character)
                (if (`/Game/PathOfLight/bp_Imports/bp_Character.DistractionObject` _asbp_character) :!label _label_2
                  (`/Engine/EditorBlueprintResources/StandardMacros.DoOnce` false :!label _label_3
                    (:`Completed`
                      (bind _outactors (`GameplayStatics.GetAllActorsOfClass` "/Game/PathOfLight/Blueprints/bp_ThrowKeyTest.bp_ThrowKeyTest_C"))
                      (bind _rootcomponent (`Actor.RootComponent` (`.ReturnValue` (`GameplayStatics.FindNearestActor` (`SceneComponent.K2_GetComponentLocation` (`Character.Mesh` _asbp_character)) _outactors))))
                      (`|SpawnActorFromClass` "/Game/PathOfLight/Blueprints/MichaelF_PT_BP/bp_Object_Pickup.bp_Object_Pickup_C" (`KismetMathLibrary.MakeTransform` (`SceneComponent.K2_GetComponentLocation` _rootcomponent) (`SceneComponent.K2_GetComponentRotation` _rootcomponent)) "Undefined" "MultiplyWithRoot" null null)
                      (`|ExecutionSequence`
                        (:`then_0`
                          _)
                        (:`then_1`
                          (set `/Game/PathOfLight/bp_Imports/bp_Character.DistractionObject` false _asbp_character)
                          (goto _label_3 :!via `Reset`))))))
                (`self.K2_DestroyActor`)))))
        (elif (not (`/Game/PathOfLight/bp_Imports/bp_Character.ThrowKey` _asbp_character))
          (goto _label))))))

(event `self.Interact Collider_0.OnComponentBeginOverlap`
  (params (OverlappedComponent :type "PrimitiveComponent Object Reference") (OtherActor :type "Actor Object Reference") (OtherComp :type "PrimitiveComponent Object Reference") (OtherBodyIndex :type Integer) (bFromSweep :type Boolean) (SweepResult :type "HitResult Structure (by ref)"))
  ;[1 1 1] Pick Up Mechanic with UI Prompts
  (bind _asbp_character (cast `/Game/PathOfLight/bp_Imports/bp_Character` OtherActor))
  (`MeshComponent.SetOverlayMaterial` (`self.ObjectSM_0`) "/Game/PathOfLight/Materials/m_Outline_Inst.m_Outline_Inst")
  (goto _label :!via `Open`))

(event `self.Interact Collider_0.OnComponentEndOverlap`
  (params (OverlappedComponent :type "PrimitiveComponent Object Reference") (OtherActor :type "Actor Object Reference") (OtherComp :type "PrimitiveComponent Object Reference") (OtherBodyIndex :type Integer))
  ;[1 1 1] Pick Up Mechanic with UI Prompts
  (cast `/Game/PathOfLight/bp_Imports/bp_Character` OtherActor)
  (`MeshComponent.SetOverlayMaterial` (`self.ObjectSM_0`) null)
  (goto _label :!via `Close`))

(event `DestroyCube`
  ;[1 1 1] Pick Up Mechanic with UI Prompts
  (goto _label_2))

(fn `UserConstructionScript`)