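; Pickup actor for the Lumi staff, which bobs on two alternating timelines with an attached ember effect.
; Box overlap with the player character toggles input and an outline overlay on the staff.
; Pressing interact in range triggers the character's interaction, then after a short delay sets HasStaff and reveals the character's staff and light.
; It also destroys itself, spawns a win volume at a hardcoded location and shows the flash-obtained widget.
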(event `PIckingUp`)

(event `self.Interaction`
  (`self.PIckingUp`))

(event `EnhancedInput|/Game/PathOfLight/bp_Imports/ia_Interact`
  (params (ActionValue :type Boolean) (ElapsedSeconds :type "Float (double-precision)") (TriggeredSeconds :type "Float (double-precision)") (InputAction :type "InputAction Object Reference" :default "/Game/PathOfLight/bp_Imports/ia_Interact.ia_Interact"))
  (:`Triggered`
    (if (`self.InRange?`)
      (bind _asbp_character (cast `/Game/PathOfLight/bp_Imports/bp_Character` (`GameplayStatics.GetPlayerCharacter` 0)))
      (`/Game/PathOfLight/bp_Imports/bp_Character.Interact` _asbp_character)
      (`KismetSystemLibrary.Delay` 0.4)
      (`|ExecutionSequence`
        (:`then_0`
          (set `/Game/PathOfLight/bp_Imports/bp_Character.HasStaff?` true _asbp_character)
          (`self.K2_DestroyActor`)
          (`|SpawnActorFromClass` "/Game/PathOfLight/Blueprints/bp_winvolume.bp_winvolume_C" (`KismetMathLibrary.MakeTransform` (5448.0 -3408.0 1636.0) (struct) (2.75 0.0 3.46875)) "Undefined" "MultiplyWithRoot" null null)
          (bind _returnvalue (`|CreateWidget` "/Game/PathOfLight/UI/Menu_Screens/wbp_FlashObtained.wbp_FlashObtained_C" (`GameplayStatics.GetPlayerController` 0)))
          (`UserWidget.AddToViewport` _returnvalue 0))
        (:`then_1`
          (`SceneComponent.SetVisibility` (`/Game/PathOfLight/bp_Imports/bp_Character.rig_LumiStaff` _asbp_character) true false)
          (`SceneComponent.SetVisibility` (`/Game/PathOfLight/bp_Imports/bp_Character.LumiLight` _asbp_character) true false))))))

(event `self.ReceiveBeginPlay`
  (bind _staff (`self.Staff`))
  (bind _returnvalue (`NiagaraFunctionLibrary.SpawnSystemAttached` "/Game/PathOfLight/VFX/Fire_and_smoke/VFX_Ember.VFX_Ember" (`self.Staff`) "None" (0.0 0.0 0.0) (struct) "KeepRelativeOffset"))
  (set `self.Fairy` _returnvalue)
  (bind (_direction _float_up) (`Timeline|Timeline` :!label _label)
    (:`Update`
      (`SceneComponent.K2_SetRelativeLocation` _staff _float_up false false))
    (:`Finished`
      (bind (_direction_2 _float_down) (`Timeline|Timeline_0` :!via `ReverseFromEnd`)
        (:`Update`
          (`SceneComponent.K2_SetRelativeLocation` _staff _float_down false false))
        (:`Finished`
          (goto _label :!via `PlayFromStart`))))))

(event `self.Box.OnComponentBeginOverlap`
  (params (OverlappedComponent :type "PrimitiveComponent Object Reference") (OtherActor :type "Actor Object Reference") (OtherComp :type "PrimitiveComponent Object Reference") (OtherBodyIndex :type Integer) (bFromSweep :type Boolean) (SweepResult :type "HitResult Structure (by ref)"))
  (cast `/Game/PathOfLight/bp_Imports/bp_Character` OtherActor)
  (set `self.InRange?` true)
  (`self.EnableInput` (`GameplayStatics.GetPlayerController` 0))
  (`MeshComponent.SetOverlayMaterial` (`self.Staff`) "/Game/PathOfLight/Materials/m_Outline_Inst.m_Outline_Inst"))

(event `self.Box.OnComponentEndOverlap`
  (params (OverlappedComponent :type "PrimitiveComponent Object Reference") (OtherActor :type "Actor Object Reference") (OtherComp :type "PrimitiveComponent Object Reference") (OtherBodyIndex :type Integer))
  (cast `/Game/PathOfLight/bp_Imports/bp_Character` OtherActor)
  (set `self.InRange?` false)
  (`self.DisableInput` (`GameplayStatics.GetPlayerController` 0))
  (`MeshComponent.SetOverlayMaterial` (`self.Staff`) null))

(fn `UserConstructionScript`)