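; Prototype enemy character that growls on spawn and chases the player once spotted.
; Each Tick, a long line trace and shorter sphere trace from eyesight components look for "Player"-tagged actors, each triggering PlayerChase once on the first bp_EnemyPatrol found, not necessarily itself.
; PlayerChase raises speed and re-issues AIMoveTo after a delay, supporting two player classes.
; A four-point patrol loop exists but nothing here starts it; random-patrol and pawn-sensing events are empty.
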(event `self.ReceiveBeginPlay`
  (`GameplayStatics.PlaySoundAtLocation` "/Game/PathOfLight/Sounds/Monster_Growl.Monster_Growl" (`self.K2_GetActorLocation` self) (struct) 1.0 1.0 0.0 null null null null))

(event `Random Patrol`
  ;[1 1 1] random patrol
)

(event `Enemy Patrol`
  ;[1 1 1] Set Patrol
  (set `CharacterMovementComponent.MaxWalkSpeed` 200.0 (`self.CharacterMovement`))
  (`|AIMoveTo` self (`self.Point1`) null
    (:`OnSuccess`
      (`|AIMoveTo` self (`self.Point2`) null
        (:`OnSuccess`
          (`|AIMoveTo` self (`self.Point3`) null
            (:`OnSuccess`
              (`|AIMoveTo` self (`self.Point4`) null
                (:`then`
                  (`self.Enemy Patrol`))))))))))

(event `self.PawnSensing.OnSeePawn`
  (params (Pawn :type "Pawn Object Reference"))
  ;[1 1 1] Pawn Sensing
)

(event `Player Chase`
  (bind _returnvalue (`GameplayStatics.GetPlayerPawn` 0))
  ;[1 1 1] Player Chase
  (`|ExecutionSequence`
    (:`then_0`
      (bind _asbp_character_camera (cast `/Game/PathOfLight/bp_Imports/bp_character_camera` _returnvalue))
      (set `CharacterMovementComponent.MaxWalkSpeed` 400.0 (`self.CharacterMovement`))
      (`|AIMoveTo` self (0.0 0.0 0.0) _asbp_character_camera
        (:`then`
          (`KismetSystemLibrary.RetriggerableDelay` 2.0)
          (`self.Player Chase`))))
    (:`then_1`
      (bind _asbp_character (cast `/Game/PathOfLight/bp_Imports/bp_Character` _returnvalue))
      (set `CharacterMovementComponent.MaxWalkSpeed` 400.0 (`self.CharacterMovement`))
      (`|AIMoveTo` self (0.0 0.0 0.0) _asbp_character
        (:`then`
          (`KismetSystemLibrary.RetriggerableDelay` 2.0)
          (`self.Player Chase`))))))

(event `self.ReceiveTick`
  (params (DeltaSeconds :type "Float (single-precision)"))
  (bind _eyesight2 (`self.eyesight2`))
  (bind _eyesight (`self.eyesight`))
  (bind _returnvalue (`SceneComponent.K2_GetComponentLocation` _eyesight))
  (bind _returnvalue_2 (`SceneComponent.K2_GetComponentLocation` _eyesight2))
  ;[1 1 1] Collision Tracing
  (bind _outactors (`GameplayStatics.GetAllActorsWithTag` "Enemy"))
  (bind (_outhit _returnvalue_3) (`KismetSystemLibrary.LineTraceSingleByProfile` _returnvalue (+ _returnvalue (* (`SceneComponent.GetForwardVector` _eyesight) 2000.0)) "Pawn" false _outactors "ForOneFrame"))
  (bind (_outhit_2 _returnvalue_4) (`KismetSystemLibrary.SphereTraceSingle` :`Start` _returnvalue_2 :`End` (+ _returnvalue_2 (* (`SceneComponent.GetForwardVector` _eyesight2) 700.0)) :`Radius` 75.0 :`TraceChannel` "TraceTypeQuery1" :`DrawDebugType` "ForOneFrame"))
  (`|ExecutionSequence`
    (:`then_0`
      (if _returnvalue_3
        (if (`self.ActorHasTag` (`.HitActor` (`GameplayStatics.BreakHitResult` _outhit)) "Player")
          (`/Engine/EditorBlueprintResources/StandardMacros.DoOnce` false
            (:`Completed`
              (`KismetSystemLibrary.PrintText` "Hit")
              (bind _returnvalue_5 (`GameplayStatics.GetActorOfClass` "bp_EnemyPatrol_C"))
              (`self.Player Chase` _returnvalue_5))))))
    (:`then_1`
      (if _returnvalue_4
        (if (`self.ActorHasTag` (`.HitActor` (`GameplayStatics.BreakHitResult` _outhit_2)) "Player")
          (`/Engine/EditorBlueprintResources/StandardMacros.DoOnce` false
            (:`Completed`
              (`KismetSystemLibrary.PrintText` "Hit")
              (bind _returnvalue_6 (`GameplayStatics.GetActorOfClass` "bp_EnemyPatrol_C"))
              (`self.Player Chase` _returnvalue_6))))))))

(fn `UserConstructionScript`)