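; Prototype rock pickup that the player collects and that, once thrown, distracts blind enemies.
; Sphere overlap outlines the rock and opens a gate for PickUpRock, which updates character state and UI, then destroys the actor.
; A held throw key is swapped out by spawning its colour variant at the nearest pickup.
; On a thrown impact, it plays sound, reports noise and sends nearby BP_BlindEnemy actors to the nearest pickup's location.
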(event `OnDestroyed Rock` :!signature `self.OnDestroyed`
  (params (DestroyedActor :type "Actor Object Reference"))
  (`SceneComponent.SetVisibility` (`/Game/PathOfLight/bp_Imports/bp_Character.Rock` (stale `PickUpRock` _asbp_character)) true false)
  (`/Game/PathOfLight/bp_Imports/HUD_UI.RockPickup` (`/Game/PathOfLight/bp_Imports/bp_Character.CooldownUIRef` (stale `PickUpRock` _asbp_character))))

(event `self.ReceiveBeginPlay`
  (`self.EnableInput` (`GameplayStatics.GetPlayerController` 0))
  (add `self.OnDestroyed` (delegate `OnDestroyed Rock`)))

(event `PickUpRock`
  ;[1 1 1] Pick Up Mechanic with UI Prompts
  (bind _asbp_character (cast `/Game/PathOfLight/bp_Imports/bp_Character` (`GameplayStatics.GetPlayerCharacter` 0)))
  (if (`/Game/PathOfLight/bp_Imports/bp_Character.CanPickupAgain` _asbp_character)
    (if (`/Game/PathOfLight/bp_Imports/bp_Character.NoHeldItem` _asbp_character)
      (`/Engine/EditorBlueprintResources/StandardMacros.Gate` true :!label _label
        (:`Exit`
          (`Character.PlayAnimMontage` _asbp_character "/Game/PathOfLight/Animations/anim_LumiInteract_Montage.anim_LumiInteract_Montage" 2.0 "None")
          (`KismetSystemLibrary.Delay` 0.2)
          (`GameplayStatics.PlaySound2D` "/Game/PathOfLight/Sounds/ColeSFX/Rock_Pickup.Rock_Pickup" 0.05 0.8 0.2 null null)
          (`SceneComponent.SetVisibility` (`/Game/PathOfLight/bp_Imports/bp_Character.Rock` (stale `self.Sphere.OnComponentBeginOverlap` _asbp_character)) true false)
          (`/Game/PathOfLight/bp_Imports/HUD_UI.RockPickup` (`/Game/PathOfLight/bp_Imports/bp_Character.CooldownUIRef` _asbp_character))
          (bind _result (`/Engine/EditorBlueprintResources/StandardMacros.IncrementInt` (`/Game/PathOfLight/bp_Imports/bp_Character.ObjectAmount` (stale `self.Sphere.OnComponentBeginOverlap` _asbp_character)))
            (:`  `
              (set `/Game/PathOfLight/bp_Imports/bp_Character.ObjectAmount` _result (stale `self.Sphere.OnComponentBeginOverlap` _asbp_character))
              (set `/Game/PathOfLight/bp_Imports/bp_Character.DistractionObject` true (stale `self.Sphere.OnComponentBeginOverlap` _asbp_character))
              (set `/Game/PathOfLight/bp_Imports/bp_Character.NoHeldItem` false (stale `self.Sphere.OnComponentBeginOverlap` _asbp_character))
              (set `/Game/PathOfLight/bp_Imports/bp_Character.CanThrow` true (stale `self.Sphere.OnComponentBeginOverlap` _asbp_character))
              (if (`SceneComponent.IsVisible` (`/Game/PathOfLight/bp_Imports/bp_Character.Throwable` _asbp_character))
                (set `PrimitiveComponent.bGenerateOverlapEvents` false (`self.Sphere`))
                ;[1 1 1] Throw Key Color
                (`KismetSystemLibrary.Delay` 0.1)
                (bind _outactors (`GameplayStatics.GetAllActorsOfClass` "bp_Object_PickupTest_C"))
                (bind _colorindex (`/Game/PathOfLight/bp_Imports/bp_Character.ColorIndex` _asbp_character))
                (if (== _colorindex 0)
                  (bind _rootcomponent (`Actor.RootComponent` (`.ReturnValue` (`GameplayStatics.FindNearestActor` (`SceneComponent.K2_GetComponentLocation` (`Character.Mesh` _asbp_character)) _outactors))))
                  (bind (_returnvalue_x _returnvalue_y _returnvalue_z) (`KismetMathLibrary.BreakVector` (`SceneComponent.K2_GetComponentLocation` _rootcomponent)))
                  (bind _returnvalue (+ _returnvalue_z 10.0))
                  (bind _returnvalue_2 (`SceneComponent.K2_GetComponentRotation` _rootcomponent))
                  (`|SpawnActorFromClass` "/Game/PathOfLight/Blueprints/bp_ThrowKeyTest.bp_ThrowKeyTest_C" (`KismetMathLibrary.MakeTransform` (`KismetMathLibrary.MakeVector` _returnvalue_x _returnvalue_y _returnvalue) _returnvalue_2) "AlwaysSpawn" "MultiplyWithRoot" null null)
                  (`|ExecutionSequence` :!label _label_2
                    (:`then_0`
                      (`SceneComponent.SetVisibility` (`/Game/PathOfLight/bp_Imports/bp_Character.Throwable` _asbp_character) false false)
                      (set `/Game/PathOfLight/bp_Imports/bp_Character.ThrowKey` false (stale `self.Sphere.OnComponentBeginOverlap` _asbp_character))
                      (`KismetSystemLibrary.Delay` 0.01)
                      (`self.K2_DestroyActor` :!label _label_3))
                    (:`then_1`
                      (`/Game/PathOfLight/bp_Imports/HUD_UI.ThrowKeyHide` (`/Game/PathOfLight/bp_Imports/bp_Character.CooldownUIRef` _asbp_character))))
                  (elif (== _colorindex 1)
                    (`|SpawnActorFromClass` "/Game/PathOfLight/Blueprints/bp_ThrowKeyTest_Red.bp_ThrowKeyTest_Red_C" (`KismetMathLibrary.MakeTransform` (`KismetMathLibrary.MakeVector` _returnvalue_x _returnvalue_y _returnvalue) _returnvalue_2) "AlwaysSpawn" "MultiplyWithRoot" null null)
                    (goto _label_2)
                    (elif (== _colorindex 2)
                      (`|SpawnActorFromClass` "/Game/PathOfLight/Blueprints/bp_ThrowKeyTest_Blue.bp_ThrowKeyTest_Blue_C" (`KismetMathLibrary.MakeTransform` (`KismetMathLibrary.MakeVector` _returnvalue_x _returnvalue_y _returnvalue) _returnvalue_2) "AlwaysSpawn" "MultiplyWithRoot" null null)
                      (goto _label_2)
                      (elif (== _colorindex 3)
                        (`|SpawnActorFromClass` "/Game/PathOfLight/Blueprints/bp_ThrowKeyTest_Green.bp_ThrowKeyTest_Green_C" (`KismetMathLibrary.MakeTransform` (`KismetMathLibrary.MakeVector` _returnvalue_x _returnvalue_y _returnvalue) _returnvalue_2) "AlwaysSpawn" "MultiplyWithRoot" null null)
                        (goto _label_2)
                        (elif (== _colorindex 4)
                          (`|SpawnActorFromClass` "/Game/PathOfLight/Blueprints/bp_ThrowKeyTest_Yellow.bp_ThrowKeyTest_Yellow_C" (`KismetMathLibrary.MakeTransform` (`KismetMathLibrary.MakeVector` _returnvalue_x _returnvalue_y _returnvalue) _returnvalue_2) "AlwaysSpawn" "MultiplyWithRoot" null null)
                          (goto _label_2)
                          (elif (== _colorindex 5)
                            (`|SpawnActorFromClass` "/Game/PathOfLight/Blueprints/bp_ThrowKeyPurple2.bp_ThrowKeyPurple2_C" (`KismetMathLibrary.MakeTransform` (`KismetMathLibrary.MakeVector` _returnvalue_x _returnvalue_y _returnvalue) _returnvalue_2) "AlwaysSpawn" "MultiplyWithRoot" null null)
                            (goto _label_2)))))))
                (else
                  (goto _label_3)))))))
      (elif (not (`SceneComponent.IsVisible` (`/Game/PathOfLight/bp_Imports/bp_Character.Rock` _asbp_character)))
        (goto _label)))))

(event `self.Sphere.OnComponentBeginOverlap`
  (params (OverlappedComponent :type "PrimitiveComponent Object Reference") (OtherActor :type "Actor Object Reference") (OtherComp :type "PrimitiveComponent Object Reference") (OtherBodyIndex :type Integer) (bFromSweep :type Boolean) (SweepResult :type "HitResult Structure (by ref)"))
  ;[1 1 1] Pick Up Mechanic with UI Prompts
  (bind _asbp_character (cast `/Game/PathOfLight/bp_Imports/bp_Character` OtherActor))
  (set `/Game/PathOfLight/bp_Imports/bp_Character.RockOverlap?` true _asbp_character)
  (`MeshComponent.SetOverlayMaterial` (`self.ObjectSM`) "/Game/PathOfLight/Materials/m_Outline_Inst.m_Outline_Inst")
  (goto _label :!via `Open`))

(event `self.Sphere.OnComponentEndOverlap`
  (params (OverlappedComponent :type "PrimitiveComponent Object Reference") (OtherActor :type "Actor Object Reference") (OtherComp :type "PrimitiveComponent Object Reference") (OtherBodyIndex :type Integer))
  ;[1 1 1] Pick Up Mechanic with UI Prompts
  (bind _asbp_character (cast `/Game/PathOfLight/bp_Imports/bp_Character` OtherActor))
  (set `/Game/PathOfLight/bp_Imports/bp_Character.RockOverlap?` false _asbp_character)
  (`MeshComponent.SetOverlayMaterial` (`self.ObjectSM`) null)
  (goto _label :!via `Close`))

(event `self.ReceiveHit`
  (params (MyComp :type "PrimitiveComponent Object Reference") (Other :type "Actor Object Reference") (OtherComp :type "PrimitiveComponent Object Reference") (bSelfMoved :type Boolean) (HitLocation :type "Vector Structure") (HitNormal :type "Vector Structure") (NormalImpulse :type "Vector Structure") (Hit :type "HitResult Structure (by ref)"))
  (bind _returnvalue (`GameplayStatics.GetPlayerCharacter` 0))
  ;[1 1 1] Sound Spawn Collision
  (bind _asbp_character (cast `/Game/PathOfLight/bp_Imports/bp_Character` _returnvalue))
  (if (`/Game/PathOfLight/bp_Imports/bp_Character.Thrown` _asbp_character)
    (if (`self.Thrown?`)
      (bind _outactors (`GameplayStatics.GetAllActorsOfClass` "bp_Object_PickupTest_C"))
      (set `self.Thrown?` false)
      (set `/Game/PathOfLight/bp_Imports/bp_Character.Thrown` false _asbp_character)
      (`/Engine/EditorBlueprintResources/StandardMacros.DoOnce` false :!label _label_4
        (:`Completed`
          (bind _returnvalue_2 (`self.K2_GetActorLocation` (`.ReturnValue` (`GameplayStatics.FindNearestActor` HitLocation _outactors))))
          (`GameplayStatics.PlaySoundAtLocation` "/Game/PathOfLight/Sounds/ThrowSFX/Rock_Hit_Ground.Rock_Hit_Ground" _returnvalue_2 (struct) 1.0 1.0 0.4 "/Game/PathOfLight/Sounds/FootstepSoundAttenuation.FootstepSoundAttenuation" null null null)
          (`AISense_Hearing.ReportNoiseEvent` _returnvalue_2 1.0 _returnvalue 300.0)
          (bind _outactors_2 (`KismetSystemLibrary.SphereOverlapActors` HitLocation 1500.0 (`|MakeArray` "ObjectTypeQuery3" :!type "EObjectTypeQuery Enum") "/Game/PathOfLight/LD_Prototyping/JavonW/Enemies/BP_BlindEnemy.BP_BlindEnemy_C" (`|MakeArray` _asbp_character :!type "Actor Object Reference")))
          (bind (_arrayindex _arrayelement) (`/Engine/EditorBlueprintResources/StandardMacros.ReverseForEachLoop` _outactors_2)
            (:`LoopBody`
              (bind _asbp_blind_enemy (cast `/Game/PathOfLight/LD_Prototyping/JavonW/Enemies/BP_BlindEnemy` _arrayelement))
              (`|ExecutionSequence`
                (:`then_0`
                  (set `/Game/PathOfLight/LD_Prototyping/JavonW/Enemies/BP_BlindEnemy.DistractionLocation` _returnvalue_2 _asbp_blind_enemy)
                  (`/Game/PathOfLight/LD_Prototyping/JavonW/Enemies/BP_BlindEnemy.GetDistracted` _asbp_blind_enemy)
                  (goto _label_4 :!via `Reset`))
                (:`then_1`
                  (bind _outactors_3 (`GameplayStatics.GetAllActorsOfClassWithTag` "/Game/PathOfLight/LD_Prototyping/JavonW/Enemies/BP_BlindEnemy.BP_BlindEnemy_C" "Enemy"))
                  (bind (_distance _returnvalue_3) (`GameplayStatics.FindNearestActor` _returnvalue_2 _outactors_3))
                  (if (not (>= _distance 1500.0))
                    (bind _asbp_blind_enemy_2 (cast `/Game/PathOfLight/LD_Prototyping/JavonW/Enemies/BP_BlindEnemy` _returnvalue_3))
                    (set `/Game/PathOfLight/LD_Prototyping/JavonW/Enemies/BP_BlindEnemy.DistractionLocation` _returnvalue_2 _asbp_blind_enemy_2)
                    (`/Game/PathOfLight/LD_Prototyping/JavonW/Enemies/BP_BlindEnemy.GetDistracted` _asbp_blind_enemy_2)
                    (goto _label_4 :!via `Reset`)))))))))))

(fn `UserConstructionScript`)