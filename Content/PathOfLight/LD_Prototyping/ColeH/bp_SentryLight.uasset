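; Prototype sentry light that sweeps back and forth and flags anything that overlaps its Cone component.
; After an initial delay on BeginPlay, a self-calling BackAndForth event flips the RotatingMovement rate between opposite directions at equal timed intervals, looping indefinitely.
; The cone overlap only prints an "ALERT" string, with no filtering of the overlapping actor or further response.
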(event `self.ReceiveBeginPlay`
  (`KismetSystemLibrary.Delay` 1.9)
  (`self.Back and Forth`))

(event `Back and Forth`
  (set `RotatingMovementComponent.RotationRate` (struct :`Roll` 30.0) (`self.RotatingMovement`))
  (`KismetSystemLibrary.Delay` 3.8)
  (set `RotatingMovementComponent.RotationRate` (struct :`Roll` -30.0) (`self.RotatingMovement`))
  (`KismetSystemLibrary.Delay` 3.8)
  (`self.Back and Forth`))

(event `self.Cone.OnComponentBeginOverlap`
  (params (OverlappedComponent :type "PrimitiveComponent Object Reference") (OtherActor :type "Actor Object Reference") (OtherComp :type "PrimitiveComponent Object Reference") (OtherBodyIndex :type Integer) (bFromSweep :type Boolean) (SweepResult :type "HitResult Structure (by ref)"))
  (`KismetSystemLibrary.PrintString` "ALERT"))

(fn `UserConstructionScript`)