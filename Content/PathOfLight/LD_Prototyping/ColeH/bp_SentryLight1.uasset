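; Prototype sentry light that sweeps back and forth and alerts an enemy patrol when it spots the player.
; A self-calling delayed event flips RotatingMovement's yaw rate to create the sweep.
; Each Tick runs a debug-drawn line trace, ignoring Enemy-tagged actors, and a sphere trace along the Arrow.
; Each trace's own DoOnce calls PlayerChase on a single Bp_EnemyPatrol found by class, with no reset.
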(event `self.ReceiveBeginPlay`
  (`KismetSystemLibrary.Delay` 1.0)
  (`self.Back and Forth`))

(event `Back and Forth`
  ;[1 1 1] Back and Forth
  (set `RotatingMovementComponent.RotationRate` (struct :`Pitch` 30.0) (`self.RotatingMovement`))
  (`KismetSystemLibrary.Delay` 2.0)
  (set `RotatingMovementComponent.RotationRate` (struct :`Pitch` -30.0) (`self.RotatingMovement`))
  (`KismetSystemLibrary.Delay` 2.0)
  (`self.Back and Forth`))

(event `self.ReceiveTick`
  (params (DeltaSeconds :type "Float (single-precision)"))
  (bind _arrow (`self.Arrow`))
  (bind _returnvalue (`SceneComponent.K2_GetComponentLocation` _arrow))
  (bind _returnvalue_2 (+ _returnvalue (* (`SceneComponent.GetForwardVector` _arrow) 2000.0)))
  (bind _outactors (`GameplayStatics.GetAllActorsWithTag` "Enemy"))
  (bind (_outhit _returnvalue_3) (`KismetSystemLibrary.LineTraceSingleByProfile` _returnvalue _returnvalue_2 "Pawn" false _outactors "ForOneFrame"))
  (bind (_outhit_2 _returnvalue_4) (`KismetSystemLibrary.SphereTraceSingle` :`Start` _returnvalue :`End` _returnvalue_2 :`Radius` 50.0 :`TraceChannel` "TraceTypeQuery1" :`DrawDebugType` "ForOneFrame"))
  (`|ExecutionSequence`
    (:`then_0`
      (if _returnvalue_3
        (if (`self.ActorHasTag` (`.HitActor` (`GameplayStatics.BreakHitResult` _outhit)) "Player")
          (`/Engine/EditorBlueprintResources/StandardMacros.DoOnce` false
            (:`Completed`
              (`KismetSystemLibrary.PrintText` "Hit")
              (bind _returnvalue_5 (`GameplayStatics.GetActorOfClass` "/Game/PathOfLight/LD_Prototyping/ColeH/bp_EnemyPatrol.bp_EnemyPatrol_C"))
              (`/Game/PathOfLight/LD_Prototyping/ColeH/bp_EnemyPatrol.Player Chase` _returnvalue_5))))))
    (:`then_1`
      (if _returnvalue_4
        (if (`self.ActorHasTag` (`.HitActor` (`GameplayStatics.BreakHitResult` _outhit_2)) "Player")
          (`/Engine/EditorBlueprintResources/StandardMacros.DoOnce` false
            (:`Completed`
              (`KismetSystemLibrary.PrintText` "Hit")
              (bind _returnvalue_6 (`GameplayStatics.GetActorOfClass` "/Game/PathOfLight/LD_Prototyping/ColeH/bp_EnemyPatrol.bp_EnemyPatrol_C"))
              (`/Game/PathOfLight/LD_Prototyping/ColeH/bp_EnemyPatrol.Player Chase` _returnvalue_6))))))))

(fn `UserConstructionScript`)