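; Parent interactable Blueprint that offers shared overlap and input logic for objects the player character can interact with.
; BeginOverlap and EndOverlap events track InRange and, for bp_Character, enable or disable input from player controller 0.
; Both events set the passed prompt's root visible and call SetOverlayMaterial with no material, so only the input toggle differs visually unseen.
; The ia_Interact input calls Interaction, gated by a half-second cooldown against repeated presses.
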(event `EnhancedInput|/Game/PathOfLight/bp_Imports/ia_Interact`
  (params (ActionValue :type Boolean) (ElapsedSeconds :type "Float (double-precision)") (TriggeredSeconds :type "Float (double-precision)") (InputAction :type "InputAction Object Reference" :default "/Game/PathOfLight/bp_Imports/ia_Interact.ia_Interact"))
  (:`Triggered`
    (if (not (`self.cooldown active`))
      (`|ExecutionSequence`
        (:`then_0`
          (set `self.cooldown active` true)
          (`KismetSystemLibrary.Delay` 0.5)
          (set `self.cooldown active` false))
        (:`then_1`
          (`/Game/PathOfLight/LD_Prototyping/JavonW/BPI_Interface.Interaction`))))))

(event `Begin Overlap`
  (params (`Actor Overlapping` :type "Actor Object Reference") (Interaction :type "Actor Object Reference") (`Something Mesh` :type "MeshComponent Object Reference"))
  (set `self.In Range` true)
  (cast `/Game/PathOfLight/bp_Imports/bp_Character` `Actor Overlapping`)
  (`SceneComponent.SetVisibility` (`Actor.RootComponent` Interaction) true false)
  (`MeshComponent.SetOverlayMaterial` `Something Mesh` null)
  (`self.EnableInput` (`GameplayStatics.GetPlayerController` 0)))

(event `End Overlap`
  (params (`Actor Overlapping` :type "Actor Object Reference") (Interaction :type "Actor Object Reference") (`Something Mesh` :type "MeshComponent Object Reference"))
  (set `self.In Range` false)
  (cast `/Game/PathOfLight/bp_Imports/bp_Character` `Actor Overlapping`)
  (`SceneComponent.SetVisibility` (`Actor.RootComponent` Interaction) true false)
  (`MeshComponent.SetOverlayMaterial` `Something Mesh` null)
  (`self.DisableInput` (`GameplayStatics.GetPlayerController` 0)))

(fn `UserConstructionScript`)