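; Parent enemy Blueprint that handles stealth detection and a lethal melee trace against the player character.
; Hearing and sight events raise a clamped-on-decay detection score unless the player is crouched (hearing also ignores dashing), while a looping timer lowers it.
; At the threshold, it switches the AI Blackboard state, with hearing also setting a point of interest.
; A socket-to-socket sphere trace destroys any character hit, and detection is passed to the player for comparison.
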(event `ParentAttackTrace`
  (params (Mesh :type "SkeletalMeshComponent Object Reference") (traceStart :type Name) (traceStop :type Name))
  (bind _outhit (`KismetSystemLibrary.SphereTraceSingle` (`SceneComponent.GetSocketLocation` Mesh traceStart) (`SceneComponent.GetSocketLocation` Mesh traceStop) 75.0 "TraceTypeQuery1" false (`self.GetAllChildActors` true)))
  (bind _output_get (set `self.Hit Actor` (`.HitActor` (`GameplayStatics.BreakHitResult` _outhit))))
  (bind _asbp_character (cast `/Game/PathOfLight/bp_Imports/bp_Character` _output_get))
  (`/Engine/EditorBlueprintResources/StandardMacros.IsValid` _asbp_character
    (:`Is Valid`
      (`self.K2_DestroyActor` _output_get))))

(event `Parent Check Char`
  (`/Game/PathOfLight/bp_Imports/bp_Character.CompareNoiseInts` (`self.As Bp Character`) (`self.DEtection`)))

(event `self.ReceiveBeginPlay`
  (bind _asbp_character (cast `/Game/PathOfLight/bp_Imports/bp_Character` (`GameplayStatics.GetPlayerCharacter` 0)))
  (set `self.As Bp Character` _asbp_character))

(event `TraceStart`
  (set `self.attackTrace` true))

(event `TraceStop`
  (set `self.attackTrace` false))

(event `TickDownDetection`
  (bind _asbp_character (cast `/Game/PathOfLight/bp_Imports/bp_Character` (`GameplayStatics.GetPlayerCharacter` 0)))
  (set `self.As Bp Character` _asbp_character)
  (`KismetSystemLibrary.K2_SetTimerDelegate` (delegate `TickDown`) 1.0 true))

(event `TickDown`
  (set `self.DEtection` (`KismetMathLibrary.Clamp` (- (`self.DEtection`) 1) 0 12)))

(event `HearNoise`
  (params (HeardVector :type "Vector Structure") (Character :type "Pawn Object Reference"))
  ;[1 1 1] Enemy hearing detection - Increments
  (bind _asbp_character (cast `/Game/PathOfLight/bp_Imports/bp_Character` Character)
    (:`then`
      (if (`Character.bIsCrouched` _asbp_character)
        _
        (elif (not (`/Game/PathOfLight/bp_Imports/bp_Character.Dashing` _asbp_character))
          (set `self.DEtection` (+ (`self.DEtection`) 2))
          (`KismetSystemLibrary.Delay` 1.0)
          (if (>= (`self.DEtection`) 10)
            (`BlackboardComponent.SetValueAsEnum` (`AIController.Blackboard` (`AIBlueprintHelperLibrary.GetAIController` self)) (`self.Key`) (enumliteral `/Game/PathOfLight/LD_Prototyping/JavonW/Enemies/AI/Enums/E_AIStates` "NewEnumerator3"))
            (`BlackboardComponent.SetValueAsVector` (`AIController.Blackboard` (`AIBlueprintHelperLibrary.GetAIController` self)) (`self.POI`) HeardVector)
            (else
              (`BlackboardComponent.SetValueAsEnum` (`AIController.Blackboard` (`AIBlueprintHelperLibrary.GetAIController` self)) (`self.Key`) (enumliteral `/Game/PathOfLight/LD_Prototyping/JavonW/Enemies/AI/Enums/E_AIStates` "NewEnumerator0")))))))
    (:`CastFailed`
      (`BlackboardComponent.SetValueAsEnum` (`AIController.Blackboard` (`AIBlueprintHelperLibrary.GetAIController` self)) (`self.Key`) (enumliteral `/Game/PathOfLight/LD_Prototyping/JavonW/Enemies/AI/Enums/E_AIStates` "NewEnumerator0")))))

(event `See Nosie`
  (params (Character :type "Pawn Object Reference") (CanSee :type Boolean))
  (bind _blackboard (`AIController.Blackboard` (`AIBlueprintHelperLibrary.GetAIController` self)))
  ;[1 1 1] Enemy Sight
  (bind _asbp_character (cast `/Game/PathOfLight/bp_Imports/bp_Character` Character)
    (:`then`
      (set `self.CanSee` true)
      (if (not (`Character.bIsCrouched` _asbp_character))
        (set `self.DEtection` (+ (`self.DEtection`) 5))
        (`KismetSystemLibrary.Delay` 1.0)
        (if (>= (`self.DEtection`) 10)
          (`BlackboardComponent.SetValueAsEnum` _blackboard (`self.Key`) (enumliteral `/Game/PathOfLight/LD_Prototyping/JavonW/Enemies/AI/Enums/E_AIStates` "NewEnumerator3")))))
    (:`CastFailed`
      (set `self.CanSee` false)
      (`BlackboardComponent.SetValueAsEnum` _blackboard (`self.Key`) (enumliteral `/Game/PathOfLight/LD_Prototyping/JavonW/Enemies/AI/Enums/E_AIStates` "NewEnumerator0")))))

(fn `UserConstructionScript`)