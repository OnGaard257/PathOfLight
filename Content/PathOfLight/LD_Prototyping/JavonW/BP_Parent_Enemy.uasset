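; Parent enemy Blueprint providing stealth detection and one-hit melee kills against the player.
; Hearing and sight events raise a shared detection meter, weighing crouching and dashing, while a looping timer drains it.
; Meter thresholds switch the Blackboard AI state, with hearing also setting a point of interest, and the value is reported to the player character.
; Socket-to-socket capsule traces destroy a non-invincible player and reset detection; TouchDeath plays a montage while focusing the player.
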(event `TouchDeath`
  (params (AnimMontage :type "AnimMontage Object Reference") (Character :type "Character Object Reference"))
  (bind _returnvalue (`AIBlueprintHelperLibrary.GetAIController` self))
  (bind _asbp_character (cast `/Game/PathOfLight/bp_Imports/bp_Character` (`GameplayStatics.GetPlayerCharacter` 0)))
  (`AIController.K2_SetFocus` _returnvalue _asbp_character)
  (bind _returnvalue_2 (`self.PlayAnimMontage` Character AnimMontage 1.0 "None"))
  (`KismetSystemLibrary.Delay` _returnvalue_2)
  (`AIController.K2_ClearFocus` _returnvalue))

(event `ParentAttackTrace`
  (params (Mesh :type "SkeletalMeshComponent Object Reference") (traceStart :type Name) (traceStop :type Name) (traceSize :type "Float (double-precision)" :default 75.0))
  ;[1 1 1] Attack Trace
  (bind _outhits (`KismetSystemLibrary.CapsuleTraceMulti` (`SceneComponent.GetSocketLocation` Mesh traceStart) (`SceneComponent.GetSocketLocation` Mesh traceStop) traceSize 300.0 "TraceTypeQuery1" false (`self.GetAllChildActors` true)))
  (for _array_element _outhits
    (bind _output_get (set `self.Hit Actor` (`.HitActor` (`GameplayStatics.BreakHitResult` _array_element))))
    (bind _asbp_character (cast `/Game/PathOfLight/bp_Imports/bp_Character` _output_get))
    (`/Engine/EditorBlueprintResources/StandardMacros.IsValid` _asbp_character
      (:`Is Valid`
        (if (`self.ActorHasTag` _output_get "Player")
          (if (not (`/Game/PathOfLight/bp_Imports/bp_Character.IsInvincible?` _asbp_character))
            (`self.K2_DestroyActor` _asbp_character)
            (set `self.DEtection` 0)
            (`BlackboardComponent.SetValueAsEnum` (`AIController.Blackboard` (`AIBlueprintHelperLibrary.GetAIController` self)) (`self.Key`) (enumliteral `/Game/PathOfLight/LD_Prototyping/JavonW/Enemies/AI/Enums/E_AIStates` "NewEnumerator0"))))))))

(event `Parent Check Char`
  (bind _asbp_character (cast `/Game/PathOfLight/bp_Imports/bp_Character` (`GameplayStatics.GetPlayerCharacter` 0)))
  (`/Game/PathOfLight/bp_Imports/bp_Character.CompareNoiseInts` _asbp_character (`self.DEtection`)))

(event `TraceStart`
  (set `self.attackTrace` true))

(event `self.ReceiveBeginPlay`
  (bind _asbp_character (cast `/Game/PathOfLight/bp_Imports/bp_Character` (`GameplayStatics.GetPlayerCharacter` 0)))
  (set `self.As Bp Character` _asbp_character))

(event `TraceStop`
  (set `self.attackTrace` false))

(event `TickDownDetection`
  ;[1 1 1] DO NOT TOUCH (time on event will probably need tweaking)
  (bind _asbp_character (cast `/Game/PathOfLight/bp_Imports/bp_Character` (`GameplayStatics.GetPlayerCharacter` 0)))
  (set `self.As Bp Character` _asbp_character)
  (`KismetSystemLibrary.K2_SetTimerDelegate` (delegate `TickDown`) 0.9 true))

(event `TickDown`
  ;[1 1 1] DO NOT TOUCH (time on event will probably need tweaking)
  (set `self.DEtection` (`KismetMathLibrary.Clamp` (- (`self.DEtection`) 1) 0 12))
  (set `self.RecentlyHeard` true))

(event `HearNoise`
  (params (HeardVector :type "Vector Structure") (Character :type "Pawn Object Reference") (FootstepSense :type Integer :default 2) (DashSense :type Integer :default 6) (InvestigationDefault :type Integer :default 10))
  ;[1 1 1] Enemy hearing detection - Increments
  (set `self.RecentlyHeard` false)
  (bind _asbp_character (cast `/Game/PathOfLight/bp_Imports/bp_Character` Character)
    (:`then`
      (if (`Character.bIsCrouched` _asbp_character)
        (if (>= (`self.DEtection`) InvestigationDefault) :!label _label
          (`BlackboardComponent.SetValueAsEnum` (`AIController.Blackboard` (`AIBlueprintHelperLibrary.GetAIController` self)) (`self.Key`) (enumliteral `/Game/PathOfLight/LD_Prototyping/JavonW/Enemies/AI/Enums/E_AIStates` "NewEnumerator3") :!label _label_2)
          (`BlackboardComponent.SetValueAsVector` (`AIController.Blackboard` (`AIBlueprintHelperLibrary.GetAIController` self)) (`self.POI`) HeardVector)
          (if (== (`self.DEtection`) 12)
            (`BlackboardComponent.SetValueAsEnum` (`AIController.Blackboard` (`AIBlueprintHelperLibrary.GetAIController` self)) (`self.Key`) (enumliteral `/Game/PathOfLight/LD_Prototyping/JavonW/Enemies/AI/Enums/E_AIStates` "NewEnumerator1")))
          (else
            (`BlackboardComponent.SetValueAsEnum` (`AIController.Blackboard` (`AIBlueprintHelperLibrary.GetAIController` self)) (`self.Key`) (enumliteral `/Game/PathOfLight/LD_Prototyping/JavonW/Enemies/AI/Enums/E_AIStates` "NewEnumerator0"))))
        (elif (`/Game/PathOfLight/bp_Imports/bp_Character.Dashing` _asbp_character)
          (set `self.DEtection` (+ (`self.DEtection`) DashSense))
          (if (> (`self.DEtection`) InvestigationDefault)
            (goto _label_2))
          (else
            (set `self.DEtection` (+ (`self.DEtection`) FootstepSense))
            (goto _label)))))
    (:`CastFailed`
      (`BlackboardComponent.SetValueAsEnum` (`AIController.Blackboard` (`AIBlueprintHelperLibrary.GetAIController` self)) (`self.Key`) (enumliteral `/Game/PathOfLight/LD_Prototyping/JavonW/Enemies/AI/Enums/E_AIStates` "NewEnumerator0")))))

(event `See Nosie`
  (params (Character :type "Pawn Object Reference") (CanSee :type Boolean))
  (bind _blackboard (`AIController.Blackboard` (`AIBlueprintHelperLibrary.GetAIController` self)))
  ;[1 1 1] Enemy Sight
  (bind _asbp_character (cast `/Game/PathOfLight/bp_Imports/bp_Character` Character)
    (:`then`
      (set `self.CanSee` true)
      (if (not (`Character.bIsCrouched` _asbp_character))
        (set `self.DEtection` (+ (`self.DEtection`) 12))
        (`KismetSystemLibrary.Delay` 1.0)
        (if (>= (`self.DEtection`) 10)
          (`BlackboardComponent.SetValueAsEnum` _blackboard (`self.Key`) (enumliteral `/Game/PathOfLight/LD_Prototyping/JavonW/Enemies/AI/Enums/E_AIStates` "NewEnumerator3"))
          (if (>= (`self.DEtection`) 12)
            (`BlackboardComponent.SetValueAsEnum` (`AIController.Blackboard` (`AIBlueprintHelperLibrary.GetAIController` self)) (`self.Key`) (enumliteral `/Game/PathOfLight/LD_Prototyping/JavonW/Enemies/AI/Enums/E_AIStates` "NewEnumerator1"))))))
    (:`CastFailed`
      (set `self.CanSee` false)
      (`BlackboardComponent.SetValueAsEnum` _blackboard (`self.Key`) (enumliteral `/Game/PathOfLight/LD_Prototyping/JavonW/Enemies/AI/Enums/E_AIStates` "NewEnumerator0")))))

(fn `UserConstructionScript`)