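; BP_BlindEnemy is a blind enemy character that detects targets by hearing.
; PawnSensing noise events pass the location and instigator to HearNoise and raise a detection value, with TickDownDetection started at BeginPlay.
; Search, give-up and attack events play montages that report back through CallOnAttackEnd, while functions supply the patrol route and set walk speed by movement state.
; Flash-orb stun logic is present but disconnected.
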(event `self.ReceiveActorBeginOverlap`
  (params (OtherActor :type "Actor Object Reference"))
  ;[1 1 1] Flash
)

(event `self.PawnSensing.OnHearNoise`
  (params (Instigator :type "Pawn Object Reference") (Location :type "Vector Structure (by ref)") (Volume :type "Float (single-precision)"))
  ;[1 1 1] Hearing for Detection
  (`self.HearNoise` Location Instigator)
  (set `self.DEtection` (+ (`self.DEtection`) 2))
  (set `self.Can_Hear` true))

(event `self.ReceiveBeginPlay`
  ;[1 1 1] Decrease Detection
  (`self.TickDownDetection`))

(event `self.ReceiveTick`
  (params (DeltaSeconds :type "Float (single-precision)")))

(event `PlaySearch`
  (`|PlayMontage` (`self.Mesh`) "/Game/PathOfLight/Animations/Blind_Search_Montage.Blind_Search_Montage"
    (:`OnCompleted`
      _)
    (:`OnInterrupted`
      _))
  (`self.OnAttackEnd`))

(event `PlayGiveUp`
  (`|PlayMontage` (`self.Mesh`) "/Game/PathOfLight/Animations/Blind_GiveUp_Montage.Blind_GiveUp_Montage"
    (:`OnCompleted`
      _)
    (:`OnInterrupted`
      _))
  (`self.OnAttackEnd`))

(event `PlayAttack`
  (`|PlayMontage` (`self.Mesh`) "/Game/PathOfLight/Animations/Blind_Attack_Montage.Blind_Attack_Montage"
    (:`OnCompleted`
      _)
    (:`OnInterrupted`
      _))
  (`self.OnAttackEnd`))

(fn `GetPatrolRoute`
  (returns (PatrolRoute :type "/Game/PathOfLight/LD_Prototyping/JavonW/Enemies/AI/BP_PatrolRoutes Object Reference"))
  (return (`self.PatrolRoute`)))

(fn `SetMovementSpeed`
  (params (Speed :type "/Game/PathOfLight/LD_Prototyping/JavonW/Enemies/AI/Enums/E_MovementSpeed Enum" :default "NewEnumerator0"))
  (returns (SpeedValue :type "Float (double-precision)"))
  (bind _output_get (set `CharacterMovementComponent.MaxWalkSpeed` (select `/Game/PathOfLight/LD_Prototyping/JavonW/Enemies/AI/Enums/E_MovementSpeed` Speed :`NewEnumerator1` 200.0 :`NewEnumerator2` 300.0 :`NewEnumerator3` 450.0 :!type "Float (single-precision)") (`self.CharacterMovement`)))
  (return _output_get))

(fn `UserConstructionScript`)