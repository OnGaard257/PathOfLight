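; Jackal enemy character that detects the player by sight and hearing, attacks, and can be stunned by flash orbs.
; PawnSensing feeds detection functions, while callable events play montages and sounds for behaviors like notice, search and give-up, firing end callbacks.
; Attacks toggle a per-tick trace; touching the Kill component triggers TouchDeath.
; Flash orb overlap temporarily disables movement and sensing, then resets detection; timelines and presets drive walk speed.
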(event `self.PawnSensing.OnSeePawn`
  (params (Pawn :type "Pawn Object Reference"))
  ;[1 1 1] Sight for Detection
  (`self.See Nosie` Pawn))

(event `self.ReceiveActorBeginOverlap`
  (params (OtherActor :type "Actor Object Reference"))
  ;[1 1 1] Flash
  (cast `/Game/PathOfLight/Blueprints/MichaelF_PT_BP/bp_Flash_Orb` OtherActor)
  (`self.Stun`)
  (`CharacterMovementComponent.DisableMovement` (`self.CharacterMovement`))
  (`PawnSensingComponent.SetSensingUpdatesEnabled` (`self.PawnSensing`) false)
  (`AIController.K2_ClearFocus` (`AIBlueprintHelperLibrary.GetAIController` self))
  (set `self.CanSee` false)
  (`KismetSystemLibrary.Delay` 4.0)
  (`CharacterMovementComponent.SetMovementMode` (`self.CharacterMovement`) "MOVE_Walking" 0)
  (`PawnSensingComponent.SetSensingUpdatesEnabled` (`self.PawnSensing`) true)
  (set `self.DEtection` 0))

(event `self.PawnSensing.OnHearNoise`
  (params (Instigator :type "Pawn Object Reference") (Location :type "Vector Structure (by ref)") (Volume :type "Float (single-precision)"))
  ;[1 1 1] Hearing for Detection
  (`self.HearNoise` Location Instigator 2 6 (`self.Investigation Default`)))

(event `PlayAttack`
  ;[1 1 1] Attack Anim
  (`|ExecutionSequence`
    (:`then_0`
      (set `self.Attacking?` true)
      (`|PlayMontage` (`self.Mesh`) "/Game/PathOfLight/Animations/EnemyAnimate/JackalAttackMontage.JackalAttackMontage"
        (:`OnCompleted`
          _)
        (:`OnInterrupted`
          _))
      (`self.OnAttackEnd`)
      (set `self.Attacking?` false))
    (:`then_1`
      (`KismetSystemLibrary.Delay` 0.2)
      (`GameplayStatics.PlaySoundAtLocation` "/Game/PathOfLight/Sounds/monster-snarl-3-105348.monster-snarl-3-105348" (`SceneComponent.K2_GetComponentLocation` (`self.Mesh`)) (struct) 0.6 1.0 0.0 "/Game/PathOfLight/Sounds/GrowlSoundAttenuation.GrowlSoundAttenuation" null null null))))

(event `self.ReceiveBeginPlay`
  ;[1 1 1] Decrease Detection
  (`self.TickDownDetection`)
  (set `PawnSensingComponent.SightRadius` (`self.Sight Radius`) (`self.PawnSensing`)))

(event `PlayGiveUp`
  ;[1 1 1] Give Up Anim
  (`|ExecutionSequence`
    (:`then_0`
      (`|PlayMontage` (`self.Mesh`) "/Game/PathOfLight/Animations/EnemyAnimate/JackalGiveUpMontage.JackalGiveUpMontage"
        (:`OnCompleted`
          _)
        (:`OnInterrupted`
          _))
      (`self.OnAttackEnd`))
    (:`then_1`
      (`KismetSystemLibrary.Delay` 0.2)
      (`GameplayStatics.PlaySoundAtLocation` "/Game/PathOfLight/Sounds/NickSFX/SFX_BlindGiveUp.SFX_BlindGiveUp" (`SceneComponent.K2_GetComponentLocation` (`self.Mesh`)) (struct) 0.8 1.0 0.0 "/Game/PathOfLight/Sounds/GrowlSoundAttenuation.GrowlSoundAttenuation" null null null))))

(event `TraceStart`
  ;[1 1 1] Code for spawning attack radius
  (set `self.attackTrace` true))

(event `TraceStop`
  ;[1 1 1] Code for spawning attack radius
  (set `self.attackTrace` false))

(event `self.ReceiveTick`
  (params (DeltaSeconds :type "Float (single-precision)"))
  ;[1 1 1] Code for spawning attack radius
  (`|ExecutionSequence`
    (:`then_0`
      (if (`self.attackTrace`)
        (`self.ParentAttackTrace` (`self.Mesh`) (`self.jackalStartTrace`) (`self.jackalEndTrace`))))))

(event `PlaySearch`
  ;[1 1 1] Search Anim
  (`|ExecutionSequence`
    (:`then_0`
      (`|PlayMontage` (`self.Mesh`) "/Game/PathOfLight/Animations/EnemyAnimate/JackalSearchMontage.JackalSearchMontage"
        (:`OnCompleted`
          _)
        (:`OnInterrupted`
          _))
      (`self.OnAttackEnd`))
    (:`then_1`
      (`KismetSystemLibrary.Delay` 0.2)
      (`GameplayStatics.PlaySoundAtLocation` "/Game/PathOfLight/Sounds/NickSFX/SFX_BlindLost.SFX_BlindLost" (`SceneComponent.K2_GetComponentLocation` (`self.Mesh`)) (struct) 0.4 1.0 0.0 "/Game/PathOfLight/Sounds/GrowlSoundAttenuation.GrowlSoundAttenuation" null null null))))

(event `self.Kill.OnComponentBeginOverlap`
  (params (OverlappedComponent :type "PrimitiveComponent Object Reference") (OtherActor :type "Actor Object Reference") (OtherComp :type "PrimitiveComponent Object Reference") (OtherBodyIndex :type Integer) (bFromSweep :type Boolean) (SweepResult :type "HitResult Structure (by ref)"))
  ;[1 1 1] Touch Mesh plays attack
  (cast `/Game/PathOfLight/bp_Imports/bp_Character` OtherActor)
  (set `self.DEtection` 12)
  (`|ExecutionSequence`
    (:`then_0`
      (`self.TouchDeath` "/Game/PathOfLight/Animations/EnemyAnimate/JackalAttackMontage.JackalAttackMontage" self))
    (:`then_1`
      (`KismetSystemLibrary.Delay` 0.2)
      (`GameplayStatics.PlaySoundAtLocation` "/Game/PathOfLight/Sounds/monster-snarl-3-105348.monster-snarl-3-105348" (`SceneComponent.K2_GetComponentLocation` (`self.Mesh`)) (struct) 1.0 1.0 0.0 "/Game/PathOfLight/Sounds/GrowlSoundAttenuation.GrowlSoundAttenuation" null null null))))

(event `Stun`
  ;[1 1 1] Stun Anim
  (`|PlayMontage` (`self.Mesh`) "/Game/PathOfLight/Animations/EnemyAnimate/JackalStunMontage.JackalStunMontage"
    (:`OnCompleted`
      _)
    (:`OnInterrupted`
      _))
  (`self.OnAttackEnd`))

(event `AccelerateSpeed`
  (bind (_direction _track1) (`Timeline|Speed` :!via `PlayFromStart`)
    (:`Update`
      (set `CharacterMovementComponent.MaxWalkSpeed` _track1 (`self.CharacterMovement`)))
    (:`Finished`
      (`self.ReachedSpeed`))))

(event `PlayLook`
  ;[1 1 1] Look Anim
  (`|ExecutionSequence`
    (:`then_0`
      (`|PlayMontage` (`self.Mesh`) "/Game/PathOfLight/Animations/Bat_LookAround_Montage1.Bat_LookAround_Montage1"
        (:`OnCompleted`
          _)
        (:`OnInterrupted`
          _))
      (`self.LookEnd`))
    (:`then_1`
      (`KismetSystemLibrary.Delay` 0.2)
      (`GameplayStatics.PlaySoundAtLocation` "/Game/PathOfLight/Sounds/NickSFX/SFX_BlindLost.SFX_BlindLost" (`SceneComponent.K2_GetComponentLocation` (`self.Mesh`)) (struct) 0.2 1.0 0.0 "/Game/PathOfLight/Sounds/GrowlSoundAttenuation.GrowlSoundAttenuation" null null null))))

(event `WalkToChaseSpeed`
  (bind (_direction _walkaccelerate) (`Timeline|WalkToChase` :!via `PlayFromStart`)
    (:`Update`
      (set `CharacterMovementComponent.MaxWalkSpeed` _walkaccelerate (`self.CharacterMovement`)))
    (:`Finished`
      (`self.ReachedSpeed`))))

(event `PlayNotice`
  ;[1 1 1] Notice Anim
  (`|ExecutionSequence`
    (:`then_0`
      (`|PlayMontage` (`self.Mesh`) "/Game/PathOfLight/Animations/EnemyAnimate/jackal_notice_anim.jackal_notice_anim"
        (:`OnCompleted`
          _)
        (:`OnInterrupted`
          _))
      (`self.OnAttackEnd`))
    (:`then_1`
      (`KismetSystemLibrary.Delay` 0.2)
      (`GameplayStatics.PlaySoundAtLocation` "/Game/PathOfLight/Sounds/ImplementSFX/LuminaryStudios_JackalHowlSampl3.LuminaryStudios_JackalHowlSampl3" (`SceneComponent.K2_GetComponentLocation` (`self.Mesh`)) (struct) 1.0 1.0 0.0 "/Game/PathOfLight/Sounds/GrowlSoundAttenuation.GrowlSoundAttenuation" null null null))))

(fn `GetPatrolRoute`
  (returns (PatrolRoute :type "/Game/PathOfLight/LD_Prototyping/JavonW/Enemies/AI/BP_PatrolRoutes Object Reference"))
  (return (`self.PatrolRoute`)))

(fn `SetMovementSpeed`
  (params (Speed :type "/Game/PathOfLight/LD_Prototyping/JavonW/Enemies/AI/Enums/E_MovementSpeed Enum" :default "NewEnumerator0"))
  (returns (SpeedValue :type "Float (double-precision)"))
  (bind _output_get (set `CharacterMovementComponent.MaxWalkSpeed` (select `/Game/PathOfLight/LD_Prototyping/JavonW/Enemies/AI/Enums/E_MovementSpeed` Speed :`NewEnumerator1` 200.0 :`NewEnumerator2` 300.0 :`NewEnumerator3` 450.0 :`NewEnumerator4` 600.0 :`NewEnumerator5` 650.0 :!type "Float (single-precision)") (`self.CharacterMovement`)))
  (return _output_get))

(fn `UserConstructionScript`)