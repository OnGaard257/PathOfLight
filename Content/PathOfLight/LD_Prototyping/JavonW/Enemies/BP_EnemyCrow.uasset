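; Crow enemy character in a prototyping folder that patrols, detects pawns, attacks, and can be stunned by flash orbs.
; PawnSensing sight and hearing feed detection functions, with a countdown started at BeginPlay and only a debug print at max detection.
; Attack, search, give-up and stun montages all signal attack end, while Tick runs the parent's attack trace when enabled.
; Flash orb overlap temporarily disables movement and sensing; helper functions expose patrol route and speed tiers.
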(event `self.ReceiveActorBeginOverlap`
  (params (OtherActor :type "Actor Object Reference"))
  ;[1 1 1] Flash
  (cast `/Game/PathOfLight/Blueprints/bp_Flash_Orb` OtherActor)
  (`self.Stun`)
  (`CharacterMovementComponent.DisableMovement` (`self.CharacterMovement`))
  (`PawnSensingComponent.SetSensingUpdatesEnabled` (`self.PawnSensing`) false)
  (`KismetSystemLibrary.Delay` 4.0)
  (`CharacterMovementComponent.SetMovementMode` (`self.CharacterMovement`) "MOVE_Walking" 0)
  (`PawnSensingComponent.SetSensingUpdatesEnabled` (`self.PawnSensing`) true)
  (`KismetSystemLibrary.Delay` 0.2))

(event `self.PawnSensing.OnHearNoise`
  (params (Instigator :type "Pawn Object Reference") (Location :type "Vector Structure (by ref)") (Volume :type "Float (single-precision)"))
  ;[1 1 1] Enemy hearing detection - Increments
  (`self.HearNoise` Location Instigator))

(event `self.PawnSensing.OnSeePawn`
  (params (Pawn :type "Pawn Object Reference"))
  ;[1 1 1] Enemy sight detection - Increments
  (`self.See Nosie` Pawn))

(event `self.ReceiveBeginPlay`
  ;[1 1 1] Tick Down
  (`self.TickDownDetection`))

(event `DetectMax`
  (`KismetSystemLibrary.PrintString` "Howdy"))

(event `PlayAttack`
  (`|PlayMontage` (`self.Mesh`) "/Game/PathOfLight/Animations/EnemyAnimate/CrowAttackMontage.CrowAttackMontage"
    (:`OnCompleted`
      _)
    (:`OnInterrupted`
      _))
  (`self.OnAttackEnd`))

(event `PlayGiveUp`
  (`|PlayMontage` (`self.Mesh`) "/Game/PathOfLight/Animations/EnemyAnimate/CrowGiveUpMontage.CrowGiveUpMontage"
    (:`OnCompleted`
      _)
    (:`OnInterrupted`
      _))
  (`self.OnAttackEnd`))

(event `PlaySearch`
  (`|PlayMontage` (`self.Mesh`) "/Game/PathOfLight/Animations/EnemyAnimate/CrowSearchMontage.CrowSearchMontage"
    (:`OnCompleted`
      _)
    (:`OnInterrupted`
      _))
  (`self.OnAttackEnd`))

(event `Stun`
  (`|PlayMontage` (`self.Mesh`) "/Game/PathOfLight/Animations/EnemyAnimate/Crow_Stun_Montage.Crow_Stun_Montage"
    (:`OnCompleted`
      _)
    (:`OnInterrupted`
      _))
  (`self.OnAttackEnd`))

(event `self.ReceiveTick`
  (params (DeltaSeconds :type "Float (single-precision)"))
  (if (`self.attackTrace`)
    (`self.ParentAttackTrace` (`self.Mesh`) (`self.crowStartTrace`) (`self.crowEndTrace`))))

(fn `GetPatrolRoute`
  (returns (PatrolRoute :type "/Game/PathOfLight/LD_Prototyping/JavonW/Enemies/AI/BP_PatrolRoutes Object Reference"))
  (return (`self.PatrolRoute`)))

(fn `SetMovementSpeed`
  (params (Speed :type "/Game/PathOfLight/LD_Prototyping/JavonW/Enemies/AI/Enums/E_MovementSpeed Enum" :default "NewEnumerator0"))
  (returns (SpeedValue :type "Float (double-precision)"))
  (bind _output_get (set `CharacterMovementComponent.MaxWalkSpeed` (select `/Game/PathOfLight/LD_Prototyping/JavonW/Enemies/AI/Enums/E_MovementSpeed` Speed :`NewEnumerator1` 100.0 :`NewEnumerator2` 300.0 :`NewEnumerator3` 500.0 :!type "Float (single-precision)") (`self.CharacterMovement`)))
  (return _output_get))

(fn `UserConstructionScript`)