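; BP_Matriarch is an enemy character that detects the player by sight and hearing, patrols and attacks.
; Pawn sensing feeds inherited-style detection handlers, while montage events for attack, search, notice, give-up and stun signal completion through CallOnAttackEnd.
; Toggled tick traces handle swipes, and touching the player triggers TouchDeath.
; Shield overlap staggers it, pausing movement and senses temporarily; speed comes from presets or an acceleration timeline.
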(event `self.ReceiveActorBeginOverlap`
  (params (OtherActor :type "Actor Object Reference"))
  ;[1 1 1] Flash
  (cast `/Game/PathOfLight/Blueprints/MichaelF_PT_BP/bp_ShieldPT` OtherActor
    (:`then`
      (`KismetSystemLibrary.PrintString` "block lol")
      (`self.Stun`)
      (`CharacterMovementComponent.DisableMovement` (`self.CharacterMovement`))
      (`PawnSensingComponent.SetSensingUpdatesEnabled` (`self.PawnSensing`) false)
      (`KismetSystemLibrary.Delay` 4.0)
      (`CharacterMovementComponent.SetMovementMode` (`self.CharacterMovement`) "MOVE_Walking" 0)
      (`PawnSensingComponent.SetSensingUpdatesEnabled` (`self.PawnSensing`) true))
    (:`CastFailed`
      (`KismetSystemLibrary.PrintString` "Beep"))))

(event `self.PawnSensing.OnHearNoise`
  (params (Instigator :type "Pawn Object Reference") (Location :type "Vector Structure (by ref)") (Volume :type "Float (single-precision)"))
  ;[1 1 1] Hearing for Detection
  (`self.HearNoise` Location Instigator 3 8 5))

(event `self.PawnSensing.OnSeePawn`
  (params (Pawn :type "Pawn Object Reference"))
  ;[1 1 1] Enemy sight detection - Increments
  (`self.See Nosie` Pawn))

(event `Grabbed1stKey`
  ;[1 1 1] Grabbed 1st Light Key
  (bind _asbp_character (cast `/Game/PathOfLight/bp_Imports/bp_Character` (`GameplayStatics.GetPlayerCharacter` 0)))
  (if (> (`/Game/PathOfLight/bp_Imports/bp_Character.KeysObtained` _asbp_character) 0)
    _))

(event `self.ReceiveBeginPlay`
  ;[1 1 1] Decrease Detection
)

(event `self.ReceiveTick`
  (params (DeltaSeconds :type "Float (single-precision)"))
  ;[1 1 1] Attack Trace
  (if (`self.attackTrace`)
    (`self.ParentAttackTrace` (`self.Mesh`) (`self.MatriarchStartTrace`) (`self.MatriarchEndTrace`) 200.0)))

(event `TraceStart`
  ;[1 1 1] Attack Trace
  (set `self.attackTrace` true))

(event `TraceStop`
  ;[1 1 1] Attack Trace
  (set `self.attackTrace` false))

(event `PlayAttack`
  ;[1 1 1] Attack Anim Call
  (set `self.Attacking?` true)
  (`|ExecutionSequence`
    (:`then_0`
      (`|PlayMontage` (`self.Mesh`) "/Game/PathOfLight/Animations/Matriarch_Swipe.Matriarch_Swipe"
        (:`OnCompleted`
          _)
        (:`OnInterrupted`
          _))
      (`self.OnAttackEnd`)
      (set `self.Attacking?` false))
    (:`then_1`
      (`KismetSystemLibrary.Delay` 0.2)
      (`GameplayStatics.PlaySoundAtLocation` "/Game/PathOfLight/Sounds/MatriarchSFX/MatriarchVocals/sfx_M_LightsShort.sfx_M_LightsShort" (`SceneComponent.K2_GetComponentLocation` (`self.CapsuleComponent`)) (struct) 1.0 1.0 0.0 "/Game/PathOfLight/Sounds/GrowlSoundAttenuation.GrowlSoundAttenuation" null null null))))

(event `PlayGiveUp`
  ;[1 1 1] Give up anim call
  (`|ExecutionSequence`
    (:`then_0`
      (`|PlayMontage` (`self.Mesh`) "/Game/PathOfLight/Animations/EnemyAnimate/JackalGiveUpMontage.JackalGiveUpMontage"
        (:`OnCompleted`
          _)
        (:`OnInterrupted`
          _))
      (`self.OnAttackEnd`))
    (:`then_1`
      (`KismetSystemLibrary.Delay` 0.2)
      (`GameplayStatics.PlaySoundAtLocation` "/Game/PathOfLight/Sounds/MatriarchSFX/MatriarchVocals/sfx_M_LightsLong.sfx_M_LightsLong" (`SceneComponent.K2_GetComponentLocation` (`self.CapsuleComponent`)) (struct) 0.5 1.0 0.0 "/Game/PathOfLight/Sounds/GrowlSoundAttenuation.GrowlSoundAttenuation" null null null))))

(event `PlaySearch`
  ;[1 1 1] Search anim call
  (`|PlayMontage` (`self.Mesh`) "/Game/PathOfLight/Animations/Matriarch_Search_Montage.Matriarch_Search_Montage"
    (:`OnCompleted`
      _)
    (:`OnInterrupted`
      _))
  (`self.OnAttackEnd`))

(event `Stun`
  ;[1 1 1] Stun anim call
  (`|PlayMontage` (`self.Mesh`) "/Game/PathOfLight/Animations/MatriarchStagger.MatriarchStagger"
    (:`OnCompleted`
      _)
    (:`OnInterrupted`
      _))
  (`self.OnAttackEnd`))

(event `Notice`
  ;[1 1 1] Notice anim call
  (`|ExecutionSequence`
    (:`then_0`
      (`|PlayMontage` (`self.Mesh`) "/Game/PathOfLight/Animations/Matriarch_Notice.Matriarch_Notice"
        (:`OnCompleted`
          _)
        (:`OnInterrupted`
          _))
      (`self.OnAttackEnd`))
    (:`then_1`
      (`KismetSystemLibrary.Delay` 0.2)
      (`GameplayStatics.PlaySoundAtLocation` "/Game/PathOfLight/Sounds/MatriarchSFX/MatriarchVocals/sfx_M_ISeeYou_long.sfx_M_ISeeYou_long" (`SceneComponent.K2_GetComponentLocation` (`self.CapsuleComponent`)) (struct) 1.0 1.0 0.0 "/Game/PathOfLight/Sounds/GrowlSoundAttenuation.GrowlSoundAttenuation" null null null))))

(event `Accelerate`
  ;[1 1 1] Acceleration event call
  (bind (_direction _walkaccelerate) (`Timeline|Timeline` :!via `PlayFromStart`)
    (:`Update`
      (set `CharacterMovementComponent.MaxWalkSpeed` _walkaccelerate (`self.CharacterMovement`)))
    (:`Finished`
      (`self.Reached Speed`))))

(event `self.CapsuleComponent.OnComponentBeginOverlap`
  (params (OverlappedComponent :type "PrimitiveComponent Object Reference") (OtherActor :type "Actor Object Reference") (OtherComp :type "PrimitiveComponent Object Reference") (OtherBodyIndex :type Integer) (bFromSweep :type Boolean) (SweepResult :type "HitResult Structure (by ref)"))
  ;[1 1 1] Collision hit call
  (cast `/Game/PathOfLight/bp_Imports/bp_Character` OtherActor
    (:`then`
      (set `self.DEtection` 12)
      (`self.TouchDeath` "/Game/PathOfLight/Animations/Matriarch_Swipe.Matriarch_Swipe" self))
    (:`CastFailed`
      (`KismetSystemLibrary.PrintString` "AAAAAAAAAAAAAAAAA"))))

(fn `GetPatrolRoute`
  (returns (PatrolRoute :type "/Game/PathOfLight/LD_Prototyping/JavonW/Enemies/AI/BP_PatrolRoutes Object Reference"))
  (return (`self.PatrolRoute`)))

(fn `SetMovementSpeed`
  (params (Speed :type "/Game/PathOfLight/LD_Prototyping/JavonW/Enemies/AI/Enums/E_MovementSpeed Enum" :default "NewEnumerator0"))
  (returns (SpeedValue :type "Float (double-precision)"))
  (bind _output_get (set `CharacterMovementComponent.MaxWalkSpeed` (select `/Game/PathOfLight/LD_Prototyping/JavonW/Enemies/AI/Enums/E_MovementSpeed` Speed :`NewEnumerator1` 200.0 :`NewEnumerator2` 300.0 :`NewEnumerator3` 450.0 :`NewEnumerator4` 600.0 :`NewEnumerator5` 650.0 :!type "Float (single-precision)") (`self.CharacterMovement`)))
  (return _output_get))

(fn `UserConstructionScript`)