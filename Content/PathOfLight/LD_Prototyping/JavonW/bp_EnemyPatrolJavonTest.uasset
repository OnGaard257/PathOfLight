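; Prototype enemy patrol actor meant to move along a BP_PatrolPoint spline, marked as work in progress and not working.
; MoveObject plays a timeline, rate-scaled by completion time, that sets actor transform from spline world location and local rotation.
; The patrol lookup and MoveObject call are disconnected from the empty BeginPlay, so movement never starts.
; The distance Lerp's Alpha stays zero, so spline length has no effect.
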(event `self.ReceiveBeginPlay`
  ;[1 1 1] WIP Spline Path Follow (Currently does not work)
)

(event `Move Object`
  (bind _spline (`/Game/PathOfLight/LD_Prototyping/JavonW/BP_PatrolPoint.Spline` (`self.Patrol REF`)))
  ;[1 1 1] WIP Spline Path Follow (Currently does not work)
  (`TimelineComponent.SetPlayRate` (`self.Move Object T`) (/ 1.0 (`self.TimeToComplete(InSeconds)`)))
  (bind (_direction _moved_track) (`Timeline|Move Object T`)
    (:`Update`
      (bind _returnvalue (`KismetMathLibrary.Lerp` _moved_track (`SplineComponent.GetSplineLength` (`/Game/PathOfLight/LD_Prototyping/JavonW/BP_PatrolPoint.Spline` (`self.Patrol REF`)))))
      (`self.K2_SetActorTransform` (`KismetMathLibrary.MakeTransform` (`SplineComponent.GetLocationAtDistanceAlongSpline` _spline _returnvalue "World") (`SplineComponent.GetRotationAtDistanceAlongSpline` _spline _returnvalue "Local"))))))

(fn `UserConstructionScript`)