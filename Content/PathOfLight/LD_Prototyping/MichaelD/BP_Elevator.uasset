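; BP_Elevator is a prototype elevator that rises once enough puzzle keys have been collected.
; CollectPuzzleKey increments a counter, and MoveElevatorCheck calls MoveElevator when that count reaches the maximum.
; MoveElevator plays a Timeline that lerps the Plane component's relative Z location upward.
; A DoOnce sits after the MoveElevator call, so it does not gate repeated triggering.
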(event `Move Elevator`
  (bind (_direction _elevator_movement) (`Timeline|Timeline`)
    (:`Update`
      (`SceneComponent.K2_SetRelativeLocation` (`self.Plane`) (`KismetMathLibrary.MakeVector` 0.0 0.0 (`KismetMathLibrary.Lerp` 0.0 500.0 _elevator_movement)) false false))))

(event `Collect PuzzleKey`
  (`/Engine/EditorBlueprintResources/StandardMacros.IncrementInt` (`self.currentitemsCollected`)))

(event `Move Elevator Check`
  (if (>= (`self.currentitemsCollected`) (`self.maxitemsCollectable`))
    (`self.Move Elevator`)
    (`/Engine/EditorBlueprintResources/StandardMacros.DoOnce` false)))

(fn `UserConstructionScript`)