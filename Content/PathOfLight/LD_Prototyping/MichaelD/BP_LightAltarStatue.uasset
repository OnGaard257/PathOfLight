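; Altar statue interactable that shuts a door, plays a one-time prayer sequence and grants the player throwing and staff light.
; A box overlap shows a prompt and enables interact input.
; Interacting repositions the door handle, closes the door by timeline, and removes the prompt and trigger.
; With player input disabled, timelines pulse the prayer light, setting CanThrow during fade-out, while choir audio plays and a delayed staff-light fade-in restores input.
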(event `EnhancedInput|/Game/PathOfLight/bp_Imports/ia_Interact`
  (params (ActionValue :type Boolean) (ElapsedSeconds :type "Float (double-precision)") (TriggeredSeconds :type "Float (double-precision)") (InputAction :type "InputAction Object Reference" :default "/Game/PathOfLight/bp_Imports/ia_Interact.ia_Interact"))
  (bind _doorhandlereference (`self.DoorHandleReference`))
  (:`Triggered`
    (`|ExecutionSequence`
      (:`then_0`
        (`self.K2_SetActorLocation` _doorhandlereference (867.0 -772.0 371.0) false false)
        (`self.K2_SetActorRotation` _doorhandlereference (struct :`Pitch` 90.0) false))
      (:`then_1`
        (bind (_direction _closing_rotation) (`Timeline|DoorClose`)
          (:`Update`
            (`SceneComponent.K2_SetRelativeRotation` (`Actor.RootComponent` (`self.DoorReference`)) (`KismetMathLibrary.MakeRotator` 0.0 0.0 _closing_rotation) false false))))
      (:`then_2`
        (`/Engine/EditorBlueprintResources/StandardMacros.DoOnce` false
          (:`Completed`
            (`self.DisableInput` (`GameplayStatics.GetPlayerPawn` 0) (`GameplayStatics.GetPlayerController` 0))
            (`|ExecutionSequence`
              (:`then_0`
                (`LightComponent.SetIntensity` (`self.PrayerLight`) 0.0)
                (bind (_direction_2 _altarlightfadein) (`Timeline|AltarLightFadeIn`)
                  (:`Update`
                    (`LightComponent.SetIntensity` (`self.PrayerLight`) _altarlightfadein))
                  (:`Finished`
                    (bind (_direction_3 _altarlightfadeout) (`Timeline|AltarLightFadeOut` :`NewTime` 5.0)
                      (:`Update`
                        (`LightComponent.SetIntensity` (`self.PrayerLight`) _altarlightfadeout)
                        (bind _asbp_character (cast `/Game/PathOfLight/bp_Imports/bp_Character` (stale `self.Box.OnComponentBeginOverlap` OtherActor)))
                        (set `/Game/PathOfLight/bp_Imports/bp_Character.CanThrow` true _asbp_character))))))
              (:`then_1`
                (`GameplayStatics.PlaySoundAtLocation` "/Game/PathOfLight/Sounds/Altar_Choir_Final.Altar_Choir_Final" (0.0 0.0 0.0) (struct) 1.0 1.0 0.0 null null null null)
                (`KismetSystemLibrary.Delay` 10.0)
                (set `/Game/PathOfLight/bp_Imports/bp_Character.LumiLightIntensity` 1000.0 (stale `self.Box.OnComponentBeginOverlap` _asbp_character))
                (bind (_direction_4 _stafflightfadein) (`Timeline|LumiLightStaffFadeIn`)
                  (:`Update`
                    (`LightComponent.SetIntensity` (`/Game/PathOfLight/bp_Imports/bp_Character.LumiLight` (stale `self.Box.OnComponentBeginOverlap` _asbp_character)) _stafflightfadein))
                  (:`Finished`
                    (`self.EnableInput` (`GameplayStatics.GetPlayerPawn` 0) (`GameplayStatics.GetPlayerController` 0)))))))))
      (:`then_3`
        (`Widget.RemoveFromParent` (`self.InteractPrompt2`))
        (`ActorComponent.K2_DestroyComponent` (`self.Box`))))))

(event `self.Box.OnComponentBeginOverlap`
  (params (OverlappedComponent :type "PrimitiveComponent Object Reference") (OtherActor :type "Actor Object Reference") (OtherComp :type "PrimitiveComponent Object Reference") (OtherBodyIndex :type Integer) (bFromSweep :type Boolean) (SweepResult :type "HitResult Structure (by ref)"))
  (`|ExecutionSequence`
    (:`then_0`
      (bind _asbp_character (cast `/Game/PathOfLight/bp_Imports/bp_Character` OtherActor))
      (`self.EnableInput` (`GameplayStatics.GetPlayerController` 0)))
    (:`then_1`
      (if (== OtherActor (`GameplayStatics.GetPlayerCharacter` 0))
        (`UserWidget.AddToViewport` (`self.InteractPrompt2`) 0)))))

(event `self.ReceiveBeginPlay`
  (bind _returnvalue (`|CreateWidget` "/Game/PathOfLight/UI/wbp_InteractPrompt.wbp_InteractPrompt_C"))
  (set `self.InteractPrompt2` _returnvalue))

(event `self.Box.OnComponentEndOverlap`
  (params (OverlappedComponent :type "PrimitiveComponent Object Reference") (OtherActor :type "Actor Object Reference") (OtherComp :type "PrimitiveComponent Object Reference") (OtherBodyIndex :type Integer))
  (if (== (`GameplayStatics.GetPlayerCharacter` 0) OtherActor)
    (`Widget.RemoveFromParent` (`self.InteractPrompt2`))))

(fn `UserConstructionScript`)