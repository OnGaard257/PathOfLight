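; Tutorial door Blueprint that opens once enough light key pickups are collected.
; LightKeyPickup increments a collected counter, and MoveDoor calls OpenDoor when that count reaches the maximum collectable.
; OpenDoor plays a timeline whose ElevatorMovement track drives the door mesh's relative yaw to swing it open.
; A DoOnce follows the OpenDoor call rather than preceding it, so it does not prevent repeated opening.
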(event `OpenDoor`
  (bind (_direction _elevator_movement) (`Timeline|Timeline`)
    (:`Update`
      (`SceneComponent.K2_SetRelativeRotation` (`self.Door`) (`KismetMathLibrary.MakeRotator` 0.0 0.0 _elevator_movement) false false))))

(event `LightKeyPickup`
  (`/Engine/EditorBlueprintResources/StandardMacros.IncrementInt` (`self.currentitemsCollected`)))

(event `MoveDoor`
  (if (>= (`self.currentitemsCollected`) (`self.maxitemsCollectable`))
    (`self.OpenDoor`)
    (`/Engine/EditorBlueprintResources/StandardMacros.DoOnce` false)))

(fn `UserConstructionScript`)