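; BP_FlickeringLightSlow is a point light Blueprint meant to flicker slowly at random intervals.
; The construction script sets the base intensity, and BeginPlay runs a random retriggerable delay into a FlipFlop whose A output dims the light and loops back.
; The B output is unconnected and the restore-intensity branch never runs, so the light dims once and the loop stops after the next delay.
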(event `self.ReceiveBeginPlay`
  (`KismetSystemLibrary.RetriggerableDelay` (`KismetMathLibrary.RandomFloatInRange` (`self.MinTime`) (`self.MaxTime`)) :!label _label)
  (`/Engine/EditorBlueprintResources/StandardMacros.FlipFlop`
    (:`A`
      (`LightComponent.SetIntensity` (`self.PointLight`) (`self.MinFlickerIntensity`))
      (goto _label))))

(fn `UserConstructionScript`
  (`LightComponent.SetIntensity` (`self.PointLight`) (`self.Intensity`)))