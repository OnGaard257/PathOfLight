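; BP_LightKey is a key pickup that adds to the player character's KeysObtained count on overlap.
; Its collider's begin-overlap event casts to bp_Character, increments the count, spawns the Key_Pickup effect at the key, plays Softer_Pickup at world origin, then destroys the actor.
; A Sequence holds two identical copies of this chain, so the increment, effect and sound are each issued twice per overlap.
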(event `self.Collider.OnComponentBeginOverlap`
  (params (OverlappedComponent :type "PrimitiveComponent Object Reference") (OtherActor :type "Actor Object Reference") (OtherComp :type "PrimitiveComponent Object Reference") (OtherBodyIndex :type Integer) (bFromSweep :type Boolean) (SweepResult :type "HitResult Structure (by ref)"))
  (`|ExecutionSequence`
    (:`then_0`
      (bind _asbp_character (cast `/Game/PathOfLight/bp_Imports/bp_Character` OtherActor))
      (`/Engine/EditorBlueprintResources/StandardMacros.IncrementInt` (`/Game/PathOfLight/bp_Imports/bp_Character.KeysObtained` _asbp_character)
        (:`  `
          (`NiagaraFunctionLibrary.SpawnSystemAtLocation` "/Game/PathOfLight/VFX/Misc_Effects/Key_Pickup.Key_Pickup" (`self.K2_GetActorLocation`))
          (`GameplayStatics.SpawnSoundAtLocation` "/Game/PathOfLight/Sounds/Softer_Pickup.Softer_Pickup" (0.0 0.0 0.0) (struct) 0.9 1.0 0.0 null null)
          (`self.K2_DestroyActor`))))
    (:`then_1`
      (bind _asbp_character_2 (cast `/Game/PathOfLight/bp_Imports/bp_Character` OtherActor))
      (`/Engine/EditorBlueprintResources/StandardMacros.IncrementInt` (`/Game/PathOfLight/bp_Imports/bp_Character.KeysObtained` _asbp_character_2)
        (:`  `
          (`NiagaraFunctionLibrary.SpawnSystemAtLocation` "/Game/PathOfLight/VFX/Misc_Effects/Key_Pickup.Key_Pickup" (`self.K2_GetActorLocation`))
          (`GameplayStatics.SpawnSoundAtLocation` "/Game/PathOfLight/Sounds/Softer_Pickup.Softer_Pickup" (0.0 0.0 0.0) (struct) 0.9 1.0 0.0 null null)
          (`self.K2_DestroyActor`))))))

(fn `UserConstructionScript`)