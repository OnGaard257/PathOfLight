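; Light key pickup that shows an interact prompt and outline while the player character overlaps its sphere.
; Interact, gated by the overlap and an empty-hand check, passes a DoOnce to increment KeysObtained, halt character movement and trigger TuckAway.
; A separate DestroyOrb event plays the pickup sound, resets the DoOnce and destroys the LightKey-tagged actor nearest the character's mesh, rather than itself.
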(event `self.ReceiveBeginPlay`
  (`|ExecutionSequence`
    (:`then_0`
      (bind _returnvalue (`|CreateWidget` "/Game/PathOfLight/UI/wbp_InteractPrompt.wbp_InteractPrompt_C"))
      (set `self.InteractPrompt` _returnvalue))
    (:`then_1`
      (`self.EnableInput` (`GameplayStatics.GetPlayerController` 0)))))

(event `Destroy Orb`
  (bind _outactors (`GameplayStatics.GetAllActorsWithTag` "LightKey"))
  (`GameplayStatics.PlaySoundAtLocation` "/Game/PathOfLight/Sounds/Softer_Pickup.Softer_Pickup" (0.0 0.0 0.0) (struct) 0.5 1.0 0.0 null null null null)
  (`|ExecutionSequence`
    (:`then_0`
      (goto _label_2 :!via `Reset`))
    (:`then_1`
      (`self.K2_DestroyActor` (`.ReturnValue` (`GameplayStatics.FindNearestActor` (`SceneComponent.K2_GetComponentLocation` (`Character.Mesh` (stale `EnhancedInput|/Game/PathOfLight/bp_Imports/ia_Interact` _asbp_character))) _outactors))))))

(event `EnhancedInput|/Game/PathOfLight/bp_Imports/ia_Interact`
  (params (ActionValue :type Boolean) (ElapsedSeconds :type "Float (double-precision)") (TriggeredSeconds :type "Float (double-precision)") (InputAction :type "InputAction Object Reference" :default "/Game/PathOfLight/bp_Imports/ia_Interact.ia_Interact"))
  (:`Triggered`
    (bind _asbp_character (cast `/Game/PathOfLight/bp_Imports/bp_Character` (`GameplayStatics.GetPlayerPawn` 0)))
    (if (`/Game/PathOfLight/bp_Imports/bp_Character.NoHeldItem` _asbp_character)
      (`/Engine/EditorBlueprintResources/StandardMacros.Gate` true :!label _label
        (:`Exit`
          (`/Engine/EditorBlueprintResources/StandardMacros.DoOnce` false :!label _label_2
            (:`Completed`
              (bind _keysobtained (`/Game/PathOfLight/bp_Imports/bp_Character.KeysObtained` _asbp_character))
              (bind _result (`/Engine/EditorBlueprintResources/StandardMacros.IncrementInt` _keysobtained)
                (:`  `
                  (set `/Game/PathOfLight/bp_Imports/bp_Character.KeysObtained` _result _asbp_character)
                  (`KismetSystemLibrary.PrintString` (`KismetStringLibrary.Conv_IntToString` _keysobtained))
                  (`CharacterMovementComponent.SetMovementMode` (`Character.CharacterMovement` _asbp_character) "MOVE_None" 0)
                  (set `/Game/PathOfLight/bp_Imports/bp_Character.TuckAway?` true _asbp_character)
                  (`/Game/PathOfLight/bp_Imports/bp_Character.TuckAway` _asbp_character))))))))))

(event `self.Sphere1.OnComponentBeginOverlap`
  (params (OverlappedComponent :type "PrimitiveComponent Object Reference") (OtherActor :type "Actor Object Reference") (OtherComp :type "PrimitiveComponent Object Reference") (OtherBodyIndex :type Integer) (bFromSweep :type Boolean) (SweepResult :type "HitResult Structure (by ref)"))
  (`|ExecutionSequence`
    (:`then_0`
      (cast `/Game/PathOfLight/bp_Imports/bp_Character` OtherActor)
      (`MeshComponent.SetOverlayMaterial` (`self.Sphere`) "/Game/PathOfLight/Materials/m_Outline_Inst.m_Outline_Inst")
      (goto _label :!via `Open`))
    (:`then_1`
      (if (== (`GameplayStatics.GetPlayerCharacter` 0) OtherActor)
        (`UserWidget.AddToViewport` (`self.InteractPrompt`) 0)))))

(event `self.Sphere1.OnComponentEndOverlap`
  (params (OverlappedComponent :type "PrimitiveComponent Object Reference") (OtherActor :type "Actor Object Reference") (OtherComp :type "PrimitiveComponent Object Reference") (OtherBodyIndex :type Integer))
  (`|ExecutionSequence`
    (:`then_0`
      (cast `/Game/PathOfLight/bp_Imports/bp_Character` OtherActor)
      (`MeshComponent.SetOverlayMaterial` (`self.Sphere`) null)
      (goto _label :!via `Close`))
    (:`then_1`
      (if (== (`GameplayStatics.GetPlayerCharacter` 0) OtherActor)
        (`Widget.RemoveFromParent` (`self.InteractPrompt`))))))

(fn `UserConstructionScript`)