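; Cavern light key pickup: a fairy-lit orb the player collects with Interact, showing a prompt and outline while overlapped.
; Overlap opens a gate for Interact, which, unless the character is busy, passes a DoOnce to lock movement and play the tuck-away.
; DestroyOrb spawns a color-matched thrown key if one is held, increments KeysObtained, activates a tag-selected data layer and destroys the nearest LightKey-tagged actor.
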(event `self.ReceiveBeginPlay`
  (`|ExecutionSequence`
    (:`then_0`
      (bind _returnvalue (`|CreateWidget` "/Game/PathOfLight/UI/Tutorials/wbp_InteractPrompt.wbp_InteractPrompt_C"))
      (set `self.InteractPrompt` _returnvalue))
    (:`then_1`
      (`self.EnableInput` (`GameplayStatics.GetPlayerController` 0)))
    (:`then_2`
      (bind _returnvalue_2 (`NiagaraFunctionLibrary.SpawnSystemAtLocation` "/Game/PathOfLight/VFX/Fire_and_smoke/VFX_FairyLights.VFX_FairyLights" (`self.K2_GetActorLocation`)))
      (set `self.Fairy` _returnvalue_2))))

(event `Destroy Orb`
  (bind _returnvalue (subsystem `DataLayerSubsystem`))
  (bind _defaultsceneroot (`self.DefaultSceneRoot`))
  (bind _returnvalue_2 (`SceneComponent.K2_GetComponentLocation` _defaultsceneroot))
  (bind _returnvalue_3 (`SceneComponent.K2_GetComponentRotation` _defaultsceneroot))
  (if (`/Game/PathOfLight/bp_Imports/bp_Character.ThrowKey` (stale `EnhancedInput|/Game/PathOfLight/bp_Imports/ia_Interact` _asbp_character))
    (bind _colorindex (`/Game/PathOfLight/bp_Imports/bp_Character.ColorIndex` (stale `EnhancedInput|/Game/PathOfLight/bp_Imports/ia_Interact` _asbp_character)))
    (if (== _colorindex 0)
      (`|SpawnActorFromClass` "/Game/PathOfLight/Blueprints/bp_ThrowKeyTest.bp_ThrowKeyTest_C" (`KismetMathLibrary.MakeTransform` _returnvalue_2 _returnvalue_3) "Undefined" "MultiplyWithRoot" null null)
      (set `/Game/PathOfLight/bp_Imports/bp_Character.NoHeldItem` true (stale `EnhancedInput|/Game/PathOfLight/bp_Imports/ia_Interact` _asbp_character) :!label _label)
      (bind _outactors (`GameplayStatics.GetAllActorsWithTag` "LightKey" :!label _label_2))
      (`GameplayStatics.PlaySoundAtLocation` "/Game/PathOfLight/Sounds/Softer_Pickup.Softer_Pickup" (0.0 0.0 0.0) (struct) 0.3 1.0 0.0 null null null null)
      (`|ExecutionSequence`
        (:`then_0`
          (goto _label_4 :!via `Reset`))
        (:`then_1`
          (bind _result (`/Engine/EditorBlueprintResources/StandardMacros.IncrementInt` (`/Game/PathOfLight/bp_Imports/bp_Character.KeysObtained` (stale `EnhancedInput|/Game/PathOfLight/bp_Imports/ia_Interact` _asbp_character)))
            (:`  `
              (set `/Game/PathOfLight/bp_Imports/bp_Character.KeysObtained` _result (stale `EnhancedInput|/Game/PathOfLight/bp_Imports/ia_Interact` _asbp_character))
              (bind _returnvalue_4 (`GameplayStatics.GetActorOfClass` "/Game/PathOfLight/bp_Imports/bp_Character.bp_Character_C"))
              (`/Game/PathOfLight/bp_Imports/HUD_UI.OrbCheck` (`/Game/PathOfLight/bp_Imports/bp_Character.CooldownUIRef` _returnvalue_4))
              (if (`self.ActorHasTag` "1")
                (`DataLayerSubsystem.SetDataLayerRuntimeState` _returnvalue (`self.In Data Layer`) "Activated" false)
                (else
                  (`DataLayerSubsystem.SetDataLayerRuntimeState` _returnvalue (`self.In Data Layer_0`) "Activated" false))))))
        (:`then_2`
          (`self.K2_DestroyActor` (`.ReturnValue` (`GameplayStatics.FindNearestActor` (`SceneComponent.K2_GetComponentLocation` (`Character.Mesh` (stale `EnhancedInput|/Game/PathOfLight/bp_Imports/ia_Interact` _asbp_character))) _outactors)))
          (`NiagaraFunctionLibrary.SpawnSystemAtLocation` "/Game/PathOfLight/VFX/Misc_Effects/Key_Pickup.Key_Pickup" (`self.K2_GetActorLocation`))
          (`ActorComponent.K2_DestroyComponent` (`self.Fairy`))))
      (elif (== _colorindex 1)
        (`|SpawnActorFromClass` "/Game/PathOfLight/Blueprints/bp_ThrowKeyTest_Red.bp_ThrowKeyTest_Red_C" (`KismetMathLibrary.MakeTransform` _returnvalue_2 _returnvalue_3) "Undefined" "MultiplyWithRoot" null null)
        (goto _label)
        (elif (== _colorindex 2)
          (`|SpawnActorFromClass` "/Game/PathOfLight/Blueprints/bp_ThrowKeyTest_Blue.bp_ThrowKeyTest_Blue_C" (`KismetMathLibrary.MakeTransform` _returnvalue_2 _returnvalue_3) "Undefined" "MultiplyWithRoot" null null)
          (goto _label)
          (elif (== _colorindex 3)
            (`|SpawnActorFromClass` "/Game/PathOfLight/Blueprints/bp_ThrowKeyTest_Green.bp_ThrowKeyTest_Green_C" (`KismetMathLibrary.MakeTransform` _returnvalue_2 _returnvalue_3) "Undefined" "MultiplyWithRoot" null null)
            (goto _label)
            (elif (== _colorindex 4)
              (`|SpawnActorFromClass` "/Game/PathOfLight/Blueprints/bp_ThrowKeyTest_Yellow.bp_ThrowKeyTest_Yellow_C" (`KismetMathLibrary.MakeTransform` _returnvalue_2 _returnvalue_3) "Undefined" "MultiplyWithRoot" null null)
              (goto _label))))))
    (else
      (goto _label_2))))

(event `LightKeyPickup`)

(event `EnhancedInput|/Game/PathOfLight/bp_Imports/ia_Interact`
  (params (ActionValue :type Boolean) (ElapsedSeconds :type "Float (double-precision)") (TriggeredSeconds :type "Float (double-precision)") (InputAction :type "InputAction Object Reference" :default "/Game/PathOfLight/bp_Imports/ia_Interact.ia_Interact"))
  (:`Triggered`
    (`|ExecutionSequence`
      (:`then_0`
        (bind _asbp_character (cast `/Game/PathOfLight/bp_Imports/bp_Character` (`GameplayStatics.GetPlayerPawn` 0)))
        (if (`/Game/PathOfLight/bp_Imports/bp_Character.Stunning?` _asbp_character)
          _
          (elif (`/Game/PathOfLight/bp_Imports/bp_Character.Shielding` _asbp_character)
            _
            (elif (not (`/Game/PathOfLight/bp_Imports/bp_Character.Throw Anim` _asbp_character))
              (`/Engine/EditorBlueprintResources/StandardMacros.Gate` true :!label _label_3
                (:`Exit`
                  (if (not (`/Game/PathOfLight/bp_Imports/bp_Character.Dashing` _asbp_character))
                    (`/Engine/EditorBlueprintResources/StandardMacros.DoOnce` false :!label _label_4
                      (:`Completed`
                        (`CharacterMovementComponent.SetMovementMode` (`Character.CharacterMovement` _asbp_character) "MOVE_None" 0)
                        (`/Game/PathOfLight/bp_Imports/bp_Character.TuckAway` _asbp_character)
                        (`|CreateWidget` "/Game/PathOfLight/UI/Menu_Screens/wbp_OrbObtained.wbp_OrbObtained_C"))))))))))
      (:`then_1`
        (goto _label_4 :!via `Reset`)))))

(event `self.Sphere1.OnComponentBeginOverlap`
  (params (OverlappedComponent :type "PrimitiveComponent Object Reference") (OtherActor :type "Actor Object Reference") (OtherComp :type "PrimitiveComponent Object Reference") (OtherBodyIndex :type Integer) (bFromSweep :type Boolean) (SweepResult :type "HitResult Structure (by ref)"))
  (`|ExecutionSequence`
    (:`then_0`
      (bind _asbp_character (cast `/Game/PathOfLight/bp_Imports/bp_Character` OtherActor))
      (set `/Game/PathOfLight/bp_Imports/bp_Character.LightKeyOverlap?` true _asbp_character)
      (`MeshComponent.SetOverlayMaterial` (`self.Sphere`) "/Game/PathOfLight/Materials/m_Outline_Inst.m_Outline_Inst")
      (goto _label_3 :!via `Open`))
    (:`then_1`
      (if (== (`GameplayStatics.GetPlayerCharacter` 0) OtherActor)
        (`UserWidget.AddToViewport` (`self.InteractPrompt`) 0)))))

(event `self.Sphere1.OnComponentEndOverlap`
  (params (OverlappedComponent :type "PrimitiveComponent Object Reference") (OtherActor :type "Actor Object Reference") (OtherComp :type "PrimitiveComponent Object Reference") (OtherBodyIndex :type Integer))
  (`|ExecutionSequence`
    (:`then_0`
      (bind _asbp_character (cast `/Game/PathOfLight/bp_Imports/bp_Character` OtherActor))
      (set `/Game/PathOfLight/bp_Imports/bp_Character.LightKeyOverlap?` false _asbp_character)
      (`MeshComponent.SetOverlayMaterial` (`self.Sphere`) null)
      (goto _label_3 :!via `Close`))
    (:`then_1`
      (if (== (`GameplayStatics.GetPlayerCharacter` 0) OtherActor)
        (`Widget.RemoveFromParent` (`self.InteractPrompt`))))))

(fn `UserConstructionScript`)