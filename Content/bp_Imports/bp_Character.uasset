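; Player character Blueprint with Enhanced Input movement, look, crouch and a cooldown-limited dash.
; BeginPlay adds the Cooldown_UI widget to the viewport and registers the main input mapping context.
; Dash launches the character forward, then upward after a short delay, using a DoOnce and timed reset as the cooldown, tracked by a Dashed flag.
; Crouch pairs the built-in crouch with halving the capsule's world scale until release.
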(event `self.ReceiveBeginPlay`
  ;[1 1 1] Player Locomotion
  (bind _returnvalue (`|CreateWidget` "/Game/bp_Imports/Cooldown_UI.Cooldown_UI_C"))
  (`UserWidget.AddToViewport` _returnvalue 0)
  (bind _asplayer_controller (cast `PlayerController` (`self.GetController`)))
  (bind _returnvalue_2 (pcsubsystem `EnhancedInputLocalPlayerSubsystem` _asplayer_controller))
  (`/Engine/EditorBlueprintResources/StandardMacros.IsValid` _returnvalue_2
    (:`Is Valid`
      (`EnhancedInputSubsystemInterface.AddMappingContext` _returnvalue_2 "/Game/bp_Imports/imc_Main.imc_Main" 0 (struct)))))

(event `EnhancedInput|/Game/bp_Imports/ia_Dash`
  (params (ActionValue :type "Vector2D Structure") (ElapsedSeconds :type "Float (double-precision)") (TriggeredSeconds :type "Float (double-precision)") (InputAction :type "InputAction Object Reference" :default "/Game/bp_Imports/ia_Dash.ia_Dash"))
  (bind _returnvalue (`self.K2_GetActorRotation`))
  ;[1 1 1] Dash Mechanic
  (:`Triggered`
    (`/Engine/EditorBlueprintResources/StandardMacros.DoOnce` false :!label _label
      (:`Completed`
        (`self.LaunchCharacter` (* (`KismetMathLibrary.GetForwardVector` _returnvalue) 1000.0))
        (`KismetSystemLibrary.Delay` 0.1)
        (`self.LaunchCharacter` (* (`KismetMathLibrary.GetUpVector` _returnvalue) 300.0))
        (set `self.Dashed?` true)
        (`KismetSystemLibrary.Delay` 2.0)
        (set `self.Dashed?` false)
        (goto _label :!via `Reset`)))))

(event `EnhancedInput|/Game/bp_Imports/ia_Movement`
  (params (ActionValue :type "Vector2D Structure") (ElapsedSeconds :type "Float (double-precision)") (TriggeredSeconds :type "Float (double-precision)") (InputAction :type "InputAction Object Reference" :default "/Game/bp_Imports/ia_Movement.ia_Movement"))
  (bind (_returnvalue_roll _returnvalue_pitch _returnvalue_yaw) (`KismetMathLibrary.BreakRotator` (`self.GetControlRotation`)))
  ;[1 1 1] Player Locomotion
  (:`Triggered`
    (`self.AddMovementInput` (`KismetMathLibrary.GetRightVector` (`KismetMathLibrary.MakeRotator` _returnvalue_roll 0.0 _returnvalue_yaw)) ActionValue_X)
    (`self.AddMovementInput` (`KismetMathLibrary.GetForwardVector` (`KismetMathLibrary.MakeRotator` 0.0 0.0 _returnvalue_yaw)) ActionValue_Y)))

(event `EnhancedInput|/Game/bp_Imports/ia_Look`
  (params (ActionValue :type "Vector2D Structure") (ElapsedSeconds :type "Float (double-precision)") (TriggeredSeconds :type "Float (double-precision)") (InputAction :type "InputAction Object Reference" :default "/Game/bp_Imports/ia_Look.ia_Look"))
  ;[1 1 1] Player Locomotion
  (:`Triggered`
    (`self.AddControllerYawInput` ActionValue_X)
    (`self.AddControllerPitchInput` ActionValue_Y)))

(event `EnhancedInput|/Game/bp_Imports/ia_Crouch`
  (params (ActionValue :type Boolean) (ElapsedSeconds :type "Float (double-precision)") (TriggeredSeconds :type "Float (double-precision)") (InputAction :type "InputAction Object Reference" :default "/Game/bp_Imports/ia_Crouch.ia_Crouch"))
  (bind _capsulecomponent (`self.CapsuleComponent`))
  ;[1 1 1] Crouch
  (:`Triggered`
    (`self.Crouch`)
    (`SceneComponent.SetWorldScale3D` _capsulecomponent (0.5 0.5 0.5)))
  (:`Completed`
    (`self.UnCrouch`)
    (`SceneComponent.SetWorldScale3D` _capsulecomponent (1.0 1.0 1.0))))

(fn `UserConstructionScript`)